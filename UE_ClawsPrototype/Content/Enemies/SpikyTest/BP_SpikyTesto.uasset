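; BP_SpikyTesto is a test spiky enemy that can be flipped upside down once it has been watered.
; It starts with Habitated set to true, and the Watered event clears that flag.
; Flip acts only when the flag is cleared, raising the actor, setting its pitch to 180 degrees and switching the capsule's mobility to Static.
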(event `self.ReceiveBeginPlay`
  (set `self.habitated ` true))

(event `Watered`
  (set `self.habitated ` false))

(event `Flip`
  (bind (_returnvalue_roll _returnvalue_pitch _returnvalue_yaw) (`KismetMathLibrary.BreakRotator` (`self.K2_GetActorRotation`)))
  (if (not (`self.habitated `))
    (`self.K2_SetActorLocationAndRotation` (`KismetMathLibrary.MakeVector` (.x (`self.K2_GetActorLocation`)) (.y (`self.K2_GetActorLocation`)) (+ (.z (`self.K2_GetActorLocation`)) 100.0)) (`KismetMathLibrary.MakeRotator` _returnvalue_roll 180.0 _returnvalue_yaw))
    (`SceneComponent.SetMobility` (`self.CapsuleComponent`) "Static")))

(fn `UserConstructionScript`)