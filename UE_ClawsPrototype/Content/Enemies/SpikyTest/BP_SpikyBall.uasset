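; BP_SpikyBall is a spiky ball character that starts inhabited and can be shot as a projectile once it has been vacated.
; The Wet event clears the inhabited flag, which lets BallShoot launch it along a fixed world +X and upward arc.
; After launch, a capsule hit against a WorldStatic component destroys the actor.
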(event `self.ReceiveBeginPlay`
  (set `self.HabitatedBall` true))

(event `/Game/Interfaces/BPI_Enemy.Wet`
  (set `self.HabitatedBall` false))

(event `BallShoot`
  (if (not (`self.HabitatedBall`))
    (`self.LaunchCharacter` (1500.0 0.0 750.0))
    (set `self.launched` true)))

(event `self.CapsuleComponent.OnComponentHit`
  (params (HitComponent :type "PrimitiveComponent Object Reference") (OtherActor :type "Actor Object Reference") (OtherComp :type "PrimitiveComponent Object Reference") (NormalImpulse :type "Vector Structure") (Hit :type "HitResult Structure (by ref)"))
  (if (and (`self.launched`) (`|EnumEquality` (`PrimitiveComponent.GetCollisionObjectType` OtherComp) "ECC_WorldStatic"))
    (`self.K2_DestroyActor`)))

(fn `UserConstructionScript`)