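; Speedy enemy character Blueprint that extends a parent class and caches its max walk speed on BeginPlay.
; Its Powered event sets a powered flag and launches it upward along a fixed world-space velocity, overriding current motion.
; When an actor implementing the player interface enters its sphere, it raises the PlayerJump Blackboard key on its AI controller, then clears it after a short delay.
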(event `self.ReceiveBeginPlay`
  (`parent.ReceiveBeginPlay`)
  (set `self.BaseMaxWalkSpeed` (`CharacterMovementComponent.MaxWalkSpeed` (`self.CharacterMovement`))))

(event `/Game/Interfaces/BPI_Enemy.Powered`
  (set `self.isPowered` true)
  (`self.LaunchCharacter` (-700.0 0.0 1500.0) true true))

(event `self.Sphere.OnComponentBeginOverlap`
  (params (OverlappedComponent :type "PrimitiveComponent Object Reference") (OtherActor :type "Actor Object Reference") (OtherComp :type "PrimitiveComponent Object Reference") (OtherBodyIndex :type Integer) (bFromSweep :type Boolean) (SweepResult :type "HitResult Structure (by ref)"))
  (bind _blackboard (`AIController.Blackboard` (`AIBlueprintHelperLibrary.GetAIController` self)))
  (if (`KismetSystemLibrary.DoesImplementInterface` OtherActor "/Game/Setup/BPI_Player.BPI_Player_C")
    (`BlackboardComponent.SetValueAsBool` _blackboard "PlayerJump" true)
    (`KismetSystemLibrary.Delay` 2.0)
    (`BlackboardComponent.SetValueAsBool` _blackboard "PlayerJump" false)))

(fn `UserConstructionScript`
  (`parent.UserConstructionScript`))