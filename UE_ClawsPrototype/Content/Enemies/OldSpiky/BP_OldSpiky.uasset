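; Old Spiky enemy that knocks back and stuns the player on contact, and becomes a jump booster when flipped.
; Flip disables bump collision, starts an Unflip timer and mirrors the state to the AI Blackboard.
; While flipped, belly overlap boosts player jumps and pauses the timer until exit resets it.
; Bumps use a forward-vector dot product to launch both characters apart along world X; the exact-perpendicular case is WIP.
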(event `self.ReceiveBeginPlay`
  ;[1 1 1] Comment
  (bind _get_pc_ref (message `/Game/Interfaces/BPI_PlayerController.Get PC Ref` (`GameplayStatics.GetPlayerController` 0)))
  (set `self.PlayerController` _get_pc_ref)
  (bind _get_player_ref (message `/Game/Setup/BPI_Player.Get Player Ref` (`GameplayStatics.GetPlayerCharacter` 0)))
  (set `self.Player Ref` _get_player_ref)
  (set `self.Default Max Walk Speed` (`CharacterMovementComponent.MaxWalkSpeed` (`self.CharacterMovement`)))
  (bind _asaic_old_spiky (cast `/Game/Enemies/OldSpiky/AIC_OldSpiky` (`AIBlueprintHelperLibrary.GetAIController` self))
    (:`then`
      (set `self.Blackboard` (`AIController.Blackboard` _asaic_old_spiky)))
    (:`CastFailed`
      (`KismetSystemLibrary.PrintString` "Hello"))))

(event `self.BellyCollision.OnComponentEndOverlap`
  (params (OverlappedComponent :type "PrimitiveComponent Object Reference") (OtherActor :type "Actor Object Reference") (OtherComp :type "PrimitiveComponent Object Reference") (OtherBodyIndex :type Integer))
  ;[1 1 1] When overlap Belly, register the info
  (if (and (`KismetSystemLibrary.DoesImplementInterface` OtherActor "/Game/Setup/BPI_Player.BPI_Player_C") (`self.flipped`))
    (set `self.isOnBelly` false)
    (`/Game/Utilities/BPFL.ResetTimerByEvent` (delegate `Unflip`) (`self.FlipTimer`))
    (`/Game/Setup/BP_CharaBase.Unboost Jump` (`self.Player Ref`))))

(event `self.BellyCollision.OnComponentBeginOverlap`
  (params (OverlappedComponent :type "PrimitiveComponent Object Reference") (OtherActor :type "Actor Object Reference") (OtherComp :type "PrimitiveComponent Object Reference") (OtherBodyIndex :type Integer) (bFromSweep :type Boolean) (SweepResult :type "HitResult Structure (by ref)"))
  ;[1 1 1] Launch when flipped and jump
  (if (and (`KismetSystemLibrary.DoesImplementInterface` OtherActor "/Game/Setup/BPI_Player.BPI_Player_C") (`self.flipped`))
    (set `self.isOnBelly` true)
    (`/Game/Setup/BP_CharaBase.BoostJump` (`self.Player Ref`) 500.0)
    (`KismetSystemLibrary.K2_PauseTimerHandle` (`self.FlipTimer`))))

(event `BellyBump`
  (bind (_returnvalue_x _returnvalue_y _returnvalue_z) (`KismetMathLibrary.BreakVector` (`self.GetVelocity` (`self.Player Ref`))))
  ;[1 1 1] Launch when flipped and jump
  (if (> _returnvalue_z 0.0)
    (`self.LaunchCharacter` (`self.Player Ref`) (0.0 0.0 500.0) false true)))

(event `Flip`
  (bind _returnvalue (`self.K2_GetActorLocation`))
  (bind (_returnvalue_roll _returnvalue_pitch _returnvalue_yaw) (`KismetMathLibrary.BreakRotator` (`self.K2_GetActorRotation`)))
  ;[1 1 1] Flip
  (if (`self.flipped`)
    (`GameplayStatics.PlaySound2D` "/Game/SoundDesign/Sounds/PowerClawOff_Cue.PowerClawOff_Cue" 1.0 1.0 0.0 null null)
    (else
      (`GameplayStatics.PlaySoundAtLocation` "/Game/SoundDesign/Sounds/S_FlipSpiky_Cue.S_FlipSpiky_Cue" _returnvalue (struct) 1.0 1.0 0.0 null null null null)
      (`self.K2_SetActorLocationAndRotation` (`KismetMathLibrary.MakeVector` (.x _returnvalue) (.y _returnvalue) (+ (.z _returnvalue) 18.0)) (`KismetMathLibrary.MakeRotator` _returnvalue_roll 180.0 _returnvalue_yaw))
      (bind _output_get (set `self.flipped` true))
      (bind _returnvalue_2 (`KismetSystemLibrary.K2_SetTimerDelegate` (delegate `Unflip`) 4.0))
      (`PrimitiveComponent.SetCollisionEnabled` (`self.BumpCollision`) "NoCollision")
      (set `self.FlipTimer` _returnvalue_2)
      (bind _blackboard (`self.Blackboard`)
        (:`then`
          (`BlackboardComponent.SetValueAsBool` _blackboard "Flipped" _output_get))
        (:`else`)))))

(event `self.ReceiveTick`
  (params (DeltaSeconds :type "Float (single-precision)")))

(event `self.BumpCollision.OnComponentHit`
  (params (HitComponent :type "PrimitiveComponent Object Reference") (OtherActor :type "Actor Object Reference") (OtherComp :type "PrimitiveComponent Object Reference") (NormalImpulse :type "Vector Structure") (Hit :type "HitResult Structure (by ref)"))
  (bind (_bblockinghit _binitialoverlap _time _distance _location _impactpoint _normal _impactnormal) (`GameplayStatics.BreakHitResult` Hit))
  ;[1 0.4327 0] CRADE When player enters in contact, launch BUMP function
  (if (`KismetSystemLibrary.DoesImplementInterface` OtherActor "/Game/Setup/BPI_Player.BPI_Player_C")
    (`KismetSystemLibrary.DrawDebugArrow` _impactpoint (+ _impactpoint (* (`KismetMathLibrary.Normal` _impactnormal) -400.0)) 10.0 (struct :`R` 1.0 :`B` 0.692445 :`A` 1.0) 10.0 5.0)
    (if (`KismetMathLibrary.BooleanNOR` (`self.flipped`) (`self._isBumping`))
      ;;[1 0 0.8894] Cette fonction devrait plus être dans le player, dans la mesure ou plusieurs ennemis peuvent le bump
      (`self.Bump Trial`))))

(event `Unflip`
  (bind (_returnvalue_x _returnvalue_y _returnvalue_z) (`KismetMathLibrary.BreakVector` (`self.K2_GetActorLocation`)))
  (bind (_returnvalue_roll _returnvalue_pitch _returnvalue_yaw) (`KismetMathLibrary.BreakRotator` (`self.K2_GetActorRotation`)))
  ;[1 1 1] Unflip
  (`KismetSystemLibrary.K2_ClearAndInvalidateTimerHandle` (`self.FlipTimer`))
  (`self.K2_SetActorLocationAndRotation` (`KismetMathLibrary.MakeVector` _returnvalue_x _returnvalue_y (- _returnvalue_z 18.0)) (`KismetMathLibrary.MakeRotator` _returnvalue_roll 180.0 _returnvalue_yaw))
  (`GameplayStatics.PlaySoundAtLocation` "/Game/SoundDesign/Sounds/FlipEnemy_Cue.FlipEnemy_Cue" (`self.K2_GetActorLocation`) (struct) 1.0 1.0 0.0 null null null null)
  (bind _output_get (set `self.flipped` false))
  (`PrimitiveComponent.SetCollisionEnabled` (`self.BumpCollision`) "QueryOnly")
  (bind _blackboard (`self.Blackboard`)
    (:`then`
      (`BlackboardComponent.SetValueAsBool` _blackboard "Flipped" _output_get))
    (:`else`)))

(event `self.BumpCollision.OnComponentBeginOverlap`
  (params (OverlappedComponent :type "PrimitiveComponent Object Reference") (OtherActor :type "Actor Object Reference") (OtherComp :type "PrimitiveComponent Object Reference") (OtherBodyIndex :type Integer) (bFromSweep :type Boolean) (SweepResult :type "HitResult Structure (by ref)"))
  ;[1 0.4327 0] CRADE When player enters in contact, launch BUMP function
)

(event `Bump Trial`
  ;[1 1 1] Bump Function
  (set `self._isBumping` true)
  (`NavMovementComponent.StopActiveMovement` (`self.CharacterMovement`))
  (`MovementComponent.StopMovementImmediately` (`Character.CharacterMovement` (`self.Player Ref`)))
  ;;[1 1 1] Si >0 c'est que le cos est >0 donc que l'angle des 2 vect est entre 00° (donc alignés) et 89°, soit à droite du Spiky, donc on le launch à droite.
  (bind _output_get (set `self.Dot Value` (`KismetMathLibrary.Dot_VectorVector` (`KismetMathLibrary.Normal` (- (`self.K2_GetActorLocation` (`self.Player Ref`)) (`self.K2_GetActorLocation`))) (`self.GetActorForwardVector`))))
  (if (> _output_get 0.0)
    (`self.LaunchCharacter` (`self.Player Ref`) (1500.0 0.0 800.0) false false)
    (`self.LaunchCharacter` (-500.0 0.0 100.0) true true)
    (else
      ;;[1 1 1] Si <0 c'est que le cos est <0 donc que l'angle des 2 vect est entre 91° et 180° (aligné opposé), soit à gauche du Spiky, donc on le launch à gauche
      (if (< (`self.Dot Value`) 0.0)
        (`self.LaunchCharacter` (`self.Player Ref`) (-1500.0 0.0 800.0) false false)
        (`self.LaunchCharacter` (500.0 0.0 100.0) true true)
        (else
          ;;[1 0.9054 0.03333] Sinon, ==0, et c'est que l'angle des 2 vect est de 90°, donc pile au milieu du spiky, donc pour savoir où le launch va falloir faire un truc plus complexe >>>> WIP
          (`self.LaunchCharacter` (-1500.0 0.0 800.0))
          (`self.LaunchCharacter` (500.0 0.0 100.0) true true)))))
  (`GameplayStatics.PlaySound2D` "/Game/SoundDesign/Sounds/Jump_Cue.Jump_Cue" 1.0 1.0 0.0 null null)
  (set `self._isBumping` false)
  (`/Game/Setup/PC_ClawsProto.Stun` (`self.PlayerController`) 1.0))

(fn `UserConstructionScript`)