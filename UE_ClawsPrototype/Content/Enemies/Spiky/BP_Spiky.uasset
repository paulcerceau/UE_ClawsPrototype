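; BP_Spiky is a Character Blueprint for the Spiky enemy, which reacts to Wet and Powered events through a HabitatedSpike flag.
; Wet clears the flag, while Powered, if it is still set, calls LaunchCharacter with zero velocity and marks the enemy as launched.
; Once launched, a shell ball component hit against a WorldStatic object destroys the actor.
; Disconnected nodes that would flip it over and make its capsule static never run.
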(event `/Game/Interfaces/BPI_Enemy.Wet`
  (if (`self.HabitatedSpike`)
    (set `self.HabitatedSpike` false)))

(event `/Game/Interfaces/BPI_Enemy.Powered`
  (if (`self.HabitatedSpike`)
    (`self.LaunchCharacter` (0.0 0.0 0.0))
    (set `self.Launched` true)))

(event `self.GPE_ShellBall_Blockout.OnComponentHit`
  (params (HitComponent :type "PrimitiveComponent Object Reference") (OtherActor :type "Actor Object Reference") (OtherComp :type "PrimitiveComponent Object Reference") (NormalImpulse :type "Vector Structure") (Hit :type "HitResult Structure (by ref)"))
  (if (and (`self.Launched`) (`|EnumEquality` (`PrimitiveComponent.GetCollisionObjectType` OtherComp) "ECC_WorldStatic"))
    (`self.K2_DestroyActor`)))

(fn `UserConstructionScript`)