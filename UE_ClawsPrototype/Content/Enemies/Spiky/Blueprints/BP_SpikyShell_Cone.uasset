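; Cone variant of the Spiky enemy's shell, which flips over when powered.
; The Powered event raises the actor by FlipHeightValue and sets its pitch to an absolute 180 degrees in one instant move, keeping X, Y, roll and yaw.
; GetACShell returns the cone-specific ACSpikyShellCone.
; BeginPlay, overlap and Tick are disabled stubs, and construction only calls the parent.
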(event `/Game/Interfaces/BPI_Enemy.Powered`
  (bind (_returnvalue_roll _returnvalue_pitch _returnvalue_yaw) (`KismetMathLibrary.BreakRotator` (`self.K2_GetActorRotation`)))
  (`self.K2_SetActorLocationAndRotation` (`KismetMathLibrary.MakeVector` (.x (`self.K2_GetActorLocation`)) (.y (`self.K2_GetActorLocation`)) (+ (.z (`self.K2_GetActorLocation`)) (`self.FlipHeightValue`))) (`KismetMathLibrary.MakeRotator` _returnvalue_roll 180.0 _returnvalue_yaw)))

(fn `Get AC Shell`
  (returns (`AC SpikyShell` :type "/Game/Enemies/Spiky/Blueprints/AC_SpikyShell Object Reference"))
  (return (`self.AC_SpikyShell_Cone`)))

(fn `UserConstructionScript`
  (`parent.UserConstructionScript`))