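; Spiky shelled enemy that hides its body on proximity overlap and knocks the player back on contact, briefly disabling input.
; Powered toggles a flip while hidden, with a timer meant to restore rotation and spawn position unless the Flipreset volume is occupied.
; Wet reveals the body and, when unflipped, nudges the actor away from the player along X.
; The construction script sets the shell mesh, and component mobility switches around moves.
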(event `self.ReceiveBeginPlay`
  (`|ExecutionSequence`
    (:`then_0`
      (`SceneComponent.SetMobility` (`self.ShellMesh`) "Static")
      (bind _asbp_chara_base (cast `/Game/Setup/BP_CharaBase` (`GameplayStatics.GetPlayerCharacter` 0)))
      (set `self.As BP Chara Base` _asbp_chara_base)
      (bind _aspc_claws_proto (cast `/Game/Setup/PC_ClawsProto` (`GameplayStatics.GetPlayerController` 0)))
      (set `self.As PC Claws Proto` _aspc_claws_proto))
    (:`then_1`
      (if (not (`self.Visible`))
        (`SceneComponent.SetVisibility` (`self.SpikyMesh`) false false)))
    (:`then_2`
      (set `self.Spawn` (`SceneComponent.K2_GetComponentLocation` (`self.Box`))))))

(event `self.Hidding distance.OnComponentBeginOverlap`
  (params (OverlappedComponent :type "PrimitiveComponent Object Reference") (OtherActor :type "Actor Object Reference") (OtherComp :type "PrimitiveComponent Object Reference") (OtherBodyIndex :type Integer) (bFromSweep :type Boolean) (SweepResult :type "HitResult Structure (by ref)"))
  (set `self.Visible` false)
  (`SceneComponent.SetVisibility` (`self.SpikyMesh`) false false))

(event `self.Hidding distance.OnComponentEndOverlap`
  (params (OverlappedComponent :type "PrimitiveComponent Object Reference") (OtherActor :type "Actor Object Reference") (OtherComp :type "PrimitiveComponent Object Reference") (OtherBodyIndex :type Integer))
  (if (not (`self.flipped`))
    (set `self.Visible` true)
    (`SceneComponent.SetVisibility` (`self.SpikyMesh`) true false)))

(event `self.Flipreset.OnComponentBeginOverlap`
  (params (OverlappedComponent :type "PrimitiveComponent Object Reference") (OtherActor :type "Actor Object Reference") (OtherComp :type "PrimitiveComponent Object Reference") (OtherBodyIndex :type Integer) (bFromSweep :type Boolean) (SweepResult :type "HitResult Structure (by ref)"))
  (set `self.On spiky` true)
  (`KismetSystemLibrary.K2_ClearAndInvalidateTimerHandle` (`self.FlipTimer`))
  (`self.CheckFlipBack`))

(event `/Game/Interfaces/BPI_Enemy.Powered`
  (if (`self.Visible`)
    _
    (elif (`self.flipped`)
      (`self.FlipBack`)
      (if (not (`self.On spiky`))
        (set `self.flipped` false)
        (`SceneComponent.SetMobility` (`self.SpikyMesh`) "Movable")
        (`SceneComponent.K2_SetWorldLocation` (`self.Box`) (`self.Spawn`) false false))
      (else
        (`self.Flip`)
        (set `self.flipped` true)
        (`self.CheckFlipBack`)))))

(event `self.Flipreset.OnComponentEndOverlap`
  (params (OverlappedComponent :type "PrimitiveComponent Object Reference") (OtherActor :type "Actor Object Reference") (OtherComp :type "PrimitiveComponent Object Reference") (OtherBodyIndex :type Integer))
  (set `self.On spiky` false))

(event `CheckFlipBack`
  (bind _returnvalue (`KismetSystemLibrary.K2_SetTimerDelegate` (`|CreateDelegate` :!event `FlipBackOk`) 5.0))
  (set `self.FlipTimer` _returnvalue))

(event `FlipBackOk`
  (if (`self.On spiky`)
    (`self.CheckFlipBack`)
    (elif (`self.flipped`)
      (`SceneComponent.SetMobility` (`self.SpikyMesh`) "Movable")
      (`self.FlipBack`)
      (`SceneComponent.K2_SetWorldLocation` (`self.Box`) (`self.Spawn`) false false))))

(event `/Game/Interfaces/BPI_Enemy.Wet`
  (bind _returnvalue_x (`KismetMathLibrary.BreakVector` (`self.K2_GetActorLocation`)))
  (bind _returnvalue_x_2 (`KismetMathLibrary.BreakVector` (`self.K2_GetActorLocation` (`GameplayStatics.GetPlayerCharacter` 0))))
  (set `self.Visible` true)
  (`SceneComponent.SetVisibility` (`self.SpikyMesh`) true false)
  (if (not (`self.flipped`))
    (`SceneComponent.SetMobility` (`self.SpikyMesh`) "Movable")
    (if (> _returnvalue_x_2 _returnvalue_x)
      (`self.K2_AddActorWorldOffset` (-5.0 0.0 0.0))
      (if (and (`self.On spiky`) (`self.flipped`))
        (`KismetSystemLibrary.Delay` 7.0)
        (`SceneComponent.SetMobility` (`self.SpikyMesh`) "Movable")
        (`SceneComponent.K2_SetWorldLocation` (`self.Box`) (`self.Spawn`) false false))
      (else
        (`self.K2_AddActorWorldOffset` (5.0 0.0 0.0) true)
        (if (and (`self.On spiky`) (`self.flipped`))
          (`KismetSystemLibrary.Delay` 7.0)
          (`SceneComponent.SetMobility` (`self.SpikyMesh`) "Movable")
          (`SceneComponent.K2_SetWorldLocation` (`self.Box`) (`self.Spawn`) false false))))))

(event `self.BumpBox.OnComponentBeginOverlap`
  (params (OverlappedComponent :type "PrimitiveComponent Object Reference") (OtherActor :type "Actor Object Reference") (OtherComp :type "PrimitiveComponent Object Reference") (OtherBodyIndex :type Integer) (bFromSweep :type Boolean) (SweepResult :type "HitResult Structure (by ref)"))
  (bind _as_bp_chara_base (`self.As BP Chara Base`))
  (bind _as_pc_claws_proto (`self.As PC Claws Proto`))
  (bind _as_pc_claws_proto_2 (`self.As PC Claws Proto`))
  (bind _as_bp_chara_base_2 (`self.As BP Chara Base`))
  (if (`KismetSystemLibrary.DoesImplementInterface` OtherActor "/Game/Setup/BPI_Player.BPI_Player_C")
    (bind _output_get (set `self.DOT Value` (`KismetMathLibrary.Dot_VectorVector` (`KismetMathLibrary.Normal` (- (`self.K2_GetActorLocation` (`self.As BP Chara Base`)) (`SceneComponent.K2_GetComponentLocation` (`self.ShellMesh`)))) (`SceneComponent.GetForwardVector` (`self.ShellMesh`)))))
    (if (>= _output_get 0.0)
      (`Character.LaunchCharacter` _as_bp_chara_base (1500.0 0.0 1000.0) true true)
      (`KismetSystemLibrary.Delay` 0.5)
      (`self.DisableInput` _as_bp_chara_base _as_pc_claws_proto)
      (`KismetSystemLibrary.Delay` 0.2)
      (`self.EnableInput` _as_bp_chara_base _as_pc_claws_proto_2)
      (else
        (`Character.LaunchCharacter` _as_bp_chara_base_2 (-1500.0 0.0 1000.0) true true)
        (`KismetSystemLibrary.Delay` 0.5)
        (`self.DisableInput` _as_bp_chara_base_2 _as_pc_claws_proto)
        (`KismetSystemLibrary.Delay` 0.2)
        (`self.EnableInput` _as_bp_chara_base_2 _as_pc_claws_proto_2)))))

(fn `ChangeShell`
  (params (Shell :type "/Game/Enemies/Spiky/Blueprints/BP_SpikyShell_Parent Class Reference"))
  (`StaticMeshComponent.SetStaticMesh` (`self.ShellMesh`) (defaults `Object` Shell)))

(fn `Flip`
  (bind (_returnvalue_roll _returnvalue_pitch _returnvalue_yaw) (`KismetMathLibrary.BreakRotator` (`self.K2_GetActorRotation`)))
  (`SceneComponent.SetMobility` (`self.ShellMesh`) "Movable")
  (`self.K2_SetActorLocationAndRotation` (`KismetMathLibrary.MakeVector` (.x (`self.K2_GetActorLocation`)) (.y (`self.K2_GetActorLocation`)) (+ (.z (`self.K2_GetActorLocation`)) (`self.FlippedHeighVariable`))) (`KismetMathLibrary.MakeRotator` _returnvalue_roll 180.0 _returnvalue_yaw))
  (set `self.flipped` true)
  (`SceneComponent.SetMobility` (`self.ShellMesh`) "Static"))

(fn `FlipBack`
  (bind (_returnvalue_roll _returnvalue_pitch _returnvalue_yaw) (`KismetMathLibrary.BreakRotator` (`self.K2_GetActorRotation`)))
  (`SceneComponent.SetMobility` (`self.SpikyMesh`) "Movable")
  (`self.K2_SetActorLocationAndRotation` (`KismetMathLibrary.MakeVector` (.x (`self.K2_GetActorLocation`)) (.y (`self.K2_GetActorLocation`)) (- (.z (`self.K2_GetActorLocation`)) (`self.FlippedHeighVariable`))) (`KismetMathLibrary.MakeRotator` _returnvalue_roll 180.0 _returnvalue_yaw))
  (set `self.flipped` false)
  (`SceneComponent.SetMobility` (`self.SpikyMesh`) "Static"))

(fn `UserConstructionScript`
  (`self.ChangeShell` (`self.Shell`)))