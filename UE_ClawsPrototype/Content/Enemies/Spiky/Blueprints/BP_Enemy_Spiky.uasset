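; Spiky enemy Blueprint that sets its shell's skeletal mesh from shell data held by a BPSpiky actor in the level.
; The construction script calls ChangeShell, which finds that actor by class, reads the shell data asset from its shell component and applies the mesh to SKShell.
; The event graph holds only disabled default events, so the file adds no runtime behavior of its own.
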(fn `ChangeShell`
  (params (Shell :type "/Game/Enemies/Spiky/Blueprints/BP_SpikyShell_Parent Class Reference"))
  (bind _returnvalue (`GameplayStatics.GetActorOfClass` Shell))
  (bind _ac_spikyshell (`/Game/Enemies/Spiky/Blueprints/BP_SpikyShell_Parent.Get AC Shell` _returnvalue))
  (bind _shell_pda_asset (`/Game/Enemies/Spiky/Blueprints/AC_SpikyShell.Get Shells PDA` _ac_spikyshell))
  (bind _output_get (set `self.Shell PDA Asset` _shell_pda_asset))
  (bind (_spiky_commondata_classtoinstanciate _spiky_commondata_shellactor _spiky_commondata_shellskmesh) (break `/Game/Enemies/Spiky/Data/S_SpikyShell` (`/Game/Enemies/Spiky/Data/PDA_SpikyShell.Spiky_CommonData` _output_get)))
  (bind _output_get_2 (set `self.ShellMesh` _spiky_commondata_shellskmesh))
  (`SkeletalMeshComponent.SetSkeletalMeshAsset` (`self.SK_Shell`) _output_get_2))

(fn `UserConstructionScript`
  (`parent.UserConstructionScript`)
  (`self.ChangeShell` (`self.BP_Spiky`)))