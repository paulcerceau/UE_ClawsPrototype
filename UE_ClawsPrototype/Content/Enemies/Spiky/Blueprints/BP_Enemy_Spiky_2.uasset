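; Spiky enemy that knocks back and briefly stuns the player on contact unless flipped, reacting to Water and Power claws with Wwise audio.
; Water pushes it along X through a temporary Tick lerp, with line traces halting it at walls or ledges.
; Power toggles a raised, flipped state; a timer rights it once its Flipreset volume is clear.
; A HidingZone sphere and blocked pushes trigger timed hiding.
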(event `self.ReceiveTick`
  (params (DeltaSeconds :type "Float (single-precision)"))
  ;[0.9294 0.2275 0.2275] EXTREMELY TEMPORARY
  (if (`self.TryingToMove`)
    (set `self.MovementElapsedTime` (+ (`self.MovementElapsedTime`) DeltaSeconds))
    (if (> (`self.MovementElapsedTime`) (`self.MovementDuration`))
      (set `self.TryingToMove` false)
      (set `self.MovementElapsedTime` 0.0)
      (set `self.InteractionState` "NewEnumerator1")
      ;[1 1 1] Stop sounds water Spiky
      (`AkGameplayStatics.PostEvent` "/Game/WwiseAudio/Events/Work_Unit_Elise_Events/Spiky/Stop_SPIKY_WaterClaw_Flee_LP.Stop_SPIKY_WaterClaw_Flee_LP" self)
      (`AkGameplayStatics.PostEvent` "/Game/WwiseAudio/Events/Work_Unit_Elise_Events/Spiky/Play_SPIKY_WaterClaw_Flee_End.Play_SPIKY_WaterClaw_Flee_End" self)
      (set `self.SoundWetPlayed` false)
      (else
        ;[1 1 1] Stop movement if there is a wall or no ground
        (bind _bcanmove (`self.CanMoveInDirection` (`self.MovementDirection`)))
        (if _bcanmove
          (`self.K2_SetActorLocation` (`KismetMathLibrary.VLerp` (`self.FromPos`) (`self.ToPos`) (/ (`self.MovementElapsedTime`) (`self.MovementDuration`))))
          (else
            (`self.Hide`)
            (set `self.InteractionState` "NewEnumerator1")
            (set `self.MovementDuration` 0.0)))))))

(event `self.ReceiveBeginPlay`
  ;[0.8824 0.9294 0.2275] BeginPlay
  (`self.InitializeReferences`)
  (set `self.SpawnLocation` (`self.K2_GetActorLocation`)))

(event `/Game/Interfaces/BPI_WetPowered.GetWatered`
  (params (HitLocation :type "Vector Structure"))
  ;[1 1 1] WaterClaw
  (if (not (`|EnumEquality` (`self.InteractionState`) "NewEnumerator3"))
    (set `self.InteractionState` "NewEnumerator2")
    (bind (_succeed _pushdirection) (`self.Try Push Spiky` HitLocation))
    (set `self.MovementDirection` _pushdirection))
  ;;[1 1 1] Sound Water on Spiky
  (`AkGameplayStatics.PostEvent` "/Game/WwiseAudio/Events/Work_Unit_Elise_Events/Spiky/Play_SPIKY_WaterClaw_Shell.Play_SPIKY_WaterClaw_Shell" self)
  (if (not (`self.SoundWetPlayed`))
    (`AkGameplayStatics.PostEvent` "/Game/WwiseAudio/Events/Work_Unit_Elise_Events/Spiky/Play_SPIKY_WaterClaw.Play_SPIKY_WaterClaw" self)
    (set `self.SoundWetPlayed` true)))

(event `/Game/Interfaces/BPI_WetPowered.GetPowered`
  (params (HitLocation :type "Vector Structure"))
  ;[1 1 1] PowerClaw
  (if (`|EnumEquality` (`self.InteractionState`) "NewEnumerator3")
    (`self.FlipBack`)
    (if (not (`self.bOnSpiky`))
      (set `self.InteractionState` "NewEnumerator1")
      (`AkGameplayStatics.PostEventAtLocation` "/Game/WwiseAudio/Events/Work_Unit_Elise_Events/Spiky/Play_SPIKY_PowerClaw_FlippedDown.Play_SPIKY_PowerClaw_FlippedDown" (`SceneComponent.K2_GetComponentLocation` (`self.SK_Spiky`))))
    (else
      (`self.Flip`)
      (`self.CheckFlipBack`)
      (`AkGameplayStatics.PostEventAtLocation` "/Game/WwiseAudio/Events/Work_Unit_Elise_Events/Spiky/Play_SPIKY_PowerClaw_FlippedUp.Play_SPIKY_PowerClaw_FlippedUp" (`SceneComponent.K2_GetComponentLocation` (`self.SK_Spiky`))))))

(event `self.SK_Spiky.OnComponentHit`
  (params (HitComponent :type "PrimitiveComponent Object Reference") (OtherActor :type "Actor Object Reference") (OtherComp :type "PrimitiveComponent Object Reference") (NormalImpulse :type "Vector Structure") (Hit :type "HitResult Structure (by ref)"))
  (bind _returnvalue_x (`KismetMathLibrary.BreakVector` (`self.K2_GetActorLocation` OtherActor)))
  (bind _returnvalue_x_2 (`KismetMathLibrary.BreakVector` (`self.K2_GetActorLocation`)))
  (bind _as_bp_chara_base (`self.As BP Chara Base`))
  ;[1 1 1] Bumping
  (if (and (`KismetSystemLibrary.DoesImplementInterface` OtherActor "/Game/Setup/Remi/BPI_Player.BPI_Player_C") (not (`|EnumEquality` (`self.InteractionState`) "NewEnumerator3")))
    (if (< _returnvalue_x_2 _returnvalue_x)
      (`Character.LaunchCharacter` _as_bp_chara_base (1000.0 0.0 1000.0) true true)
      (else
        (`Character.LaunchCharacter` (`self.As BP Chara Base`) (-1000.0 0.0 1000.0) true true)))
    (`/Game/Setup/Remi/PC_ClawsProto.Stun` (`self.As PC Claws Proto`) 0.1)
    (`/Game/Setup/Remi/BP_CharaBase.AlterAirMobility` _as_bp_chara_base 0.3 5.0 2.0 0.5)
    (`/Game/Setup/Remi/BP_CharaBase.ResetJump` _as_bp_chara_base 1)))

(event `self.Flipreset.OnComponentBeginOverlap`
  (params (OverlappedComponent :type "PrimitiveComponent Object Reference") (OtherActor :type "Actor Object Reference") (OtherComp :type "PrimitiveComponent Object Reference") (OtherBodyIndex :type Integer) (bFromSweep :type Boolean) (SweepResult :type "HitResult Structure (by ref)"))
  ;[1 1 1] Flip/Unflip
  (set `self.bOnSpiky` true)
  (`KismetSystemLibrary.K2_ClearAndInvalidateTimerHandle` (`self.FlipTimer`))
  (`self.CheckFlipBack`))

(event `self.Flipreset.OnComponentEndOverlap`
  (params (OverlappedComponent :type "PrimitiveComponent Object Reference") (OtherActor :type "Actor Object Reference") (OtherComp :type "PrimitiveComponent Object Reference") (OtherBodyIndex :type Integer))
  ;[1 1 1] Flip/Unflip
  (set `self.bOnSpiky` false))

(event `self.HidingZone.OnComponentBeginOverlap`
  (params (OverlappedComponent :type "PrimitiveComponent Object Reference") (OtherActor :type "Actor Object Reference") (OtherComp :type "PrimitiveComponent Object Reference") (OtherBodyIndex :type Integer) (bFromSweep :type Boolean) (SweepResult :type "HitResult Structure (by ref)"))
  ;[0.9294 0.9294 0.9294] Hide triggers
  (if (`KismetSystemLibrary.DoesImplementInterface` OtherActor "/Game/Setup/Remi/BPI_Player.BPI_Player_C")
    (`self.Hide`)))

(event `Hide`
  ;[1 1 1] Hide events
  (set `self.MovementState` "NewEnumerator2")
  (bind _returnvalue (`KismetSystemLibrary.K2_SetTimerDelegate` (`|CreateDelegate` :!event `unhide`) 5.0))
  (set `self.HideTH` _returnvalue))

(event `CheckFlipBack`
  ;[1 1 1] Flip/Unflip
  (bind _returnvalue (`KismetSystemLibrary.K2_SetTimerDelegate` (`|CreateDelegate` :!event `FlipBackOk`) 5.0))
  (set `self.FlipTimer` _returnvalue))

(event `self.HidingZone.OnComponentEndOverlap`
  (params (OverlappedComponent :type "PrimitiveComponent Object Reference") (OtherActor :type "Actor Object Reference") (OtherComp :type "PrimitiveComponent Object Reference") (OtherBodyIndex :type Integer))
  ;[0.9294 0.9294 0.9294] Hide triggers
  (if (`KismetSystemLibrary.DoesImplementInterface` OtherActor "/Game/Setup/Remi/BPI_Player.BPI_Player_C")
    (`self.unhide`)))

(event `Unhide`
  ;[1 1 1] Hide events
  (if (or (<= (`KismetMathLibrary.Vector_Distance` (`self.K2_GetActorLocation` (`self.As BP Chara Base`)) (`self.K2_GetActorLocation`)) (`self.HideDistance`)) (`|EnumEquality` (`self.InteractionState`) "NewEnumerator3"))
    (`/Game/Utilities/BPFL.ResetTimerByEvent` (`|CreateDelegate` :!event `unhide`) (`self.HideTH`))
    (else
      (set `self.MovementState` "NewEnumerator1")
      (`KismetSystemLibrary.K2_ClearAndInvalidateTimerHandle` (`self.HideTH`)))))

(event `FlipBackOk`
  ;[1 1 1] Flip/Unflip
  (if (`self.bOnSpiky`)
    (`self.CheckFlipBack`)
    (elif (`|EnumEquality` (`self.InteractionState`) "NewEnumerator3")
      (`self.FlipBack`))))

(fn `CanMoveInDirection`
  (params (MovementDirection :type "Float (double-precision)"))
  (returns (bCanMove :type Boolean))
  (bind _bhitobstacle (`self.CheckForObstacle` MovementDirection))
  (bind _bisabovevoid (`self.CheckForVoid` MovementDirection))
  (return (not (or _bisabovevoid _bhitobstacle))))

(fn `CheckForObstacle`
  (params (Direction :type "Float (double-precision)"))
  (returns (bHitObstacle :type Boolean))
  (bind _returnvalue (`self.K2_GetActorLocation`))
  (bind (_outhit _returnvalue_2) (`KismetSystemLibrary.LineTraceSingle` _returnvalue (+ _returnvalue (* (`self.GetActorForwardVector`) (150.0 0.0 0.0) (`local.Direction`))) "TraceTypeQuery1"))
  (return _returnvalue_2))

(fn `CheckForVoid`
  (params (Direction :type "Float (double-precision)"))
  (returns (bIsAboveVoid :type Boolean))
  (bind _returnvalue (`self.K2_GetActorLocation`))
  (bind (_outhit _returnvalue_2) (`KismetSystemLibrary.LineTraceSingle` :`Start` _returnvalue :`End` (+ (+ _returnvalue (* (`self.GetActorForwardVector`) (150.0 0.0 0.0) (`local.Direction`))) (0.0 0.0 -125.0)) :`TraceChannel` "TraceTypeQuery1" :`TraceColor` (struct :`R` 0.514252 :`B` 1.0 :`A` 1.0) :`TraceHitColor` (struct :`R` 1.0 :`G` 0.440038 :`A` 1.0)))
  (return (not _returnvalue_2)))

(fn `CheckSpikySide`
  (returns (ReturnValue :type "Float (double-precision)"))
  (return (`KismetMathLibrary.Dot_VectorVector` (`KismetMathLibrary.Normal` (- (`self.K2_GetActorLocation` (`self.As BP Chara Base`)) (`SceneComponent.K2_GetComponentLocation` (`self.SK_Spiky`)))) (`SceneComponent.GetForwardVector` (`self.SK_Spiky`)))))

(fn `Flip`
  (bind (_returnvalue_roll _returnvalue_pitch _returnvalue_yaw) (`KismetMathLibrary.BreakRotator` (`self.K2_GetActorRotation`)))
  (bind _returnvalue (`self.K2_GetActorLocation`))
  (bind (_spawnlocation_x _spawnlocation_y _spawnlocation_z) (`KismetMathLibrary.BreakVector` (`self.SpawnLocation`)))
  (set `self.LocationBeforeFlip` _returnvalue)
  (`self.K2_SetActorLocationAndRotation` (`KismetMathLibrary.MakeVector` (.x _returnvalue) (.y _returnvalue) (+ _spawnlocation_z (`self.FlippedHeight`))) (`KismetMathLibrary.MakeRotator` _returnvalue_roll 180.0 _returnvalue_yaw))
  (set `self.InteractionState` "NewEnumerator3"))

(fn `FlipBack`
  (bind (_returnvalue_roll _returnvalue_pitch _returnvalue_yaw) (`KismetMathLibrary.BreakRotator` (`self.K2_GetActorRotation`)))
  (bind (_spawnlocation_x _spawnlocation_y _spawnlocation_z) (`KismetMathLibrary.BreakVector` (`self.SpawnLocation`)))
  (`self.K2_SetActorLocationAndRotation` (`KismetMathLibrary.MakeVector` (.x (`self.K2_GetActorLocation`)) (.y (`self.K2_GetActorLocation`)) _spawnlocation_z) (`KismetMathLibrary.MakeRotator` _returnvalue_roll 180.0 _returnvalue_yaw))
  (set `self.InteractionState` "NewEnumerator1"))

(fn `InitializeReferences`
  (bind _get_player_ref (message `/Game/Setup/Remi/BPI_Player.Get Player Ref` (`GameplayStatics.GetPlayerCharacter` 0)))
  (set `self.As BP Chara Base` _get_player_ref)
  (bind _get_pc_ref (message `/Game/Interfaces/BPI_PlayerController.Get PC Ref` (`GameplayStatics.GetPlayerController` 0)))
  (set `self.As PC Claws Proto` _get_pc_ref))

(fn `Try Push Spiky`
  (params (HitLocation :type "Vector Structure"))
  (returns (Succeed :type Boolean) (PushDirection :type "Float (double-precision)"))
  (locals (LocalPushDirection :type "Float (double-precision)") (MinimumPushAmount :type "Float (double-precision)" :default 500.0) (PushAmount :type "Float (double-precision)" :default 500.0) (RayHitLocation :type "Vector Structure"))
  (bind _returnvalue_x (`KismetMathLibrary.BreakVector` (`self.K2_GetActorLocation`)))
  (bind _hitlocation_x (`KismetMathLibrary.BreakVector` (`local.HitLocation`)))
  ;[1 1 1] Get push direction
  (bind _output_get (set `local.LocalPushDirection` (`KismetMathLibrary.SelectFloat` -1.0 1.0 (> _hitlocation_x _returnvalue_x))))
  (bind _bcanmove (`self.CanMoveInDirection` _output_get))
  (if _bcanmove
    (bind _output_get_2 (set `self.FromPos` (`self.K2_GetActorLocation`)))
    (set `self.ToPos` (+ _output_get_2 (`KismetMathLibrary.MakeVector` (* (`local.LocalPushDirection`) (`local.PushAmount`)))))
    (set `self.TryingToMove` true)
    (set `self.MovementElapsedTime` 0.0)
    (return false (`local.LocalPushDirection`))
    (else
      (`self.Hide`)
      (set `self.InteractionState` "NewEnumerator1"))))

(fn `UserConstructionScript`
  (`SphereComponent.SetSphereRadius` (`self.HidingZone`) (`self.HideDistance`) true))