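; BP_SpikyCone is a spiky cone in the Enemies set that reacts to Wet and Powered events.
; Wet clears the HabitatedSpike flag.
; Powered acts only while that flag is false, setting pitch to 180 to flip the cone, raising it by FlippedHeightValue and switching its capsule to static mobility.
; Nothing guards against repeats, so each further Powered event raises it again.
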(event `self.ReceiveBeginPlay`)

(event `/Game/Interfaces/BPI_Enemy.Wet`
  (set `self.habitatedSpike` false))

(event `/Game/Interfaces/BPI_Enemy.Powered`
  (bind (_returnvalue_roll _returnvalue_pitch _returnvalue_yaw) (`KismetMathLibrary.BreakRotator` (`self.K2_GetActorRotation`)))
  (if (not (`self.habitatedSpike`))
    (`self.K2_SetActorLocationAndRotation` (`KismetMathLibrary.MakeVector` (.x (`self.K2_GetActorLocation`)) (.y (`self.K2_GetActorLocation`)) (+ (.z (`self.K2_GetActorLocation`)) (`self.FlippedHeightValue`))) (`KismetMathLibrary.MakeRotator` _returnvalue_roll 180.0 _returnvalue_yaw))
    (`SceneComponent.SetMobility` (`self.CapsuleComponent`) "Static")))

(fn `UserConstructionScript`)