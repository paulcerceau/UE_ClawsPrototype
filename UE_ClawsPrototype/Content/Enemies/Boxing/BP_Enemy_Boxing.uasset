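; Boxing enemy that launches the player character upward when the player's capsule overlaps its Box component, acting like a bounce pad.
; A Wet event makes the bounce stronger until a timer clears the state.
; A Powered event halts the enemy's movement and knocks the player along world X with some lift, choosing the sign from whether the player is behind or in front of the enemy's facing.
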(event `self.ReceiveBeginPlay`
  (`parent.ReceiveBeginPlay`)
  (bind _asbp_chara_base (cast `/Game/Setup/BP_CharaBase` (`GameplayStatics.GetPlayerCharacter` 0)))
  (set `self.BP_Chara_Ref` _asbp_chara_base))

(event `self.Box.OnComponentBeginOverlap`
  (params (OverlappedComponent :type "PrimitiveComponent Object Reference") (OtherActor :type "Actor Object Reference") (OtherComp :type "PrimitiveComponent Object Reference") (OtherBodyIndex :type Integer) (bFromSweep :type Boolean) (SweepResult :type "HitResult Structure (by ref)"))
  (if (== OtherComp (`Character.CapsuleComponent` (`self.BP_Chara_Ref`)))
    (if (`self.isWet`)
      (`self.LaunchCharacter` (`self.BP_Chara_Ref`) (0.0 0.0 2650.0) false true)
      (else
        (`self.LaunchCharacter` (`self.BP_Chara_Ref`) (0.0 0.0 2100.0) false true)))))

(event `/Game/Interfaces/BPI_Enemy.Wet`
  (set `self.isWet` true)
  (`KismetSystemLibrary.K2_SetTimerDelegate` (delegate `Event Stop Wet`) (`self.WetDuration`)))

(event `Event Stop Wet`
  (set `self.isWet` false))

(event `/Game/Interfaces/BPI_Enemy.Powered`
  (bind _bp_chara_ref (`self.BP_Chara_Ref`))
  (bind _output_get (set `self.DotProduct` (`KismetMathLibrary.Dot_VectorVector` (`KismetMathLibrary.Normal` (- (`self.K2_GetActorLocation`) (`self.K2_GetActorLocation` (`self.BP_Chara_Ref`)))) (`self.GetActorForwardVector`))))
  (`MovementComponent.StopMovementImmediately` (`self.CharacterMovement`))
  (if (> _output_get 0.0)
    (`self.LaunchCharacter` _bp_chara_ref (1500.0 0.0 500.0) true false)
    (else
      (`self.LaunchCharacter` _bp_chara_ref (-1500.0 0.0 500.0) true false))))

(fn `UserConstructionScript`
  (`parent.UserConstructionScript`))