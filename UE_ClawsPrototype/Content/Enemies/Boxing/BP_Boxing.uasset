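; BP_Boxing is an enemy-folder actor that launches any BP_CharaBase character straight up when it overlaps the actor's Box.
; The launch overrides vertical velocity only and is stronger while the actor is wet.
; A Wet event sets that state and starts a timer that clears it after WetDuration, with debug prints on each change.
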(event `self.Box.OnComponentBeginOverlap`
  (params (OverlappedComponent :type "PrimitiveComponent Object Reference") (OtherActor :type "Actor Object Reference") (OtherComp :type "PrimitiveComponent Object Reference") (OtherBodyIndex :type Integer) (bFromSweep :type Boolean) (SweepResult :type "HitResult Structure (by ref)"))
  (if (`self.isWet`)
    (bind _asbp_chara_base (cast `/Game/Setup/BP_CharaBase` OtherActor))
    (`Character.LaunchCharacter` _asbp_chara_base (0.0 0.0 2650.0) false true)
    (else
      (bind _asbp_chara_base_2 (cast `/Game/Setup/BP_CharaBase` OtherActor))
      (`Character.LaunchCharacter` _asbp_chara_base_2 (0.0 0.0 2100.0) false true))))

(event `/Game/Interfaces/BPI_Enemy.Wet`
  (set `self.isWet` true)
  (`KismetSystemLibrary.PrintString` "iswet")
  (`KismetSystemLibrary.K2_SetTimerDelegate` (delegate `Event Stop Wet`) (`self.WetDuration`)))

(event `Event Stop Wet`
  (set `self.isWet` false)
  (`KismetSystemLibrary.PrintString` "isnotwet"))

(fn `UserConstructionScript`)