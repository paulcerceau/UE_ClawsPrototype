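; BP_Enemy_Spik is an enemy Blueprint that can be flipped over temporarily, guarded by an IsFlipped flag.
; Flip sets the Scene component's world pitch to 180, raises the flag and calls Unflip.
; Unflip waits ten seconds, sets pitch to 180 again using the current roll and yaw, then clears the flag.
; Nothing in this graph triggers Flip, and the construction script only calls the parent.
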(event `Flip`
  (bind _scene (`self.Scene`))
  (bind (_returnvalue_roll _returnvalue_pitch _returnvalue_yaw) (`KismetMathLibrary.BreakRotator` (`SceneComponent.K2_GetComponentRotation` _scene)))
  (if (not (`self.is flipped`))
    (`SceneComponent.K2_SetWorldRotation` _scene (`KismetMathLibrary.MakeRotator` _returnvalue_roll 180.0 _returnvalue_yaw) false false)
    (set `self.is flipped` true)
    (`self.Unflip`)))

(event `Unflip`
  (bind _scene (`self.Scene`))
  (bind (_returnvalue_roll _returnvalue_pitch _returnvalue_yaw) (`KismetMathLibrary.BreakRotator` (`SceneComponent.K2_GetComponentRotation` _scene)))
  (if (`self.is flipped`)
    (`KismetSystemLibrary.Delay` 10.0)
    (`SceneComponent.K2_SetWorldRotation` _scene (`KismetMathLibrary.MakeRotator` _returnvalue_roll 180.0 _returnvalue_yaw) false false)
    (set `self.is flipped` false)))

(fn `UserConstructionScript`
  (`parent.UserConstructionScript`))