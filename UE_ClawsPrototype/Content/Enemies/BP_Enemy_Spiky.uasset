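; BP_Enemy_Spiky is a spiky enemy Blueprint that can be flipped over for a timed period.
; BeginPlay sets the walk speed, caches it as DefaultSpeed and sets a faster AngrySpeed, which this file never uses.
; Flip pitches the Scene component to 180 degrees, sets IsFlipped and calls Unflip.
; After a ten-second delay, Unflip clears the flag but applies the same 180-degree pitch rather than restoring a saved rotation.
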(event `self.ReceiveBeginPlay`
  (bind _output_get (set `CharacterMovementComponent.MaxWalkSpeed` 200.0 (`self.CharacterMovement`)))
  (set `self.Default Speed` _output_get)
  (set `self.Angry Speed` 450.0))

(event `Flip`
  (bind _scene (`self.Scene`))
  (bind (_returnvalue_roll _returnvalue_pitch _returnvalue_yaw) (`KismetMathLibrary.BreakRotator` (`SceneComponent.K2_GetComponentRotation` _scene)))
  (if (not (`self.is flipped`))
    (`SceneComponent.K2_SetWorldRotation` _scene (`KismetMathLibrary.MakeRotator` _returnvalue_roll 180.0 _returnvalue_yaw) false false)
    (set `self.is flipped` true)
    (`self.Unflip`)))

(event `Unflip`
  (bind _scene (`self.Scene`))
  (bind (_returnvalue_roll _returnvalue_pitch _returnvalue_yaw) (`KismetMathLibrary.BreakRotator` (`SceneComponent.K2_GetComponentRotation` _scene)))
  (if (`self.is flipped`)
    (`KismetSystemLibrary.Delay` 10.0)
    (`SceneComponent.K2_SetWorldRotation` _scene (`KismetMathLibrary.MakeRotator` _returnvalue_roll 180.0 _returnvalue_yaw) false false)
    (set `self.is flipped` false)))

(fn `UserConstructionScript`
  (`parent.UserConstructionScript`))