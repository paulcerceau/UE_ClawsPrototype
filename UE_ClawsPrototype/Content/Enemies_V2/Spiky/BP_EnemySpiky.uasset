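; Spiky enemy that knocks back and briefly stuns the player on contact while upright, and reacts to claw powers.
; Power toggles a raised, flipped state; a timer rights it, re-arming while something overlaps its Flipreset volume.
; Water pushes it away from the player along X, unless a line trace finds an obstacle, which makes it hide.
; Player proximity also sets the hiding state.
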(event `self.Hiding distance.OnComponentBeginOverlap`
  (params (OverlappedComponent :type "PrimitiveComponent Object Reference") (OtherActor :type "Actor Object Reference") (OtherComp :type "PrimitiveComponent Object Reference") (OtherBodyIndex :type Integer) (bFromSweep :type Boolean) (SweepResult :type "HitResult Structure (by ref)"))
  ;[1 0.04119 0] Hide (redo)
  (if (`KismetSystemLibrary.DoesImplementInterface` OtherActor "/Game/Setup/Remi/BPI_Player.BPI_Player_C")
    (`self.SpikyHide`)))

(event `self.Flipreset.OnComponentEndOverlap`
  (params (OverlappedComponent :type "PrimitiveComponent Object Reference") (OtherActor :type "Actor Object Reference") (OtherComp :type "PrimitiveComponent Object Reference") (OtherBodyIndex :type Integer))
  ;[1 1 1] Flip/Unflip
  (set `self.bOnSpiky` false))

(event `self.ReceiveBeginPlay`
  ;[1 1 1] BeginPlay
  (`self.InitializeReferences`)
  (set `self.SpawnLocation` (`SceneComponent.K2_GetComponentLocation` (`self.Box`))))

(event `self.Flipreset.OnComponentBeginOverlap`
  (params (OverlappedComponent :type "PrimitiveComponent Object Reference") (OtherActor :type "Actor Object Reference") (OtherComp :type "PrimitiveComponent Object Reference") (OtherBodyIndex :type Integer) (bFromSweep :type Boolean) (SweepResult :type "HitResult Structure (by ref)"))
  ;[1 1 1] Flip/Unflip
  (set `self.bOnSpiky` true)
  (`KismetSystemLibrary.K2_ClearAndInvalidateTimerHandle` (`self.FlipTimer`))
  (`self.CheckFlipBack`))

(event `self.Hiding distance.OnComponentEndOverlap`
  (params (OverlappedComponent :type "PrimitiveComponent Object Reference") (OtherActor :type "Actor Object Reference") (OtherComp :type "PrimitiveComponent Object Reference") (OtherBodyIndex :type Integer))
  ;[1 0.04119 0] Hide (redo)
  (if (`KismetSystemLibrary.DoesImplementInterface` OtherActor "/Game/Setup/Remi/BPI_Player.BPI_Player_C")
    (set `self.Hides` false)))

(event `CheckFlipBack`
  ;[1 1 1] Flip/Unflip
  (bind _returnvalue (`KismetSystemLibrary.K2_SetTimerDelegate` (`|CreateDelegate` :!event `FlipBackOk`) 5.0))
  (set `self.FlipTimer` _returnvalue))

(event `FlipBackOk`
  ;[1 1 1] Flip/Unflip
  (if (`self.bOnSpiky`)
    (`self.CheckFlipBack`)
    (elif (`self.bIsFlipped`)
      (`self.FlipBack`)
      (`SceneComponent.K2_SetWorldLocation` (`self.Box`) (`self.LocationBeforeFlip`) false false))))

(event `/Game/Interfaces/BPI_WetPowered.GetPowered`
  (params (HitLocation :type "Vector Structure"))
  ;[1 1 1] PowerClaw
  (if (`self.bIsFlipped`)
    (`self.FlipBack`)
    (if (not (`self.bOnSpiky`))
      (set `self.bIsFlipped` false)
      (`SceneComponent.K2_SetWorldLocation` (`self.Box`) (`self.LocationBeforeFlip`) false false))
    (else
      (`self.Flip`)
      (set `self.bIsFlipped` true)
      (`self.CheckFlipBack`))))

(event `/Game/Interfaces/BPI_WetPowered.GetWatered`
  (params (HitLocation :type "Vector Structure"))
  ;[1 1 1] WaterClaw
  (if (not (`self.bIsFlipped`))
    (set `self.isWet` true)
    (bind __ (`self.TryPushSpiky`))
    ;;[1 1 1] Pas fan
    (set `self.Push Direction` __)
    (if (and (`self.bOnSpiky`) (`self.bIsFlipped`))
      (`KismetSystemLibrary.Delay` 7.0)
      (`SceneComponent.K2_SetWorldLocation` (`self.Box`) (`self.SpawnLocation`) false false)
      (set `self.isWet` false))))

(event `self.SK_Spiky.OnComponentHit`
  (params (HitComponent :type "PrimitiveComponent Object Reference") (OtherActor :type "Actor Object Reference") (OtherComp :type "PrimitiveComponent Object Reference") (NormalImpulse :type "Vector Structure") (Hit :type "HitResult Structure (by ref)"))
  (bind _returnvalue_x (`KismetMathLibrary.BreakVector` (`self.K2_GetActorLocation` OtherActor)))
  (bind _returnvalue_x_2 (`KismetMathLibrary.BreakVector` (`self.K2_GetActorLocation`)))
  (bind _as_bp_chara_base (`self.As BP Chara Base`))
  ;[1 1 1] Bumping
  (if (and (`KismetSystemLibrary.DoesImplementInterface` OtherActor "/Game/Setup/Remi/BPI_Player.BPI_Player_C") (not (`self.bIsFlipped`)))
    (if (< _returnvalue_x_2 _returnvalue_x)
      (`self.LaunchCharacter` _as_bp_chara_base (1000.0 0.0 1000.0) true true)
      (else
        (`self.LaunchCharacter` (`self.As BP Chara Base`) (-1000.0 0.0 1000.0) true true)))
    (`/Game/Setup/Remi/PC_ClawsProto.Stun` (`self.As PC Claws Proto`) 0.1)
    (`/Game/Setup/Remi/BP_CharaBase.AlterAirMobility` _as_bp_chara_base 0.3 5.0 2.0 0.5)
    (`/Game/Setup/Remi/BP_CharaBase.ResetJump` _as_bp_chara_base 1)))

(fn `CheckSpikySide`
  (returns (ReturnValue :type "Float (double-precision)"))
  (return (`KismetMathLibrary.Dot_VectorVector` (`KismetMathLibrary.Normal` (- (`self.K2_GetActorLocation` (`self.As BP Chara Base`)) (`SceneComponent.K2_GetComponentLocation` (`self.SK_Spiky`)))) (`SceneComponent.GetForwardVector` (`self.SK_Spiky`)))))

(fn `Flip`
  (bind (_returnvalue_roll _returnvalue_pitch _returnvalue_yaw) (`KismetMathLibrary.BreakRotator` (`self.K2_GetActorRotation`)))
  (bind _returnvalue (`self.K2_GetActorLocation`))
  (set `self.LocationBeforeFlip` _returnvalue)
  (`self.K2_SetActorLocationAndRotation` (`KismetMathLibrary.MakeVector` (.x _returnvalue) (.y _returnvalue) (+ (.z _returnvalue) (`self.FlippedHeight`))) (`KismetMathLibrary.MakeRotator` _returnvalue_roll 180.0 _returnvalue_yaw))
  (set `self.bIsFlipped` true))

(fn `FlipBack`
  (bind (_returnvalue_roll _returnvalue_pitch _returnvalue_yaw) (`KismetMathLibrary.BreakRotator` (`self.K2_GetActorRotation`)))
  (`self.K2_SetActorLocationAndRotation` (`KismetMathLibrary.MakeVector` (.x (`self.K2_GetActorLocation`)) (.y (`self.K2_GetActorLocation`)) (- (.z (`self.K2_GetActorLocation`)) (`self.FlippedHeight`))) (`KismetMathLibrary.MakeRotator` _returnvalue_roll 180.0 _returnvalue_yaw))
  (set `self.bIsFlipped` false))

(fn `InitializeReferences`
  (bind _asbp_chara_base (cast `/Game/Setup/Remi/BP_CharaBase` (`GameplayStatics.GetPlayerCharacter` 0)))
  (set `self.As BP Chara Base` _asbp_chara_base)
  (bind _aspc_claws_proto (cast `/Game/Setup/Remi/PC_ClawsProto` (`GameplayStatics.GetPlayerController` 0)))
  (set `self.As PC Claws Proto` _aspc_claws_proto))

(fn `SpikyHide`
  (set `self.Hides` true)
  (set `self.isWet` false))

(fn `TryPushSpiky`
  (returns (` ` :type "Float (double-precision)"))
  (locals (PushDirection :type "Float (double-precision)") (PushAmount :type "Float (double-precision)" :default 5.0))
  (bind _returnvalue_x (`KismetMathLibrary.BreakVector` (`self.K2_GetActorLocation`)))
  (bind _returnvalue (`self.K2_GetActorLocation`))
  (bind _returnvalue_x_2 (`KismetMathLibrary.BreakVector` (`self.K2_GetActorLocation` (`self.As BP Chara Base`))))
  ;[1 1 1] Get push direction
  (set `local.PushDirection` (`KismetMathLibrary.SelectFloat` -1.0 1.0 (> _returnvalue_x_2 _returnvalue_x)))
  ;[1 1 1] Check if there is something behind the Spiky
  (bind (_outhit _returnvalue_2) (`KismetSystemLibrary.LineTraceSingle` _returnvalue (+ _returnvalue (* (`self.GetActorForwardVector`) 115.0 (`local.PushDirection`))) "TraceTypeQuery1"))
  (if _returnvalue_2
    (`self.SpikyHide`)
    (else
      ;[1 1 1] Push only if the ray doesn't collide with anything
      (`self.K2_AddActorWorldOffset` (`KismetMathLibrary.MakeVector` (* (`local.PushDirection`) (`local.PushAmount`))))
      (return (`local.PushDirection`)))))

(fn `UserConstructionScript`)