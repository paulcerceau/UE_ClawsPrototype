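; Boxing enemy that knocks the player and itself apart along X with bumps and blocks, or launches the player upward.
; Tick runs cooldown and wet timers and uses a dot product to detect a player overhead.
; Player on top or wet state swaps side bump zones for the jumper zone; wetness also alters speed and forces.
; Powering flags a block for ApplyBlock, which ends wetness; tuning comes from PDA_BoxingDatas.
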(event `self.ReceiveTick`
  (params (DeltaSeconds :type "Float (single-precision)"))
  (bind _returnvalue (>= (`KismetMathLibrary.Dot_VectorVector` (`KismetMathLibrary.Normal` (- (`self.K2_GetActorLocation` (`self.playerRef`)) (`self.K2_GetActorLocation`))) (`self.GetActorUpVector`)) (- 1.0 (`/Game/Enemies_V2/Boxing/PDA_BoxingDatas.Player On Top Allowance` (`self.BoxingDatas`)))))
  (`|ExecutionSequence`
    (:`then_0`
      (`parent.ReceiveTick` DeltaSeconds))
    (:`then_1`
      ;[1 0.302 0.3137] Cooldown timer
      (if (`self.inCooldown`)
        (bind _output_get (set `self.cooldownTimer` (- (`self.cooldownTimer`) DeltaSeconds)))
        (if (<= _output_get 0.0)
          (`self.CancelBoxingCooldown`)
          (else
            ;[1 0.302 0.3137] Cooldown timer debug print
            (if (`self.EnableDebug`)
              (`KismetSystemLibrary.PrintText` (`|FormatText` "Cooldown timer : {cd}" (`self.cooldownTimer`)) true true (struct :`R` 1.0 :`G` 0.030793 :`A` 1.0) 0.0))))))
    (:`then_2`
      (if (`self.isWet`)
        ;[0.3373 0.5961 1] Wet timer debug print
        (if (`self.EnableDebug`)
          (`KismetSystemLibrary.PrintText` (`|FormatText` "Wet timer : {wet}" (`self.wetTimer`)) true true (struct :`G` 0.182862 :`B` 1.0 :`A` 1.0) 0.0))
        ;[0.3373 0.5961 1] Wet timer
        (bind _output_get_2 (set `self.wetTimer` (- (`self.wetTimer`) DeltaSeconds)))
        (if (<= _output_get_2 0.0)
          (`self.FinishWet`))))
    (:`then_3`
      ;[0.7948 1 0.9181] Compute player on top
      (if (`self.GetRespawning`)
        _
        (elif (`self.GetPlayerDetected`)
          (if (!= _returnvalue (`self.playerOnTop`))
            (set `self.playerOnTop` _returnvalue)
            (`self.UpdateBumpJumpZones`)))))))

(event `self.ReceiveBeginPlay`
  (`|ExecutionSequence`
    (:`then_0`
      (`parent.ReceiveBeginPlay`)
      (bind _aspda_boxing_datas (cast `/Game/Enemies_V2/Boxing/PDA_BoxingDatas` (`self.EnemyDatas`)))
      (set `self.BoxingDatas` _aspda_boxing_datas))
    (:`then_1`
      (`self.UpdateBumpJumpZones`))
    (:`then_2`
      (add `self.OnBeginRespawning` (delegate `BeginRespawn`))
      (add `self.OnEndRespawning` (delegate `EndRespawn`)))))

(event `BeginRespawn`
  (`self.CancelBoxingCooldown`)
  (`self.DisableAllBumpJumpZones`))

(event `EndRespawn`
  (`self.UpdateBumpJumpZones`))

(event `self.BumpRangeLeft.OnComponentBeginOverlap`
  (params (OverlappedComponent :type "PrimitiveComponent Object Reference") (OtherActor :type "Actor Object Reference") (OtherComp :type "PrimitiveComponent Object Reference") (OtherBodyIndex :type Integer) (bFromSweep :type Boolean) (SweepResult :type "HitResult Structure (by ref)"))
  (set `self.playerInBumpLeft` true))

(event `/Game/Interfaces/BPI_WetPowered.GetWatered`
  (if (not (`self.GetRespawning`))
    (`self.StartWet`)))

(event `self.BumpRangeLeft.OnComponentEndOverlap`
  (params (OverlappedComponent :type "PrimitiveComponent Object Reference") (OtherActor :type "Actor Object Reference") (OtherComp :type "PrimitiveComponent Object Reference") (OtherBodyIndex :type Integer))
  (set `self.playerInBumpLeft` false))

(event `/Game/Interfaces/BPI_WetPowered.GetPowered`
  (if (not (`self.GetRespawning`))
    (set `self.blockDetected` true)))

(event `self.BumpRangeRight.OnComponentBeginOverlap`
  (params (OverlappedComponent :type "PrimitiveComponent Object Reference") (OtherActor :type "Actor Object Reference") (OtherComp :type "PrimitiveComponent Object Reference") (OtherBodyIndex :type Integer) (bFromSweep :type Boolean) (SweepResult :type "HitResult Structure (by ref)"))
  (set `self.playerInBumpRight` true))

(event `self.BumpRangeRight.OnComponentEndOverlap`
  (params (OverlappedComponent :type "PrimitiveComponent Object Reference") (OtherActor :type "Actor Object Reference") (OtherComp :type "PrimitiveComponent Object Reference") (OtherBodyIndex :type Integer))
  (set `self.playerInBumpRight` false))

(event `self.JumperZone.OnComponentBeginOverlap`
  (params (OverlappedComponent :type "PrimitiveComponent Object Reference") (OtherActor :type "Actor Object Reference") (OtherComp :type "PrimitiveComponent Object Reference") (OtherBodyIndex :type Integer) (bFromSweep :type Boolean) (SweepResult :type "HitResult Structure (by ref)"))
  (`self.JumpPlayer`))

(fn `ApplyBlock`
  (locals (playerAtLeft :type Boolean))
  (bind _returnvalue_x (`KismetMathLibrary.BreakVector` (`self.K2_GetActorLocation`)))
  (bind _playerref (`self.playerRef`))
  (bind _boxingdatas (`self.BoxingDatas`))
  (bind _iswet (`self.isWet`))
  (bind _iswet_2 (`self.isWet`))
  (bind _boxingdatas_2 (`self.BoxingDatas`))
  (bind _boxingdatas_3 (`self.BoxingDatas`))
  (bind _returnvalue_x_2 (`KismetMathLibrary.BreakVector` (`self.K2_GetActorLocation` (`self.playerRef`))))
  (set `self.blockDetected` false)
  (set `local.playerAtLeft` (< _returnvalue_x_2 _returnvalue_x))
  (set `self.playerInBumpRight` false)
  (set `self.playerInBumpLeft` false)
  (`self.LaunchCharacter` _playerref (`KismetMathLibrary.MakeVector` (* (`KismetMathLibrary.SelectFloat` -1.0 1.0 (`local.playerAtLeft`)) (`KismetMathLibrary.SelectFloat` (`/Game/Enemies_V2/Boxing/PDA_BoxingDatas.Block Player Force X Wet` _boxingdatas_3) (`/Game/Enemies_V2/Boxing/PDA_BoxingDatas.Block Player Force X` _boxingdatas_3) _iswet_2)) 0.0 (`KismetMathLibrary.SelectFloat` (`/Game/Enemies_V2/Boxing/PDA_BoxingDatas.Block Player Force Z Wet` _boxingdatas_3) (`/Game/Enemies_V2/Boxing/PDA_BoxingDatas.Block Player Force Z` _boxingdatas_3) _iswet_2)) true true)
  (`/Game/Setup/Remi/BP_CharaBase.AlterAirMobility` _playerref (`/Game/Enemies_V2/Boxing/PDA_BoxingDatas.Block Player Air Control` _boxingdatas) (`/Game/Enemies_V2/Boxing/PDA_BoxingDatas.Block Player Falling Lateral Friction` _boxingdatas) (`/Game/Enemies_V2/Boxing/PDA_BoxingDatas.Block Player Braking Friction` _boxingdatas))
  (`self.LaunchCharacter` (`KismetMathLibrary.MakeVector` (* (`KismetMathLibrary.SelectFloat` 1.0 -1.0 (`local.playerAtLeft`)) (`KismetMathLibrary.SelectFloat` (`/Game/Enemies_V2/Boxing/PDA_BoxingDatas.Block Self Force X Wet` _boxingdatas_2) (`/Game/Enemies_V2/Boxing/PDA_BoxingDatas.Block Self Force X` _boxingdatas_2) _iswet)) 0.0 (`KismetMathLibrary.SelectFloat` (`/Game/Enemies_V2/Boxing/PDA_BoxingDatas.Block Self Force Z Wet` _boxingdatas_2) (`/Game/Enemies_V2/Boxing/PDA_BoxingDatas.Block Self Force Z` _boxingdatas_2) _iswet)) true true)
  (`self.FinishWet`))

(fn `BumpPlayer`
  (bind _playerref (`self.playerRef`))
  (bind _boxingdatas (`self.BoxingDatas`))
  (bind _boxingdatas_2 (`self.BoxingDatas`))
  (bind _boxingdatas_3 (`self.BoxingDatas`))
  (`self.LaunchCharacter` _playerref (`KismetMathLibrary.MakeVector` (* (`KismetMathLibrary.SelectFloat` -1.0 1.0 (`self.playerInBumpLeft`)) (`/Game/Enemies_V2/Boxing/PDA_BoxingDatas.Bumper Player Force X` _boxingdatas)) 0.0 (`/Game/Enemies_V2/Boxing/PDA_BoxingDatas.Bumper Player Force Z` _boxingdatas)) true true)
  (`/Game/Setup/Remi/BP_CharaBase.AlterAirMobility` _playerref (`/Game/Enemies_V2/Boxing/PDA_BoxingDatas.Bumper Player Air Control` _boxingdatas_3) (`/Game/Enemies_V2/Boxing/PDA_BoxingDatas.Bumper Player Falling Lateral Friction` _boxingdatas_3) (`/Game/Enemies_V2/Boxing/PDA_BoxingDatas.Bumper Player Braking Friction` _boxingdatas_3))
  (`self.LaunchCharacter` (`KismetMathLibrary.MakeVector` (* (`KismetMathLibrary.SelectFloat` 1.0 -1.0 (`self.playerInBumpLeft`)) (`/Game/Enemies_V2/Boxing/PDA_BoxingDatas.Bumper Self Force X` _boxingdatas_2)) 0.0 (`/Game/Enemies_V2/Boxing/PDA_BoxingDatas.Bumper Self Force Z` _boxingdatas_2)) true true))

(fn `CancelBoxingCooldown`
  (set `self.cooldownTimer` 0.0)
  (set `self.inCooldown` false))

(fn `DisableAllBumpJumpZones`
  (`PrimitiveComponent.SetCollisionEnabled` (`self.JumperZone`) "NoCollision")
  (`PrimitiveComponent.SetCollisionEnabled` (`self.BumpRangeRight`) "NoCollision")
  (`PrimitiveComponent.SetCollisionEnabled` (`self.BumpRangeLeft`) "NoCollision")
  (if (`self.EnableDebug`)
    (`SceneComponent.SetHiddenInGame` (`self.JumperZone`) true false)
    (`SceneComponent.SetHiddenInGame` (`self.BumpRangeLeft`) true false)
    (`SceneComponent.SetHiddenInGame` (`self.BumpRangeRight`) true false)))

(fn `FinishWet`
  (set `self.wetTimer` 0.0)
  (set `self.isWet` false)
  (`self.UpdateWalkSpeed`)
  (`self.UpdateBumpJumpZones`))

(fn `GetBlockDetected`
  (returns (BlockDetected :type Boolean))
  (return (`self.blockDetected`)))

(fn `GetEnemyCooldown`
  (returns (inCooldown :type Boolean))
  (return (`self.inCooldown`)))

(fn `GetPlayerInBump`
  (returns (PlayerInBump :type Boolean))
  (return (or (`self.playerInBumpLeft`) (`self.playerInBumpRight`))))

(fn `GetPlayerOnTop`
  (returns (PlayerOnTop :type Boolean))
  (return (and (`self.GetPlayerDetected`) (`self.playerOnTop`))))

(fn `GetWet`
  (returns (IsWet :type Boolean))
  (return (`self.isWet`)))

(fn `JumpPlayer`
  (bind _boxingdatas (`self.BoxingDatas`))
  (`self.LaunchCharacter` (`self.playerRef`) (`KismetMathLibrary.MakeVector` 0.0 0.0 (`KismetMathLibrary.SelectFloat` (`/Game/Enemies_V2/Boxing/PDA_BoxingDatas.Jumper Player Force Z Wet` _boxingdatas) (`/Game/Enemies_V2/Boxing/PDA_BoxingDatas.Jumper Player Force Z` _boxingdatas) (`self.isWet`))) false true))

(fn `SetChaseState`
  (params (Value :type Boolean))
  (set `self.isChasing` Value)
  (`self.UpdateWalkSpeed`))

(fn `StartBoxingCooldown`
  (params (CooldownTime :type "Float (double-precision)"))
  (if (not (`self.GetRespawnStarted`))
    (set `self.cooldownTimer` CooldownTime)
    (set `self.inCooldown` true)))

(fn `StartWet`
  (set `self.isWet` true)
  (set `self.wetTimer` (`/Game/Enemies_V2/Boxing/PDA_BoxingDatas.WetDuration` (`self.BoxingDatas`)))
  (`self.UpdateWalkSpeed`)
  (`self.UpdateBumpJumpZones`))

(fn `UpdateBumpJumpZones`
  (bind _returnvalue (or (`self.GetPlayerOnTop`) (`self.isWet`)))
  (bind _returnvalue_2 (or (`self.GetPlayerOnTop`) (`self.isWet`)))
  (bind _returnvalue_3 (select `bool` _returnvalue_2 :`false` "QueryAndPhysics" :`true` "NoCollision" :!type "ECollisionEnabled Enum"))
  (if (not (`self.GetRespawning`))
    (`PrimitiveComponent.SetCollisionEnabled` (`self.JumperZone`) (select `bool` _returnvalue_2 :`false` "NoCollision" :`true` "QueryAndPhysics" :!type "ECollisionEnabled Enum"))
    (`PrimitiveComponent.SetCollisionEnabled` (`self.BumpRangeRight`) _returnvalue_3)
    (`PrimitiveComponent.SetCollisionEnabled` (`self.BumpRangeLeft`) _returnvalue_3)
    (if (`self.EnableDebug`)
      (`SceneComponent.SetHiddenInGame` (`self.JumperZone`) (not _returnvalue) false)
      (`SceneComponent.SetHiddenInGame` (`self.BumpRangeLeft`) _returnvalue false)
      (`SceneComponent.SetHiddenInGame` (`self.BumpRangeRight`) _returnvalue false))))

(fn `UpdateWalkSpeed`
  (bind _boxingdatas (`self.BoxingDatas`))
  (set `CharacterMovementComponent.MaxWalkSpeed` (`KismetMathLibrary.SelectFloat` (`KismetMathLibrary.SelectFloat` (`/Game/Enemies_V2/Boxing/PDA_BoxingDatas.Chase Speed Wet` _boxingdatas) (`/Game/Enemies_V2/Boxing/PDA_BoxingDatas.Chase Speed` _boxingdatas) (`self.isWet`)) (`KismetMathLibrary.SelectFloat` (`/Game/Enemies_V2/Boxing/PDA_BoxingDatas.Patrol Speed Wet` _boxingdatas) (`/Game/Enemies_V2/Boxing/PDA_BoxingDatas.Patrol Speed` _boxingdatas) (`self.isWet`)) (`self.isChasing`)) (`self.CharacterMovement`)))

(fn `UserConstructionScript`
  (`parent.UserConstructionScript`))