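; Speedy enemy that grabs a player who enters its range from above, then throws them opposite its facing direction.
; An overlap arms claw spheres on hand sockets; a claw hit attaches and stuns the player and switches the camera.
; LaunchPlayer releases and launches the player, restores the camera and starts a cooldown.
; Watered and powered overrides of the parent enemy disable grab collisions until each state finishes.
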(event `self.ReceiveBeginPlay`
  ;[0.8824 0.9294 0.2275] BEGIN PLAY
  (`|ExecutionSequence`
    (:`then_0`
      (`self.SetEnemyData` (`self.SpeedyData`))
      (`parent.ReceiveBeginPlay`))
    (:`then_1`
      (`SceneComponent.K2_AttachToComponent` (`self.LeftClawSphere`) (`self.Mesh`) (`self.LeftClawSocketName`) "KeepRelative" "KeepWorld" "KeepWorld" false)
      (`SceneComponent.K2_AttachToComponent` (`self.RightClawSphere`) (`self.Mesh`) (`self.RightClawSocketName`) "KeepRelative" "KeepWorld" "KeepWorld" false)
      (`self.SetClawsCollisionsEnable` "NoCollision"))
    (:`then_2`
      (`self.SetDirectionInt` (`KismetMathLibrary.SelectInt` -1 1 (> (`self.InitialThrowDirection`) 0.0))))))

(event `self.ReceiveTick`
  (params (DeltaSeconds :type "Float (single-precision)"))
  ;[0.9294 0.2275 0.2275] EVENT TICK
  (`|ExecutionSequence`
    (:`then_0`
      (`parent.ReceiveTick` DeltaSeconds))))

(event `BeginRespawn`
  ;[1 1 1] Respawn
  (`parent.BeginRespawn`))

(event `EndRespawn`
  ;[1 1 1] Respawn
  (`parent.EndRespawn`))

(event `/Game/Interfaces/BPI_WetPowered.GetWatered`
  (params (HitLocation :type "Vector Structure"))
  ;[1 1 1] Watered/Powered
  (`parent.GetWatered` (0.0 0.0 0.0))
  (`self.SetAllCollisionsEnable` "NoCollision")
  (`NiagaraFunctionLibrary.SpawnSystemAttached` "/Game/ART_Vfx/Niagara/Systeme/NS_Droplets_Expulsed.NS_Droplets_Expulsed" (`self.Mesh`) "None" (0.0 0.0 0.0) (struct) "KeepRelativeOffset")
  (set `self.bIsInGrabSequence` false))

(event `/Game/Interfaces/BPI_WetPowered.GetPowered`
  (params (HitLocation :type "Vector Structure"))
  (bind _returnvalue_x (`KismetMathLibrary.BreakVector` (`self.K2_GetActorLocation`)))
  (bind _returnvalue_x_2 (`KismetMathLibrary.BreakVector` (`self.K2_GetActorLocation` (`self.playerRef`))))
  (bind (_poweredvector_x _poweredvector_y _poweredvector_z) (`KismetMathLibrary.BreakVector` (`/Game/Enemies_V2/Speedy/PDA_SpeedyData.PoweredVector` (`self.SpeedyData`))))
  ;[1 1 1] Watered/Powered
  (`parent.GetPowered` (0.0 0.0 0.0))
  (`self.SetAllCollisionsEnable` "NoCollision")
  (set `self.bIsInGrabSequence` false)
  (`self.LaunchCharacter` (`KismetMathLibrary.MakeVector` (* (`KismetMathLibrary.SelectFloat` 1.0 -1.0 (> _returnvalue_x_2 _returnvalue_x)) _poweredvector_x) _poweredvector_y _poweredvector_z) true true)
  (`AkGameplayStatics.PostEvent` "/Game/WwiseAudio/Events/Work_Unit_Elise_Events/Speedy/Play_SPEEDY_Powerclaw.Play_SPEEDY_Powerclaw" (`self.CharaBase`)))

(event `ReleaseSpeedy`
  ;[1 1 1] Triggered in ABP_Speedy, after wet to idle transition
)

(event `self.OnGroundGrabRange.OnComponentBeginOverlap`
  (params (OverlappedComponent :type "PrimitiveComponent Object Reference") (OtherActor :type "Actor Object Reference") (OtherComp :type "PrimitiveComponent Object Reference") (OtherBodyIndex :type Integer) (bFromSweep :type Boolean) (SweepResult :type "HitResult Structure (by ref)"))
  (bind (_returnvalue_x _returnvalue_y _returnvalue_z) (`KismetMathLibrary.BreakVector` (`self.K2_GetActorLocation` OtherActor)))
  (bind (_returnvalue_x_2 _returnvalue_y_2 _returnvalue_z_2) (`KismetMathLibrary.BreakVector` (`SceneComponent.K2_GetComponentLocation` (`self.Mesh`))))
  ;[1 1 1] When Player within grab range (enters "OnGroundGrabRange")
  (if (and (`KismetSystemLibrary.DoesImplementInterface` OtherActor "/Game/Setup/Remi/BPI_Player.BPI_Player_C") (not (`self.Get Is Respawning`)) (not (`self.bIsInGrabSequence`)) (not (`self.inCooldown`)) (not (`self.Get Is Powered`)) (not (`self.GetIsWet`)))
    ;;[1 1 1] Make sure Speedies can't grab the Player if they're under them
    (if (> _returnvalue_z _returnvalue_z_2)
      (set `self.GrabStep` "NewEnumerator0")
      (set `self.bIsInGrabSequence` true)
      (`self.SetClawsCollisionsEnable` "QueryOnly"))))

(event `self.LeftClawSphere.OnComponentBeginOverlap`
  (params (OverlappedComponent :type "PrimitiveComponent Object Reference") (OtherActor :type "Actor Object Reference") (OtherComp :type "PrimitiveComponent Object Reference") (OtherBodyIndex :type Integer) (bFromSweep :type Boolean) (SweepResult :type "HitResult Structure (by ref)"))
  ;[1 1 1] Claw grab
  (`self.Try Attach Player` OtherActor))

(event `self.RightClawSphere.OnComponentBeginOverlap`
  (params (OverlappedComponent :type "PrimitiveComponent Object Reference") (OtherActor :type "Actor Object Reference") (OtherComp :type "PrimitiveComponent Object Reference") (OtherBodyIndex :type Integer) (bFromSweep :type Boolean) (SweepResult :type "HitResult Structure (by ref)"))
  ;[1 1 1] Claw grab
  (`self.Try Attach Player` OtherActor true))

(event `LaunchPlayer`
  (bind (_camerasettingsbeforegrabbing_distance _camerasettingsbeforegrabbing_angle _camerasettingsbeforegrabbing_horizontaloffset _camerasettingsbeforegrabbing_verticaloffset) (break `/Game/Setup/Camera/SCameraSettings` (`self.CameraSettingsBeforeGrabbing`)))
  (bind _camera (`/Game/Setup/Remi/BP_CharaBase.Camera` (`self.playerRef`)))
  ;[1 1 1] Launch Player
  (if (`|EnumEquality` (`self.GrabStep`) "NewEnumerator1")
    (`self.ExitGrabSequence`)
    ;;[1 1 1] Reverse back to AdvancedFollow Camera mode
    (`/Game/Setup/Camera/BP_Camera.ChangeCameraSettings` _camera (make `/Game/Setup/Camera/SCameraSettings` _camerasettingsbeforegrabbing_distance _camerasettingsbeforegrabbing_angle _camerasettingsbeforegrabbing_horizontaloffset _camerasettingsbeforegrabbing_verticaloffset) "NewEnumerator8" 0.5 (0.0 0.0))
    (`/Game/Setup/Camera/BP_Camera.Switch Camera Mode` _camera "NewEnumerator0" 0.5)
    (`self.K2_DetachFromActor` (`self.playerRef`) "KeepWorld" "KeepWorld" "KeepWorld")
    (`CharacterMovementComponent.SetMovementMode` (`Character.CharacterMovement` (`self.playerRef`)) "MOVE_Walking" 0)
    (`self.K2_SetActorRotation` :`self` (`self.playerRef`))
    (`self.SetThrowDirection`)
    (`self.LaunchCharacter` (`self.playerRef`) (* (`/Game/Enemies_V2/Speedy/PDA_SpeedyData.ThrowVector` (`self.SpeedyData`)) (`KismetMathLibrary.MakeVector` (`self.ThrowDirection`) 1.0 1.0)) true true)
    (`/Game/Setup/Remi/PC_ClawsProto.Unstun` (`/Game/Setup/Remi/BP_CharaBase.PC_Ref` (`self.playerRef`)))
    (`/Game/Setup/Remi/BP_CharaBase.ResetJump` (`self.playerRef`) 1)
    (`self.Start Cooldown` (`self.Cooldown Time`))
    (else
      (`self.ExitGrabSequence`))))

(fn `ExitGrabSequence`
  (set `self.GrabStep` "NewEnumerator3")
  (set `self.bIsInGrabSequence` false)
  (set `self.bGrabbedPlayer` false)
  (`self.SetClawsCollisionsEnable` "NoCollision"))

(fn `FinishPowered`
  (`parent.FinishPowered`)
  (`self.SetGrabCollisionEnable` "QueryOnly"))

(fn `FinishWet`
  (`AkGameplayStatics.PostEventAtLocation` "/Game/WwiseAudio/Events/Work_Unit_Elise_Events/Speedy/Play_SPEEDY_Transition_Wet_Dry.Play_SPEEDY_Transition_Wet_Dry" (`SceneComponent.K2_GetComponentLocation` (`self.Mesh`)))
  (`parent.FinishWet`)
  (`self.K2_SetActorRotation` (struct))
  (`self.SetGrabCollisionEnable` "QueryOnly")
  (`self.Start Cooldown` 2.0))

(fn `GetIsInGrabSequence`
  (returns (` ` :type Boolean))
  (return (`self.bIsInGrabSequence`)))

(fn `SetAllCollisionsEnable`
  (params (` ` :type "ECollisionEnabled Enum" :default "NoCollision"))
  (`self.SetClawsCollisionsEnable` ` `)
  (`self.SetGrabCollisionEnable` ` `))

(fn `SetClawsCollisionsEnable`
  (params (` ` :type "ECollisionEnabled Enum" :default "NoCollision"))
  (`PrimitiveComponent.SetCollisionEnabled` (`self.LeftClawSphere`) ` `)
  (`PrimitiveComponent.SetCollisionEnabled` (`self.RightClawSphere`) ` `))

(fn `SetGrabCollisionEnable`
  (params (NewType :type "ECollisionEnabled Enum" :default "NoCollision"))
  (`PrimitiveComponent.SetCollisionEnabled` (`self.OnGroundGrabRange`) NewType))

(fn `SetIsInGrabSequence`
  (params (` ` :type Boolean))
  (set `self.bIsInGrabSequence` ` `))

(fn `SetThrowDirection`
  ;[1 1 1] Can be more complex by adding modes like in the previous speedy
  (set `self.ThrowDirection` (* (`self.GetDirectionInt`) -1.0))
  (return))

(fn `Try Attach Player`
  (params (OtherActor :type "Object Object Reference (by ref)") (bIsRightClaw :type Boolean :default false))
  (returns (Succeed :type Boolean))
  (bind _playerref (`self.playerRef`))
  (bind _camera (`/Game/Setup/Remi/BP_CharaBase.Camera` (`self.playerRef`)))
  ;[1 1 1] Can grab ?
  (if (and (`KismetSystemLibrary.DoesImplementInterface` (`local.OtherActor`) "/Game/Setup/Remi/BPI_Player.BPI_Player_C") (`|EnumEquality` (`self.GrabStep`) "NewEnumerator0") (not (`self.bIsTestingClawCollision`)))
    (set `self.bIsTestingClawCollision` true)
    ;[1 1 1] Try attach Player to corresponding Speedy's Claw
    (bind _returnvalue (`self.K2_AttachToComponent` (`self.playerRef`) (`self.Mesh`) (select `bool` (`local.bIsRightClaw`) :`false` "L_T_HAND_SKN" :`true` "R_T_HAND_SKN" :!type "Name") "SnapToTarget" "KeepWorld" "KeepWorld" false))
    (if _returnvalue
      (set `self.GrabStep` "NewEnumerator1")
      (`/Game/Setup/Remi/PC_ClawsProto.Stun` (`/Game/Setup/Remi/BP_CharaBase.PC_Ref` (`self.playerRef`)) 0.0)
      ;[1 1 1] If the Player is grabbed while wall walking
      (if (`|EnumEquality` (`/Game/Setup/Remi/BP_CharaBase.CurrentMovementComponent` (`self.playerRef`)) "NewEnumerator1")
        (`/Game/Setup/Remi/PC_ClawsProto.ExitWallRideState` (`/Game/Setup/Remi/BP_CharaBase.PC_Ref` _playerref))
        (`/Game/Setup/Remi/BP_CharaBase.Set Current Movement Component` _playerref "NewEnumerator0"))
      (`CharacterMovementComponent.DisableMovement` (`Character.CharacterMovement` (`self.playerRef`)))
      ;[1 1 1] Change camera mode to "StrictFollow" to avoid weird Camera movements
      (`/Game/Setup/Camera/BP_Camera.Switch Camera Mode` _camera "NewEnumerator8" 0.5)
      (bind _output_get (set `self.CameraSettingsBeforeGrabbing` (`/Game/Setup/Camera/BP_Camera.CameraSettings` _camera)))
      (`/Game/Setup/Camera/BP_Camera.ChangeCameraSettings` _camera (make `/Game/Setup/Camera/SCameraSettings` (break `/Game/Setup/Camera/SCameraSettings` _output_get) (`.Angle_9_523D90C842C62DECA09DD5853C25C402` (break `/Game/Setup/Camera/SCameraSettings` _output_get))) "NewEnumerator8" 0.5 (0.0 0.0))
      (`self.SetClawsCollisionsEnable` "NoCollision")
      (set `self.bGrabbedPlayer` true)
      (set `self.bIsTestingClawCollision` false)
      (return true)
      (else
        (`self.ExitGrabSequence`)
        (set `self.bIsTestingClawCollision` false)
        (return false)))
    (else
      (return false))))

(fn `UserConstructionScript`
  (`parent.UserConstructionScript`))