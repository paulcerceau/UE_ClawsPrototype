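; Base enemy character that supplies shared detection, status and respawn logic, tuned through EnemyData.
; A detection sphere gates a per-tick line trace to the player; sightings widen its radius and refresh a lose-detection timer.
; Tick countdowns drive waiting, animation-block, cooldown, wet and powered states, with chase and wet selecting walk speed.
; Respawn uses timed dig-down, teleport and dig-up phases with begin/end dispatchers, while EnableDebug shows state.
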(event `self.ReceiveBeginPlay`
  (bind _playerdetection (`self.PlayerDetection`))
  (`|ExecutionSequence`
    (:`then_0`
      ;[1 0.8314 0.9137] Setup PlayerDetection sphere
      (`SphereComponent.SetSphereRadius` _playerdetection (`/Game/Enemies_V2/Common/PDA_EnemyData.Patrol Detection Range` (`self.EnemyData`)) true)
      (`SceneComponent.SetHiddenInGame` _playerdetection (not (`self.EnableDebug`)) false))
    (:`then_1`
      ;[0.7166 0.8299 1] Get Player ref
      (bind _get_player_ref (message `/Game/Setup/Remi/BPI_Player.Get Player Ref` (`GameplayStatics.GetPlayerCharacter` 0)))
      (set `self.playerRef` _get_player_ref))
    (:`then_2`
      ;[1 1 1] Bind Events
      (add `self.OnBeginRespawning` (`|CreateDelegate` :!event `BeginRespawn`))
      (add `self.OnEndRespawning` (`|CreateDelegate` :!event `EndRespawn`)))
    (:`then_3`
      ;[1 1 1] Set initial values
      (`self.UpdateWalkSpeed`))))

(event `self.ReceiveTick`
  (params (DeltaSeconds :type "Float (single-precision)"))
  (set `self.Delta Seconds` DeltaSeconds)
  (`|ExecutionSequence`
    (:`then_0`
      ;[1 1 1] Timers
      ;;[0.8078 1 0.8431] Waiting timer
      (if (`self.enemyWaiting`)
        (bind _output_get (set `self.waitingTimer` (- (`self.waitingTimer`) (`self.Delta Seconds`))))
        (if (<= _output_get 0.0)
          (`self.CancelEnemyWaiting`)
          (else
            ;;[0.8078 1 0.8431] Waiting timer debug print
            (if (`self.EnableDebug`)
              (`KismetSystemLibrary.PrintText` (`|FormatText` "Waiting timer : {wait}" (`self.waitingTimer`)) true true (struct :`R` 0.034841 :`G` 1.0 :`B` 0.297234 :`A` 1.0) 0.0))))))
    (:`then_1`
      ;;[1 0.5176 0.6275] Movement blocked by anim timer
      (if (`self.movementBlockedByAnim`)
        (bind _output_get_2 (set `self.animBlockTimer` (- (`self.animBlockTimer`) (`self.Delta Seconds`))))
        (if (<= _output_get_2 0.0)
          (`self.CancelBlockMovementForAnim`)
          (else
            ;;[1 0.5176 0.6275] Movement blocked by anim timer debug print
            (if (`self.EnableDebug`)
              (`KismetSystemLibrary.PrintText` (`|FormatText` "Movements blocked by anim timer: {timer}" (`self.animBlockTimer`)) true true (struct :`R` 1.0 :`B` 0.439424 :`A` 1.0) 0.0))))))
    (:`then_2`
      ;;[1 0.302 0.3137] Cooldown timer
      (if (`self.inCooldown`)
        (bind _output_get_3 (set `self.cooldownTimer` (- (`self.cooldownTimer`) (`self.Delta Seconds`))))
        (if (<= _output_get_3 0.0)
          (`self.Cancel Cooldown`)
          (else
            ;;[1 0.302 0.3137] Cooldown timer debug print
            (if (`self.EnableDebug`)
              (`KismetSystemLibrary.PrintText` (`|FormatText` "Cooldown timer : {cd}" (`self.cooldownTimer`)) true true (struct :`R` 1.0 :`G` 0.030793 :`A` 1.0) 0.0))))))
    (:`then_3`
      ;;[0.3373 0.5961 1] Wet timer
      (if (`self.bIsWet`)
        (bind _output_get_4 (set `self.wetTimer` (- (`self.wetTimer`) (`self.Delta Seconds`))))
        (if (<= _output_get_4 0.0)
          (`self.FinishWet`)
          (else
            ;;[0.3373 0.5961 1] Wet timer debug print
            (if (`self.EnableDebug`)
              (`KismetSystemLibrary.PrintText` (`|FormatText` "Wet timer : {wet}" (`self.wetTimer`)) true true (struct :`G` 0.182862 :`B` 1.0 :`A` 1.0) 0.0))))))
    (:`then_4`
      (if (`self.bIsPowered`)
        (bind _output_get_5 (set `self.PoweredTimer` (- (`self.PoweredTimer`) (`self.Delta Seconds`))))
        (if (<= _output_get_5 0.0)
          (`self.FinishPowered`)
          (elif (`self.EnableDebug`)
            (`KismetSystemLibrary.PrintText` (`|FormatText` "Powered timer : {powered}" (`self.PoweredTimer`)) true true (struct :`G` 0.182862 :`B` 1.0 :`A` 1.0) 0.0)))))
    (:`then_5`
      (`|ExecutionSequence`
        (:`then_0`
          (if (`self.playerInRange`)
            (set `self.playerOnSight` false)
            ;[0.6196 1 0.7647] Raycast
            (bind _outhit (`KismetSystemLibrary.LineTraceSingle` :`Start` (`self.K2_GetActorLocation`) :`End` (`self.K2_GetActorLocation` (`self.playerRef`)) :`TraceChannel` "TraceTypeQuery1" :`DrawDebugType` (select `bool` (`self.EnableDebug`) :`true` "ForOneFrame" :!type "EDrawDebugTrace Enum") :`TraceColor` (struct :`G` 1.0 :`A` 1.0) :`TraceHitColor` (struct :`R` 1.0 :`A` 1.0) :`DrawTime` 0.0))
            (if (`KismetSystemLibrary.DoesImplementInterface` (`.HitActor` (`GameplayStatics.BreakHitResult` _outhit)) "/Game/Setup/Remi/BPI_Player.BPI_Player_C")
              (set `self.playerDetected` true)
              ;[1 0.651 0.949] Reset lose detection timer
              (set `self.loseDetectionTimer` (`/Game/Enemies_V2/Common/PDA_EnemyData.Lose Detection Time` (`self.EnemyData`)))
              (set `self.playerOnSight` true)
              ;[1 0.8314 0.9137] Change detection range
              (`SphereComponent.SetSphereRadius` (`self.PlayerDetection`) (`/Game/Enemies_V2/Common/PDA_EnemyData.Chase Detection Range` (`self.EnemyData`)) true)
              (else
                ;[0.6196 1 0.7647] Raycast debug print
                (if (`self.EnableDebug`)
                  (`KismetSystemLibrary.PrintString` "Player is in range and in front of the enemy, but there is something between them." true true (struct :`R` 0.950309 :`G` 1.0 :`B` 0.054318 :`A` 1.0) 0.0))))))
        (:`then_1`
          ;[0.4792 0.4792 1] Player detected debug print
          (if (`self.playerDetected`)
            (if (`self.EnableDebug`)
              (`KismetSystemLibrary.PrintString` "Player detected" true true (struct :`R` 0.230435 :`G` 0.352381 :`B` 1.0 :`A` 1.0) 0.0))))
        (:`then_2`
          (if (`self.playerDetected`)
            (`|ExecutionSequence`
              (:`then_0`
                ;[1 0.651 0.949] Lose detection timer debug print
                (if (`self.EnableDebug`)
                  (`KismetSystemLibrary.PrintText` (`|FormatText` "Lose detection timer: {timer}" (`self.loseDetectionTimer`)) true true (struct :`R` 1.0 :`G` 0.306216 :`B` 0.784323 :`A` 1.0) 0.0)))
              (:`then_1`
                ;[1 0.651 0.949] Decrease lose detection timer
                (bind _output_get_6 (set `self.loseDetectionTimer` (- (`self.loseDetectionTimer`) (`self.Delta Seconds`))))
                (if (<= _output_get_6 0.0)
                  (set `self.playerDetected` false)
                  ;[1 0.8314 0.9137] Change detection range
                  (`SphereComponent.SetSphereRadius` (`self.PlayerDetection`) (`/Game/Enemies_V2/Common/PDA_EnemyData.Patrol Detection Range` (`self.EnemyData`)) true))))))))
    (:`then_6`
      ;[1 0.5318 0.452] Respawning debug print
      (if (`self.EnableDebug`)
        (if (`self.bIsRespawning`)
          (`KismetSystemLibrary.PrintString` "Respawning..." true true (struct :`R` 1.0 :`G` 0.116213 :`A` 1.0) 0.0))))))

(event `BeginRespawn`
  ;[1 1 1] Respawn
  (`self.Cancel Cooldown`))

(event `EndRespawn`
  ;[1 1 1] Respawn
)

(event `self.PlayerDetection.OnComponentBeginOverlap`
  (params (OverlappedComponent :type "PrimitiveComponent Object Reference") (OtherActor :type "Actor Object Reference") (OtherComp :type "PrimitiveComponent Object Reference") (OtherBodyIndex :type Integer) (bFromSweep :type Boolean) (SweepResult :type "HitResult Structure (by ref)"))
  (set `self.playerInRange` true))

(event `self.PlayerDetection.OnComponentEndOverlap`
  (params (OverlappedComponent :type "PrimitiveComponent Object Reference") (OtherActor :type "Actor Object Reference") (OtherComp :type "PrimitiveComponent Object Reference") (OtherBodyIndex :type Integer))
  (set `self.playerInRange` false)
  (set `self.playerOnSight` false))

(event `/Game/Interfaces/BPI_WetPowered.GetWatered`
  (params (HitLocation :type "Vector Structure"))
  ;[1 1 1] Get Watered
  (if (not (`self.bIsRespawning`))
    (`self.StartWet`)))

(event `/Game/Interfaces/BPI_WetPowered.GetPowered`
  (params (HitLocation :type "Vector Structure"))
  ;[1 1 1] Get Powered
  (if (not (`self.bIsRespawning`))
    (`self.StartPowered`)))

(fn `ApplyRespawn`
  (`self.K2_SetActorLocation` (`self.respawnLocation`) false true)
  (`KismetSystemLibrary.K2_SetTimer` null "FinishRespawn" (`/Game/Enemies_V2/Common/PDA_EnemyData.Respawn Dig Up Time` (`self.EnemyData`))) ; Time so that the enemy return to patrol state when the dig up animation is finished
)

(fn `Cancel Cooldown`
  (set `self.cooldownTimer` 0.0)
  (set `self.inCooldown` false))

(fn `CancelBlockMovementForAnim`
  (set `self.animBlockTimer` 0.0)
  (set `self.movementBlockedByAnim` false))

(fn `CancelEnemyWaiting`
  (set `self.waitingTimer` 0.0)
  (set `self.enemyWaiting` false))

(fn `FinishPowered`
  (set `self.PoweredTimer` 0.0)
  (set `self.bIsPowered` false)
  (`self.UpdateWalkSpeed`))

(fn `FinishRespawn`
  (set `self.bIsRespawning` false)
  (`self.OnEndRespawning`))

(fn `FinishWet`
  (set `self.wetTimer` 0.0)
  (set `self.bIsWet` false)
  (`self.UpdateWalkSpeed`))

(fn `Get Is Powered`
  (returns (` ` :type Boolean))
  (return (`self.bIsPowered`)))

(fn `Get Is Respawning`
  (returns (` ` :type Boolean))
  (return (`self.bIsRespawning`)))

(fn `GetChaseState`
  (returns (` ` :type Boolean))
  (return (`self.bIsChasing`)))

(fn `GetDirectionInt`
  (returns (`Direction Int` :type Integer))
  (return (`self.Direction Int`)))

(fn `GetEnemyCooldown`
  (returns (inCooldown :type Boolean))
  (return (`self.inCooldown`)))

(fn `GetEnemyWaiting`
  (returns (Waiting :type Boolean))
  (return (`self.enemyWaiting`)))

(fn `GetIsWet`
  (returns (` ` :type Boolean))
  (return (`self.bIsWet`)))

(fn `GetMovementBlockedByAnim`
  (returns (Blocked :type Boolean))
  (return (`self.movementBlockedByAnim`)))

(fn `GetPlayerDetected`
  (returns (` ` :type Boolean))
  (return (`self.playerDetected`)))

(fn `GetPlayerOnSight`
  (returns (PlayerOnSight :type Boolean))
  (return (`self.playerOnSight`)))

(fn `GetPlayerPosition`
  (returns (PlayerPos :type "Vector Structure"))
  (return (`self.K2_GetActorLocation` (`self.playerRef`))))

(fn `GetRespawnStarted`
  (returns (RespawnStarted :type Boolean))
  (return (`self.respawn_started`)))

(fn `ResetRespawnStarted`
  (set `self.respawn_started` false))

(fn `SetChaseState`
  (params (Value :type Boolean))
  (set `self.bIsChasing` Value)
  (`self.UpdateWalkSpeed`))

(fn `SetDirectionInt`
  (params (`Direction Int` :type Integer))
  (set `self.Direction Int` `Direction Int`))

(fn `SetEnemyData`
  (params (` ` :type "/Game/Enemies_V2/Common/PDA_EnemyData Object Reference"))
  (set `self.EnemyData` ` `))

(fn `SetIsPowered`
  (params (` ` :type Boolean))
  (set `self.bIsPowered` ` `))

(fn `SetIsWet`
  (params (` ` :type Boolean))
  (set `self.bIsWet` ` `))

(fn `Start Cooldown`
  (params (CooldownTime :type "Float (double-precision)"))
  (if (not (`self.GetRespawnStarted`))
    (set `self.cooldownTimer` CooldownTime)
    (set `self.inCooldown` true)))

(fn `StartEnemyWaiting`
  (set `self.waitingTimer` (`/Game/Enemies_V2/Common/PDA_EnemyData.Patrol Waiting Time` (`self.EnemyData`)))
  (set `self.enemyWaiting` true))

(fn `StartPowered`
  (set `self.bIsPowered` true)
  (set `self.PoweredTimer` (`/Game/Enemies_V2/Common/PDA_EnemyData.PoweredDuration` (`self.EnemyData`))))

(fn `StartWet`
  (set `self.bIsWet` true)
  (set `self.wetTimer` (`/Game/Enemies_V2/Boxing/PDA_BoxingData.WetDuration` (`self.EnemyData`)))
  (`self.UpdateWalkSpeed`))

(fn `TriggerBlockMovementForAnim`
  (params (BlockTime :type "Float (double-precision)"))
  (set `self.animBlockTimer` BlockTime)
  (set `self.movementBlockedByAnim` true))

(fn `TriggerRespawn`
  (params (RespawnLocation :type "Vector Structure"))
  (set `self.respawnLocation` RespawnLocation)
  (set `self.bIsRespawning` true)
  (set `self.respawn_started` true)
  (`KismetSystemLibrary.K2_SetTimer` null "ApplyRespawn" (`/Game/Enemies_V2/Common/PDA_EnemyData.Respawn Dig Down Time` (`self.EnemyData`))) ; Time so that respawn apply when the dig down animation is finished
  (`self.OnBeginRespawning`))

(fn `UpdateWalkSpeed`
  (bind _enemydata (`self.EnemyData`))
  (set `CharacterMovementComponent.MaxWalkSpeed` (`KismetMathLibrary.SelectFloat` (`KismetMathLibrary.SelectFloat` (`/Game/Enemies_V2/Boxing/PDA_BoxingData.Chase Speed Wet` _enemydata) (`/Game/Enemies_V2/Boxing/PDA_BoxingData.Chase Speed` _enemydata) (`self.bIsWet`)) (`KismetMathLibrary.SelectFloat` (`/Game/Enemies_V2/Boxing/PDA_BoxingData.Patrol Speed Wet` _enemydata) (`/Game/Enemies_V2/Boxing/PDA_BoxingData.Patrol Speed` _enemydata) (`self.bIsWet`)) (`self.bIsChasing`)) (`self.CharacterMovement`)))

(fn `UserConstructionScript`)