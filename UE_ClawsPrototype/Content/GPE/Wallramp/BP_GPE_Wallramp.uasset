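; Wall ramp gameplay element that signals when the player is on it, marked as a tentative wall-walk feature.
; BeginPlay caches the player character and controller through interface messages.
; CollisionBox1 overlaps with the player's capsule call EnterRamp and ExitRamp on the controller, which holds the ramp behavior.
; The construction script positions and rotates RotationCenter and moves the text label to match one of four diagonal Orientation values.
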(event `self.ReceiveBeginPlay`
  (bind _get_player_ref (message `/Game/Setup/BPI_Player.Get Player Ref` (`GameplayStatics.GetPlayerCharacter` 0)))
  (set `self.PlayerCharacter Ref` _get_player_ref)
  (bind _get_pc_ref (message `/Game/Interfaces/BPI_PlayerController.Get PC Ref` (`GameplayStatics.GetPlayerController` 0)))
  (set `self.PlayerController Ref` _get_pc_ref))

(event `self.CollisionBox1.OnComponentBeginOverlap`
  (params (OverlappedComponent :type "PrimitiveComponent Object Reference") (OtherActor :type "Actor Object Reference") (OtherComp :type "PrimitiveComponent Object Reference") (OtherBodyIndex :type Integer) (bFromSweep :type Boolean) (SweepResult :type "HitResult Structure (by ref)"))
  ;[1 1 1] tentative wallwalk
  (if (== OtherComp (`Character.CapsuleComponent` (`self.PlayerCharacter Ref`)))
    (`/Game/Setup/PC_ClawsProto.EnterRamp` (`self.PlayerController Ref`))))

(event `self.CollisionBox1.OnComponentEndOverlap`
  (params (OverlappedComponent :type "PrimitiveComponent Object Reference") (OtherActor :type "Actor Object Reference") (OtherComp :type "PrimitiveComponent Object Reference") (OtherBodyIndex :type Integer))
  ;[1 1 1] tentative wallwalk
  (if (== OtherComp (`Character.CapsuleComponent` (`self.PlayerCharacter Ref`)))
    (`/Game/Setup/PC_ClawsProto.ExitRamp` (`self.PlayerController Ref`))))

(fn `SetOrientation`
  (bind _rotationcenter (`self.RotationCenter`))
  (bind _textrender (`self.TextRender`))
  (switch `/Game/GPE/Wallramp/ECardinalOrientation` (`self.Orientation`)
    (:`NewEnumerator0`
      (`SceneComponent.K2_SetRelativeLocationAndRotation` :`self` _rotationcenter :`NewLocation` (0.0 0.0 50.0))
      (`SceneComponent.K2_SetRelativeLocation` _textrender (-60.0 0.0 120.0) false false))
    (:`NewEnumerator1`
      (`SceneComponent.K2_SetRelativeLocationAndRotation` _rotationcenter (0.0 0.0 50.0) (struct :`Pitch` -90.0) false false)
      (`SceneComponent.K2_SetRelativeLocation` _textrender (60.0 0.0 120.0) false false))
    (:`NewEnumerator2`
      (`SceneComponent.K2_SetRelativeLocationAndRotation` _rotationcenter (0.0 0.0 -50.0) (struct :`Yaw` 180.0 :`Roll` 180.0) false false)
      (`SceneComponent.K2_SetRelativeLocation` _textrender (60.0 0.0 -120.0) false false))
    (:`NewEnumerator3`
      (`SceneComponent.K2_SetRelativeLocationAndRotation` _rotationcenter (0.0 0.0 -50.0) (struct :`Pitch` 90.0) false false)
      (`SceneComponent.K2_SetRelativeLocation` _textrender (-60.0 0.0 -120.0) false false))))

(fn `UserConstructionScript`
  (`self.SetOrientation`))