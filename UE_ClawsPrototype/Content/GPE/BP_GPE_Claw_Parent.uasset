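; Parent Blueprint for claw pickups that the player collects by walking into them.
; On begin play it caches the player character reference through an interface message.
; When the player's capsule overlaps, it passes itself to the claw prototype player controller's FindClaw, then destroys itself.
; UseClaw only prints the claw name, GetPincePowerRef is empty, and a character ObtainClaw call with mesh and material is left unconnected.
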(event `self.ReceiveBeginPlay`
  (bind _get_player_ref (message `/Game/Setup/BPI_Player.Get Player Ref` (`GameplayStatics.GetPlayerCharacter` 0)))
  (set `self.PlayerCharacter Ref` _get_player_ref))

(event `self.Capsule.OnComponentBeginOverlap`
  (params (OverlappedComponent :type "PrimitiveComponent Object Reference") (OtherActor :type "Actor Object Reference") (OtherComp :type "PrimitiveComponent Object Reference") (OtherBodyIndex :type Integer) (bFromSweep :type Boolean) (SweepResult :type "HitResult Structure (by ref)"))
  (if (== OtherComp (`Character.CapsuleComponent` (`self.PlayerCharacter Ref`)))
    (bind _aspc_claws_proto (cast `/Game/Setup/PC_ClawsProto` (`GameplayStatics.GetPlayerController` 0)))
    (`/Game/Setup/PC_ClawsProto.Find claw` _aspc_claws_proto self)
    (`self.K2_DestroyActor`)))

(fn `Get PincePower Ref`
  (returns (`Get Power Pince` :type "/Game/GPE/BP_GPE_Claw_Power Object Reference"))
  (return null))

(fn `UseClaw`
  (`KismetSystemLibrary.PrintString` (`KismetStringLibrary.Concat_StrStr` "Using: " (`self.Name`))))

(fn `UserConstructionScript`)