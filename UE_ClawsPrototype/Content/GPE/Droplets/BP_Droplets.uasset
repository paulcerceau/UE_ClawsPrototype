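; BP_Droplets is a Niagara water drip emitter that waters objects below it.
; On BeginPlay it registers itself as the Niagara export callback, receiving particle data.
; Each particle position triggers a short downward line trace; hits play a Wwise drop sound and notify BPI_WetPowered actors with the hit location, a potentially costly per-particle approach.
; A tutorial sequence event sets the drip frequency parameter.
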(event `self.ReceiveBeginPlay`
  ;[0.8824 0.9294 0.2275] BEGIN PLAY
  (`NiagaraComponent.SetNiagaraVariableObject` (`self.NS_Drops`) "User.BPCallback" self))

(event `self.ReceiveParticleData`
  (params (Data :type "Array of BasicParticleData Structure (by ref)") (NiagaraSystem :type "NiagaraSystem Object Reference") (SimulationPositionOffset :type "Vector Structure (by ref)"))
  ;[1 1 1] Watchout for performances. If it takes too much, do it with a simple ray trace
  (for _array_element Data
    (bind _position (break `BasicParticleData` _array_element))
    (bind (_outhit _returnvalue) (`KismetSystemLibrary.LineTraceSingle` _position (- _position (0.0 0.0 100.0)) "TraceTypeQuery1"))
    (if _returnvalue
      (`AkGameObject.PostAssociatedAkEvent` :`self` (`self.Ak_Play_DropWater`))
      (bind (_bblockinghit _binitialoverlap _time _distance _location _impactpoint _normal _impactnormal _physmat _hitactor) (`GameplayStatics.BreakHitResult` _outhit))
      (if (`KismetSystemLibrary.DoesImplementInterface` _hitactor "/Game/Interfaces/BPI_WetPowered.BPI_WetPowered_C")
        (message `/Game/Interfaces/BPI_WetPowered.GetWatered` _hitactor _location)))))

(event `SeqTutoPissou_Frequency`
  (`FXSystemComponent.SetFloatParameter` (`self.NS_Drops`) "User.Frequency" 8.0))

(fn `UserConstructionScript`)