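; Power Claw component that sends a "powered" message to the enemy or GPE hit in front of its owner.
; On BeginPlay it reads its range from the claw data asset, which it also exposes through GetPDAClaw.
; ActivateClaw line-traces forward, ignoring the player, and messages the hit actor via BPI_Enemy or, failing that, BPI_GPE.
; Enemy hits play the on sound, GPE hits play none here, and anything else plays the off sound.
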(event `self.ReceiveBeginPlay`
  (`parent.ReceiveBeginPlay`)
  (set `self.Range` (`/Game/GPE/Claws/Data/PDA_PowerClaw.Range` (`self.Datas`))))

(fn `ActivateClaw`
  (bind _hit_actor (`self.Hit Actor`))
  (bind _outhit (`/Game/Utilities/BPFL.Forward Lign Trace` (`self.GetOwner`) (`self.Range`) (`|MakeArray` (`GameplayStatics.GetPlayerCharacter` 0) :!type "Actor Object Reference") "ForDuration"))
  ;[1 1 1] Flip enemy
  (bind _output_get (set `self.Hit Actor` (`.HitActor` (`GameplayStatics.BreakHitResult` _outhit))))
  (if (`KismetSystemLibrary.DoesImplementInterface` _output_get "/Game/Interfaces/BPI_Enemy.BPI_Enemy_C")
    (`GameplayStatics.PlaySound2D` "/Game/SoundDesign/Sounds/PowerClawOn_Cue.PowerClawOn_Cue" 1.0 1.0 0.0 null null)
    (message `/Game/Interfaces/BPI_Enemy.Powered` _hit_actor)
    (elif (`KismetSystemLibrary.DoesImplementInterface` (`self.Hit Actor`) "/Game/Interfaces/BPI_GPE.BPI_GPE_C")
      (message `/Game/Interfaces/BPI_GPE.GPE_Powered` _hit_actor)
      (else
        (`GameplayStatics.PlaySound2D` "/Game/SoundDesign/Sounds/PowerClawOff_Cue.PowerClawOff_Cue" 1.0 1.0 0.0 null null)))))

(fn `DetectionLineTrace`
  (params (Range :type "Float (double-precision)") (ActorsToIgnore :type "Array of Actor Object Reference (by ref)"))
  (returns (OutHit :type "HitResult Structure"))
  (return))

(fn `GetPDAClaw`
  (returns (`PDA Claw` :type "/Game/GPE/Claws/Data/PDA_Claw Object Reference"))
  (return (`self.Datas`)))