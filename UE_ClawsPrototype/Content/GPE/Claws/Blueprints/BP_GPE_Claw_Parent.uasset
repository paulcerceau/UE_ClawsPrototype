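; Base Blueprint for claw pickups that hover and spin in the level until the player collects one.
; Two timelines drive the motion: a looping yaw rotation and a vertical bob that alternates direction after a delay.
; When the player's capsule overlaps the box, the claw passes itself to PC_ClawsProto's FindClaw, then destroys itself.
; UseClaw only prints the claw's name, and the component and power getters are empty stubs.
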(event `self.ReceiveTick`
  (params (DeltaSeconds :type "Float (single-precision)"))
  ;[0.9294 0.2275 0.2275] EventTick
)

(event `self.ReceiveBeginPlay`
  ;[0.8824 0.9294 0.2275] BeginPlay
  (bind _get_player_ref (message `/Game/Setup/BPI_Player.Get Player Ref` (`GameplayStatics.GetPlayerCharacter` 0)))
  (set `self.PlayerCharacter Ref` _get_player_ref)
  (set `self.BaseLocation` (`self.K2_GetActorLocation`))
  (`TimelineComponent.SetPlayRate` (`self.Hovering`) (/ 1.0 (`self.HoveringLength`)))
  (`self.Hover` true)
  (`TimelineComponent.SetPlayRate` (`self.Rotating`) (/ 1.0 (`self.TimePerRevolution`)))
  (`self.Rotate`))

(event `Rotate`
  (bind (_returnvalue_roll _returnvalue_pitch) (`KismetMathLibrary.BreakRotator` (`self.K2_GetActorRotation`)))
  (bind (_direction _curve_rotate_float) (`Timeline|Rotating` :!via `PlayFromStart`)
    (:`Update`
      (`self.K2_SetActorRotation` (`KismetMathLibrary.MakeRotator` _returnvalue_roll _returnvalue_pitch (`KismetMathLibrary.Lerp` 0.0 360.0 _curve_rotate_float))))
    (:`Finished`
      (`self.Rotate`))))

(event `Hover`
  (params (bUp :type Boolean))
  ;[1 1 1] Hover
  (if bUp
    (bind (_direction _curve_clawhovering_float) (`Timeline|Hovering` :!via `PlayFromStart` :!label _label)
      (:`Update`
        (`self.SetHoveringLocation` _curve_clawhovering_float))
      (:`Finished`
        (`KismetSystemLibrary.Delay` (`self.DelayBetweenTwoHover`))
        (`self.Hover` (not bUp))))
    (else
      (goto _label :!via `ReverseFromEnd`))))

(event `self.Box.OnComponentBeginOverlap`
  (params (OverlappedComponent :type "PrimitiveComponent Object Reference") (OtherActor :type "Actor Object Reference") (OtherComp :type "PrimitiveComponent Object Reference") (OtherBodyIndex :type Integer) (bFromSweep :type Boolean) (SweepResult :type "HitResult Structure (by ref)"))
  ;[1 1 1] Pick claw
  (if (== OtherComp (`Character.CapsuleComponent` (`self.PlayerCharacter Ref`)))
    (bind _aspc_claws_proto (cast `/Game/Setup/PC_ClawsProto` (`GameplayStatics.GetPlayerController` 0)))
    (`/Game/Setup/PC_ClawsProto.Find claw` _aspc_claws_proto self)
    (`self.K2_DestroyActor`)))

(fn `Get PincePower Ref`
  (returns (`Get Power Pince` :type "/Game/GPE/Claws/Blueprints/BP_GPE_Claw_Power Object Reference"))
  (return null))

(fn `GetAcCe`
  (returns (`Claw effect` :type "/Game/GPE/Claws/Blueprints/AC_ClawEffect Object Reference"))
  (`KismetSystemLibrary.PrintString` "Parent doesn't have an AC_CE")
  (return null))

(fn `SetHoveringLocation`
  (params (Alpha :type "Float (double-precision)"))
  (bind (_baselocation_x _baselocation_y _baselocation_z) (`KismetMathLibrary.BreakVector` (`self.BaseLocation`)))
  (`self.K2_SetActorLocation` (`KismetMathLibrary.MakeVector` _baselocation_x _baselocation_y (+ (`KismetMathLibrary.Lerp` 0.0 (`self.HoveringHeight`) Alpha) _baselocation_z))))

(fn `UseClaw`
  (`KismetSystemLibrary.PrintString` (`KismetStringLibrary.Concat_StrStr` "Using: " (`self.Name`))))

(fn `UserConstructionScript`)