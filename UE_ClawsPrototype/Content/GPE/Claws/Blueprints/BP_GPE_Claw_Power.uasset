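; BP_GPE_Claw_Power is the power variant of the claw gameplay element, built on a parent claw class.
; It delegates behavior to its ACCEPowerClaw component, whose common data supplies the skeletal mesh applied in the construction script.
; UseClaw runs the parent logic, then activates that component.
; Two getters expose the actor itself and the component.
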(fn `Get PincePower Ref`
  (returns (`Get Power Pince` :type "/Game/GPE/Claws/Blueprints/BP_GPE_Claw_Power Object Reference"))
  (return self))

(fn `GetAcCe`
  (returns (`Claw effect` :type "/Game/GPE/Claws/Blueprints/AC_ClawEffect Object Reference"))
  (return (`self.AC_CE_PowerClaw`)))

(fn `UseClaw`
  (`parent.UseClaw`)
  (`/Game/GPE/Claws/Blueprints/AC_ClawEffect.ActivateClaw` :`self` (`self.AC_CE_PowerClaw`)))

(fn `UserConstructionScript`
  (bind (_commondata_classtoinstanciate _commondata_linktoactor _commondata_mesh) (break `/Game/GPE/Claws/Data/SClaw` (`/Game/GPE/Claws/Data/PDA_Claw.CommonData` (`/Game/GPE/Claws/Blueprints/AC_CE_PowerClaw.Datas` (`self.AC_CE_PowerClaw`)))))
  (`parent.UserConstructionScript`)
  (`SkinnedMeshComponent.SetSkinnedAssetAndUpdate` (`self.SK_Claw`) _commondata_mesh true))