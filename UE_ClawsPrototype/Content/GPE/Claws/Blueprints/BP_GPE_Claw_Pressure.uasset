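; Pressure variant of the claw GPE actor, built around its ACCEPressureClaw component.
; The construction script applies the skeletal mesh from that component's common data to SKClaw.
; GetAcCe exposes the component, while GetPincePowerRef returns no value.
; BeginPlay calls the parent, then prints a debug angle in degrees, computed by arccosine of distance ratios between the NinetyAngle, LeftMost and TopMost markers.
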(event `self.ReceiveBeginPlay`
  (bind _returnvalue (`SceneComponent.K2_GetComponentLocation` (`self.LeftMost`)))
  (`parent.ReceiveBeginPlay`)
  (`KismetSystemLibrary.PrintString` (`KismetStringLibrary.Conv_DoubleToString` (`KismetMathLibrary.DegAcos` (/ (`KismetMathLibrary.Vector_Distance` (`SceneComponent.K2_GetComponentLocation` (`self.NinetyAngle`)) _returnvalue) (`KismetMathLibrary.Vector_Distance` _returnvalue (`SceneComponent.K2_GetComponentLocation` (`self.TopMost`))))))))

(fn `Get PincePower Ref`
  (returns (`Get Power Pince` :type "/Game/GPE/Claws/Blueprints/BP_GPE_Claw_Power Object Reference"))
  (return null))

(fn `GetAcCe`
  (returns (`Claw effect` :type "/Game/GPE/Claws/Blueprints/AC_ClawEffect Object Reference"))
  (return (`self.AC_CE_PressureClaw`)))

(fn `UserConstructionScript`
  (bind (_commondata_classtoinstanciate _commondata_linktoactor _commondata_mesh) (break `/Game/GPE/Claws/Data/SClaw` (`/Game/GPE/Claws/Data/PDA_Claw.CommonData` (`/Game/GPE/Claws/Blueprints/AC_CE_PressureClaw.Datas` (`self.AC_CE_PressureClaw`)))))
  (`parent.UserConstructionScript`)
  (`SkinnedMeshComponent.SetSkinnedAssetAndUpdate` (`self.SK_Claw`) _commondata_mesh true))