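; Power claw component that, when activated, flips spiky enemies the player targets.
; ActivateClaw prints a debug string, then calls DetectionLineTrace with a short range, ignoring the player character.
; A hit actor that implements BPI_Enemy and is exactly a BP_Enemy_Spiky gets Flip called on it.
; DetectionLineTrace has an empty body in this asset, and BeginPlay and Tick are disabled.
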(fn `ActivateClaw`
  (`KismetSystemLibrary.PrintString` "Power")
  (bind _outhit (`self.DetectionLineTrace` 300.0 (`|MakeArray` (`GameplayStatics.GetPlayerCharacter` 0) :!type "Actor Object Reference")))
  (bind (_bblockinghit _binitialoverlap _time _distance _location _impactpoint _normal _impactnormal _physmat _hitactor) (`GameplayStatics.BreakHitResult` _outhit))
  (if (`KismetSystemLibrary.DoesImplementInterface` _hitactor "/Game/Interfaces/BPI_Enemy.BPI_Enemy_C")
    (if (== (`GameplayStatics.GetObjectClass` _hitactor) "/Game/Enemies/BP_Enemy_Spiky.BP_Enemy_Spiky_C")
      (bind _asbp_enemy_spiky (cast `/Game/Enemies/BP_Enemy_Spiky` _hitactor))
      (`/Game/Enemies/BP_Enemy_Spiky.Flip` _asbp_enemy_spiky))))

(fn `DetectionLineTrace`
  (params (Range :type "Float (double-precision)") (ActorsToIgnore :type "Array of Actor Object Reference (by ref)"))
  (returns (OutHit :type "HitResult Structure"))
  (return))