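; Guard NPC that shows a speech bubble when the player enters its trigger box and opens a double door if they possess the mustache.
; The mustache disables movement, then stuns the player, fades the screen, rotates the doors and plays the opening sequence.
; A looping timer watches for sequence completion to refresh the bubble once with end-game content.
; Externally triggered events restore control, flash a timed bubble and load the outro level.
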(event `self.ReceiveBeginPlay`
  ;[1 1 1] BeginPlay
  (bind _asbp_chara_base (cast `/Game/Setup/Remi/BP_CharaBase` (`GameplayStatics.GetPlayerCharacter` 0)))
  (set `self.As BP Chara Base` _asbp_chara_base)
  (bind _asgm_claws_proto (cast `/Game/Setup/GM_ClawsProto` (`GameplayStatics.GetGameMode`)))
  (set `self.As GM Claws Proto` _asgm_claws_proto)
  (bind _aspc_claws_proto (cast `/Game/Setup/Remi/PC_ClawsProto` (`GameplayStatics.GetPlayerController` 0)))
  (set `self.As PC Claws Proto` _aspc_claws_proto))

(event `self.TB_Bubble.OnComponentBeginOverlap`
  (params (OverlappedComponent :type "PrimitiveComponent Object Reference") (OtherActor :type "Actor Object Reference") (OtherComp :type "PrimitiveComponent Object Reference") (OtherBodyIndex :type Integer) (bFromSweep :type Boolean) (SweepResult :type "HitResult Structure (by ref)"))
  ;[1 1 1] In TBox show dialog, outside don't + if mustache launch sequencer
  ;;[1 1 1] On Overlap launch Bubble F
  (if (`KismetSystemLibrary.DoesImplementInterface` OtherActor "/Game/Setup/Remi/BPI_Player.BPI_Player_C")
    (`self.Bubble`)
    (set `self.InGuardSight` true)
    (bind _returnvalue (`KismetSystemLibrary.K2_SetTimerDelegate` (delegate `CheckStateChanges`) 0.1 true))
    (set `self.InGuardSightTimer` _returnvalue)))

(event `Bubble`
  (bind _wb_dialog (`self.WB_Dialog`))
  ;[1 1 1] In TBox show dialog, outside don't + if mustache launch sequencer
  ;;[1 1 1] Set Bubble Dialog aspect & show
  (bind _aswb_guard_bubble (cast `/Game/UI/WB_GuardBubble` (`WidgetComponent.GetUserWidgetObject` (`self.WB_Dialog`))))
  (if (`self.DoorOpeningSeqPlayed`)
    (`/Game/UI/WB_GuardBubble.BubbleEndGame` _aswb_guard_bubble)
    (`SceneComponent.SetVisibility` _wb_dialog true false)
    (else
      (`/Game/UI/WB_GuardBubble.BubbleAsset` _aswb_guard_bubble)
      (`SceneComponent.SetVisibility` _wb_dialog true false)
      (if (`/Game/Setup/Remi/BP_CharaBase.bPossessMustache` (`self.As BP Chara Base`))
        (`CharacterMovementComponent.DisableMovement` (`Character.CharacterMovement` (`self.As BP Chara Base`)))
        (`KismetSystemLibrary.Delay` 0.8)
        (`self.DoorOpeningSequencer`)))))

(event `CheckStateChanges`
  ;[1 1 1] In TBox show dialog, outside don't + if mustache launch sequencer
  ;;[1 1 1] On Overlap launch Bubble F
  (if (`self.DoorOpeningSeqPlayed`)
    (`/Engine/EditorBlueprintResources/StandardMacros.DoOnce` false
      (:`Completed`
        (`self.Bubble`)))))

(event `self.TB_Bubble.OnComponentEndOverlap`
  (params (OverlappedComponent :type "PrimitiveComponent Object Reference") (OtherActor :type "Actor Object Reference") (OtherComp :type "PrimitiveComponent Object Reference") (OtherBodyIndex :type Integer))
  ;[1 1 1] In TBox show dialog, outside don't + if mustache launch sequencer
  ;;[1 1 1] On End Overlap hide dialog
  (if (`KismetSystemLibrary.DoesImplementInterface` OtherActor "/Game/Setup/Remi/BPI_Player.BPI_Player_C")
    (`SceneComponent.SetVisibility` (`self.WB_Dialog`) false false)
    (set `self.InGuardSight` false)
    (`KismetSystemLibrary.K2_ClearAndInvalidateTimerHandle` (`self.InGuardSightTimer`))))

(event `DoorOpeningSequencer`
  (bind _wb_blackbg (`/Game/Setup/GM_ClawsProto.WB_BlackBG` (`self.As GM Claws Proto`)))
  ;[1 1 1] In TBox show dialog, outside don't + if mustache launch sequencer
  ;;[1 1 1] Launch Sequencer
  (`SceneComponent.SetVisibility` (`self.WB_Dialog`) false false)
  (set `/Game/Setup/Remi/PC_ClawsProto.bIsStun` true (`self.As PC Claws Proto`))
  (`UserWidget.AddToViewport` _wb_blackbg 0)
  (`/Game/UI/WB_BlackBG.Fading_InOut` _wb_blackbg)
  (`KismetSystemLibrary.Delay` 1.0)
  (`SceneComponent.K2_SetRelativeRotation` (`self.DoorLeft`) (struct :`Yaw` -60.0) false false)
  (`SceneComponent.K2_SetRelativeRotation` (`self.DoorRight`) (struct :`Yaw` 60.0) false false)
  (`LevelSequencePlayer.CreateLevelSequencePlayer` "/Game/Cinematics/Sequences/Seq_DoorOpening.Seq_DoorOpening" (make `MovieSceneSequencePlaybackSettings` true (struct) 1.0 0.0 false false true true true true)))

(event `DoorOpeningSequencerFinished`
  ;[1 1 1] In TBox show dialog, outside don't + if mustache launch sequencer
  ;;[1 1 1] Launch Sequencer
  (set `self.DoorOpeningSeqPlayed` true)
  (`CharacterMovementComponent.SetMovementMode` (`Character.CharacterMovement` (`self.As BP Chara Base`)) "MOVE_Walking" 0)
  (set `/Game/Setup/Remi/PC_ClawsProto.bIsStun` false (`self.As PC Claws Proto`)))

(event `OpenOutroCinematic`
  ;[1 1 1] In TBox show dialog, outside don't + if mustache launch sequencer
  ;;[1 1 1] Launch Sequencer
  (`GameplayStatics.OpenLevel` "Lv_CinematicOutro"))

(event `DisplayBubbleArseneSeq`
  (bind _wb_dialog (`self.WB_Dialog`))
  (bind _aswb_guard_bubble (cast `/Game/UI/WB_GuardBubble` (`WidgetComponent.GetUserWidgetObject` (`self.WB_Dialog`))))
  (`/Game/UI/WB_GuardBubble.BubbleAsset` _aswb_guard_bubble)
  (`SceneComponent.SetVisibility` _wb_dialog true false)
  (`KismetSystemLibrary.Delay` 2.0)
  (`SceneComponent.SetVisibility` _wb_dialog false false))

(fn `UserConstructionScript`)