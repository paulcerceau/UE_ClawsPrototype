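; Moving platform variant that travels continuously along a path, built on a parent platform Blueprint.
; On each Move event it runs the parent logic, then samples the TargetLocations spline in local space at the elapsed time using constant velocity.
; MoveComponentTo interpolates the platform mesh to that point over the update period, leaving its rotation unchanged.
; End handling and construction defer entirely to the parent.
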(event `self.Move`
  (bind _platformmesh (`self.PlatformMesh`))
  (`parent.Move`)
  (`KismetSystemLibrary.MoveComponentTo` _platformmesh (`SplineComponent.GetLocationAtTime` (`self.TargetLocations`) (`self.ElapsedTime`) "Local" true) (`SceneComponent.RelativeRotation` _platformmesh) false false (`self.UpdatePeriod`)))

(event `self.ReachEnd`
  (`parent.ReachEnd`))

(fn `UserConstructionScript`
  (`parent.UserConstructionScript`))