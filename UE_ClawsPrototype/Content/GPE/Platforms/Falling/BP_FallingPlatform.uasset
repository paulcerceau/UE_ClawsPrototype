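; BP_FallingPlatform is a leaf platform that folds away shortly after a player touches it, then respawns.
; Idle wobble plays one of two timelines at random, forward or reversed, on the Leaf1 morph target.
; A BPI_Player overlap starts a timer and tints the dynamic material through its Substract parameter as a warning.
; Falling drives the morph fully and disables collision; timed respawn reverses morph and tint, restores collision and resumes wobbling.
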(event `self.ReceiveBeginPlay`
  (`self.Giggle`))

(event `Giggle`
  (switch `int` (select `int` (`KismetMathLibrary.RandomIntegerInRange` 0 3) :`0` 0 :`1` 1 :`2` 2 :`3` 3)
    (:`0`
      (bind (_direction _alpha) (`Timeline|Anim1` :!via `PlayFromStart` :!label _label)
        (:`Update`
          (`SkeletalMeshComponent.SetMorphTarget` (`self.LeafPlatform`) "Leaf1" (`KismetMathLibrary.Lerp` 0.0 0.1 _alpha) true))))
    (:`1`
      (goto _label :!via `ReverseFromEnd`))
    (:`2`
      (bind (_direction_2 _alpha_2) (`Timeline|Anim2` :!via `PlayFromStart` :!label _label_2)
        (:`Update`
          (`SkeletalMeshComponent.SetMorphTarget` (`self.LeafPlatform`) "Leaf1" (`KismetMathLibrary.Lerp` 0.0 0.1 _alpha_2) true))))
    (:`3`
      (goto _label_2 :!via `ReverseFromEnd`))))

(event `StopLoop`
  (`|ExecutionSequence`
    (:`then_0`
      (goto _label :!via `Stop`))
    (:`then_1`
      (goto _label_2 :!via `Stop`))))

(event `self.Box.OnComponentBeginOverlap`
  (params (OverlappedComponent :type "PrimitiveComponent Object Reference") (OtherActor :type "Actor Object Reference") (OtherComp :type "PrimitiveComponent Object Reference") (OtherBodyIndex :type Integer) (bFromSweep :type Boolean) (SweepResult :type "HitResult Structure (by ref)"))
  (if (`KismetSystemLibrary.DoesImplementInterface` OtherActor "/Game/Setup/Remi/BPI_Player.BPI_Player_C")
    (`KismetSystemLibrary.K2_SetTimerDelegate` (`|CreateDelegate` :!event `Fall`) (`self.TimeBeforeFall`))
    (bind (_direction _alpha) (`Timeline|ColorChange` :!via `PlayFromStart`)
      (:`Update`
        (`MaterialInstanceDynamic.SetScalarParameterValue` (`self.LeafMaterial`) "Substract" (`KismetMathLibrary.Lerp` 0.0 0.4 _alpha))))))

(event `Fall`
  (`self.StopLoop`)
  (bind (_direction _alpha) (`Timeline|Timeline` :!via `PlayFromStart`)
    (:`Update`
      (`SkeletalMeshComponent.SetMorphTarget` (`self.LeafPlatform`) "Leaf1" (`KismetMathLibrary.Lerp` 0.0 1.0 _alpha) true)
      (`PrimitiveComponent.SetCollisionEnabled` (`self.Collisions`) "NoCollision"))
    (:`Finished`
      (`KismetSystemLibrary.K2_SetTimerDelegate` (`|CreateDelegate` :!event `Respawn`) (`self.RespawnTime`)))))

(event `Respawn`
  (bind (_direction _alpha) (`Timeline|Timeline_0` :!via `PlayFromStart`)
    (:`Update`
      (`SkeletalMeshComponent.SetMorphTarget` (`self.LeafPlatform`) "Leaf1" (`KismetMathLibrary.Lerp` 1.0 0.0 _alpha) true)
      (`MaterialInstanceDynamic.SetScalarParameterValue` (`self.LeafMaterial`) "Substract" (`KismetMathLibrary.Lerp` 0.4 0.0 _alpha)))
    (:`Finished`
      (`PrimitiveComponent.SetCollisionEnabled` (`self.Collisions`) "QueryAndPhysics")
      (`self.Giggle`))))

(fn `UserConstructionScript`
  (bind _leafplatform (`self.LeafPlatform`))
  (`SkeletalMeshComponent.SetSkeletalMeshAsset` _leafplatform "/Game/ART_GPE/PLATFORMS/CrumbleLeafPlatform/GPE_CrumbleLeafPlatform.GPE_CrumbleLeafPlatform")
  (bind _returnvalue (`PrimitiveComponent.CreateDynamicMaterialInstance` _leafplatform 0 "/Game/ART_Materials/Materials_PropsPainter/ART_MI_PropsPainter/MI_CrumbleLeafPlatform.MI_CrumbleLeafPlatform" "None"))
  (set `self.LeafMaterial` _returnvalue))