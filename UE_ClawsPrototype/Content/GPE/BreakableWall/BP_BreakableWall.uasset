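; BP_BreakableWall is a wall that shatters through a Geometry Collection when it receives GetPowered with a hit location.
; Construction disables physics on the collection; the event enables it and destroys the SMWall mesh.
; To drive the break, it spawns a BP_HitActor at the hit point, launches its sphere along the player-to-hit direction with a large impulse, then destroys it after a brief delay.
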(event `/Game/Interfaces/BPI_WetPowered.GetPowered`
  (params (HitLocation :type "Vector Structure"))
  (set `self.Hit Location` HitLocation)
  (set `self.ImpulseDirection` (`KismetMathLibrary.GetDirectionUnitVector` (`self.K2_GetActorLocation` (`GameplayStatics.GetPlayerCharacter` 0)) (`self.Hit Location`)))
  (`PrimitiveComponent.SetSimulatePhysics` (`self.GeometryCollection`) true)
  (`ActorComponent.K2_DestroyComponent` (`self.SM_Wall`))
  (bind _returnvalue (`|SpawnActorFromClass` "/Game/GPE/BreakableWall/BP_HitActor.BP_HitActor_C" (`KismetMathLibrary.MakeTransform` (`self.Hit Location`)) "AlwaysSpawn" "MultiplyWithRoot" null null))
  (`PrimitiveComponent.AddImpulse` (`/Game/GPE/BreakableWall/BP_HitActor.SM_Sphere` _returnvalue) (* (`self.ImpulseDirection`) 1000000.0) "None" false)
  (`KismetSystemLibrary.Delay` 0.2)
  (`self.K2_DestroyActor` _returnvalue))

(fn `UserConstructionScript`
  (`PrimitiveComponent.SetSimulatePhysics` (`self.GeometryCollection`) false))