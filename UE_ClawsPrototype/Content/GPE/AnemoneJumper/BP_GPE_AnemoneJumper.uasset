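; BP_GPE_AnemoneJumper is an anemone jump pad that launches the player upward on overlapping its LaunchBox, with separate wet and dry velocities.
; Watering inflates the anemone through a morph target and starts a wet-duration timer, while powering dries and deflates it.
; Launches add the height gap to TopPosition to the Z velocity and set jump flags that ABP_AnemoneJumper resets, with droplet VFX when wet.
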(event `self.ReceiveBeginPlay`
  ;[0.8824 0.9294 0.2275] BEGIN PLAY
  ;;[1 1 1] Get Player and PlayerController references
  (bind _get_player_ref (message `/Game/Setup/Remi/BPI_Player.Get Player Ref` (`GameplayStatics.GetPlayerCharacter` 0)))
  (set `self.Player Ref` _get_player_ref)
  (bind _get_pc_ref (message `/Game/Interfaces/BPI_PlayerController.Get PC Ref` (`GameplayStatics.GetPlayerController` 0)))
  (set `self.Player Controller Ref` _get_pc_ref)
  ;;[0.6588 0.2275 0.9294] If Anemone starts on "Wet" state
  (if (`self.bIsWet`)
    (`SkeletalMeshComponent.SetMorphTarget` (`self.SK_Anemone`) "AnemonaInflate" 1.0 true)))

(event `/Game/Interfaces/BPI_WetPowered.GetWatered`
  ;[1 1 1] Get watered
  (set `self.bIsWet` true) ; /!\\ isn't already wet
  (`SkeletalMeshComponent.SetMorphTarget` (`self.SK_Anemone`) "AnemonaInflate" 1.0 true)
  (`KismetSystemLibrary.K2_SetTimerDelegate` (`|CreateDelegate` :!event `DryAnemone`) (`self.WetDuration`)))

(event `DryAnemone`
  ;[1 1 1] Dry anemone
  (set `self.bIsWet` false) ; /!\\ isn't already dry
  (`SkeletalMeshComponent.SetMorphTarget` (`self.SK_Anemone`) "AnemonaInflate" 0.0 true))

(event `/Game/Interfaces/BPI_WetPowered.GetPowered`
  ;[1 1 1] Get powered
  (`GameplayStatics.PlaySound2D` "/Game/SoundDesign/Sounds/PowerClawOff_Cue.PowerClawOff_Cue" 1.0 1.0 0.0 null null)
  (`self.DryAnemone`))

(event `self.LaunchBox.OnComponentBeginOverlap`
  (params (OverlappedComponent :type "PrimitiveComponent Object Reference") (OtherActor :type "Actor Object Reference") (OtherComp :type "PrimitiveComponent Object Reference") (OtherBodyIndex :type Integer) (bFromSweep :type Boolean) (SweepResult :type "HitResult Structure (by ref)"))
  ;[1 1 1] Launch the player when they overlap with LaunchBox
  (if (`KismetSystemLibrary.DoesImplementInterface` OtherActor "/Game/Setup/Remi/BPI_Player.BPI_Player_C")
    (if (`self.bIsWet`)
      (`self.LaunchWet`)
      (else
        (`self.LaunchDry`)))))

(event `LaunchWet`
  (bind (_returnvalue_x _returnvalue_y _returnvalue_z) (`KismetMathLibrary.BreakVector` (- (`SceneComponent.K2_GetComponentLocation` (`self.TopPosition`)) (`self.K2_GetActorLocation` (`self.Player Ref`)))))
  ;[1 1 1] Launch Wet
  (set `self.bNotifyJumpWet` true)
  (`NiagaraFunctionLibrary.SpawnSystemAttached` "/Game/ART_Vfx/Niagara/Systeme/NS_Droplets_Expulsed.NS_Droplets_Expulsed" null "None" (`self.K2_GetActorLocation` (`self.Player Ref`)) (struct) "KeepRelativeOffset" true)
  (`Character.LaunchCharacter` (`self.Player Ref`) (+ (`self.LaunchVelocityWet`) (`KismetMathLibrary.MakeVector` 0.0 0.0 _returnvalue_z)) false true))

(event `LaunchDry`
  (bind (_returnvalue_x _returnvalue_y _returnvalue_z) (`KismetMathLibrary.BreakVector` (- (`SceneComponent.K2_GetComponentLocation` (`self.TopPosition`)) (`self.K2_GetActorLocation` (`self.Player Ref`)))))
  ;[1 1 1] Launch Dry
  (set `self.bNotifyJumpDry` true)
  (`Character.LaunchCharacter` (`self.Player Ref`) (+ (`self.LaunchVelocityDry`) (`KismetMathLibrary.MakeVector` 0.0 0.0 _returnvalue_z)) false true))

(event `ResetJumpNotifications`
  ;[1 1 1] Reset Jump Notifications (called by ABP_AnemoneJumper
  (set `self.bNotifyJumpWet` false)
  (set `self.bNotifyJumpDry` false))

(fn `UserConstructionScript`)