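; Wall variant of the anemone jumper gameplay element, a child Blueprint that takes its behavior from its parent.
; Its begin play, powered, watered, wet launch and dry launch events only forward to the parent.
; The construction script does nothing, as its IsWet check that would set a big wall anemone blockout mesh is disconnected and never runs.
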(event `self.ReceiveBeginPlay`
  (`parent.ReceiveBeginPlay`))

(event `/Game/Interfaces/BPI_WetPowered.GetPowered`
  (`parent.GetPowered`))

(event `/Game/Interfaces/BPI_WetPowered.GetWatered`
  (`parent.GetWatered`))

(event `self.LaunchWet`
  (`parent.LaunchWet`))

(event `self.LaunchDry`
  (`parent.LaunchDry`))

(fn `UserConstructionScript`)