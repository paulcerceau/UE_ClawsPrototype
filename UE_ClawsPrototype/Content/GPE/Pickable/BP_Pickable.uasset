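; Configurable pickable item that hovers, spins and shines until an actor implementing BPI_CanPickStuff overlaps its box.
; The construction script sizes the box and expects exactly one static or skeletal mesh.
; BeginPlay feeds ACHover, loops a rotation timeline and picks a Niagara effect by Type.
; Pickup sends Type to the collector, destroys the visuals and box, plays Seq_PickUp with a timeline-driven camera move and sound, then destroys the actor.
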(event `self.ReceiveBeginPlay`
  (bind _ac_hover (`self.AC_Hover`))
  (bind _ns_pickable (`self.NS_Pickable`))
  ;[0.8824 0.9294 0.2275] BeginPlay
  (bind _asbp_chara_base (cast `/Game/Setup/Remi/BP_CharaBase` (`GameplayStatics.GetPlayerCharacter` 0)))
  (set `self.Actor` _asbp_chara_base)
  ;;[1 1 1] Hovering
  (set `/Game/GPE/Components/AC_Hover.HoveringDuration` (`self.Hovering Duration`) _ac_hover)
  (set `/Game/GPE/Components/AC_Hover.HoveringHeight` (`self.Hovering Height`) _ac_hover)
  (set `/Game/GPE/Components/AC_Hover.DelayBetweenTwoHover` (`self.Delay Between Two Hover`) _ac_hover)
  ;;[1 1 1] Rotating
  (`TimelineComponent.SetPlayRate` (`self.Rotating`) (/ 1.0 (`self.SecondsPerRevolution`)))
  (`self.Rotate`)
  ;;[1 1 1] Shining
  (if (`|EnumEquality` (`self.Type`) "NewEnumerator5")
    (`NiagaraComponent.SetAsset` _ns_pickable "/Game/ART_Vfx/Niagara/Systeme/NS_Pickable_Priority_02.NS_Pickable_Priority_02" true)
    (`NiagaraComponent.SetVariableFloat` _ns_pickable "User.Scale" 3.0)
    (else
      (`NiagaraComponent.SetAsset` _ns_pickable "/Game/ART_Vfx/Niagara/Systeme/NS_Pickable_Priority_01.NS_Pickable_Priority_01" true)
      (`NiagaraComponent.SetVariableFloat` _ns_pickable "User.Scale" 4.0))))

(event `Rotate`
  (bind (_returnvalue_roll _returnvalue_pitch) (`KismetMathLibrary.BreakRotator` (`self.K2_GetActorRotation`)))
  ;[1 1 1] Rotations
  (bind (_direction _curve_rotate_float) (`Timeline|Rotating` :!via `PlayFromStart`)
    (:`Update`
      (`self.K2_SetActorRotation` (`KismetMathLibrary.MakeRotator` _returnvalue_roll _returnvalue_pitch (`KismetMathLibrary.Lerp` 0.0 360.0 _curve_rotate_float))))
    (:`Finished`
      (`self.Rotate`))))

(event `self.PickableBox.OnComponentBeginOverlap`
  (params (OverlappedComponent :type "PrimitiveComponent Object Reference") (OtherActor :type "Actor Object Reference") (OtherComp :type "PrimitiveComponent Object Reference") (OtherBodyIndex :type Integer) (bFromSweep :type Boolean) (SweepResult :type "HitResult Structure (by ref)"))
  (bind (_returnvalue_x _returnvalue_y _returnvalue_z) (`KismetMathLibrary.BreakVector` (`self.K2_GetActorLocation`)))
  (if (`KismetSystemLibrary.DoesImplementInterface` OtherActor "/Game/GPE/Pickable/BPI_CanPickStuff.BPI_CanPickStuff_C")
    (message `/Game/GPE/Pickable/BPI_CanPickStuff.Pick` OtherActor (`self.Type`))
    (bind _sm_pickable (`self.SM_Pickable`)
      (:`then`
        _)
      (:`else`
        (bind _sk_pickable (`self.SK_Pickable`)
          (:`then`
            _)
          (:`else`))))
    (`ActorComponent.K2_DestroyComponent` _sk_pickable)
    (`ActorComponent.K2_DestroyComponent` _sm_pickable)
    (`ActorComponent.K2_DestroyComponent` (`self.PickableBox`))
    (`ActorComponent.K2_DestroyComponent` (`self.NS_Pickable`))
    (bind _returnvalue (`GameplayStatics.GetActorOfClass` "/Game/GPE/Pickable/BP_CineCam_Pickable.BP_CineCam_Pickable_C"))
    (`LevelSequencePlayer.CreateLevelSequencePlayer` "/Game/Cinematics/Sequences/Seq_PickUp.Seq_PickUp" (make `MovieSceneSequencePlaybackSettings` true (struct) 1.0 0.0 false false true true))
    (bind (_direction _alpha) (`Timeline|Zoom`)
      (:`Update`
        (bind (_returnvalue_x_2 _returnvalue_y_2) (`KismetMathLibrary.BreakVector` (`self.K2_GetActorLocation` _returnvalue)))
        (`self.K2_SetActorLocation` _returnvalue (`KismetMathLibrary.MakeVector` _returnvalue_x (`KismetMathLibrary.Lerp` _returnvalue_y_2 (+ _returnvalue_y 2000.0) _alpha) (+ _returnvalue_z 200.0)) false false)
        (`/Engine/EditorBlueprintResources/StandardMacros.DoOnce` false
          (:`Completed`
            (`AkGameplayStatics.PostEvent` (`self.sound`))
            (`AkGameplayStatics.SetRTPCValue` "/Game/WwiseAudio/Game_Parameters/Baptiste_GP/Fade_GP/Fade_GP_PickUp/Fade_GP_PickUp.Fade_GP_PickUp" 1.0))))
      (:`Finished`
        (`KismetSystemLibrary.Delay` 4.38)
        (`self.K2_DestroyActor`)))))

(fn `UserConstructionScript`
  (bind _returnvalue (* (`KismetMathLibrary.Vector_One`) (`self.MeshUniformSize`)))
  ;[1 1 1] Collision box parameters
  (`SceneComponent.SetRelativeScale3D` (`self.PickableBox`) (* (`KismetMathLibrary.Vector_One`) (`self.BoxUniformSize`)))
  ;[1 1 1] Mesh
  ;;[1 1 1] Set Mesh
  (`StaticMeshComponent.SetStaticMesh` (`self.SM_Pickable`) (`self.StaticMesh`))
  (`SkeletalMeshComponent.SetSkeletalMeshAsset` (`self.SK_Pickable`) (`self.SkeletalMesh`))
  ;;;[1 1 1] Avoid to have the two mesh at the same time and no mesh at all
  (set `self.bHasStaticMesh` (`KismetSystemLibrary.IsValid` (`self.StaticMesh`)))
  (set `self.bHasSkeletalMesh` (`KismetSystemLibrary.IsValid` (`self.SkeletalMesh`)))
  (if (xor (`self.bHasStaticMesh`) (`self.bHasSkeletalMesh`))
    ;;[1 1 1] Set mesh other parameters
    (if (`self.bHasStaticMesh`)
      (`SceneComponent.SetRelativeScale3D` (`self.SM_Pickable`) _returnvalue)
      (`SceneComponent.K2_AddLocalOffset` (`self.SM_Pickable`) (`self.Displacement`) false false)
      (else
        (`SceneComponent.SetRelativeScale3D` (`self.SK_Pickable`) _returnvalue)
        (`SceneComponent.K2_AddLocalOffset` (`self.SK_Pickable`) (`self.Displacement`) false false)))
    (else
      (`KismetSystemLibrary.PrintString` "You need to have STRICLY ONE MESH (either a static or a skeletal mesh)"))))