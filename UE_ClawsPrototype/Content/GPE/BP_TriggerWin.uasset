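; BP_TriggerWin is a win trigger volume that ends play by showing the thanks screen.
; On BeginPlay it caches the player character and the PC_ClawsProto controller.
; Any overlap with TBox_Win, with no check on the overlapping actor, adds WB_ThanksScreen to the viewport and disables controller input.
; Disconnected nodes hold an unused pressure-claw check, win sound, spark effect, movement lock and WinScreen flag.
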(event `self.ReceiveBeginPlay`
  (bind _asbp_chara_base (cast `/Game/Setup/Remi/BP_CharaBase` (`GameplayStatics.GetPlayerCharacter` 0)))
  (set `self.get player ref` _asbp_chara_base)
  (bind _aspc_claws_proto (cast `/Game/Setup/PC_ClawsProto` (`GameplayStatics.GetPlayerController` 0)))
  (set `self.As PC Claws Proto_0` _aspc_claws_proto))

(event `self.TBox_Win.OnComponentBeginOverlap`
  (params (OverlappedComponent :type "PrimitiveComponent Object Reference") (OtherActor :type "Actor Object Reference") (OtherComp :type "PrimitiveComponent Object Reference") (OtherBodyIndex :type Integer) (bFromSweep :type Boolean) (SweepResult :type "HitResult Structure (by ref)"))
  (bind _as_pc_claws_proto_0 (`self.As PC Claws Proto_0`))
  (bind _returnvalue (`|CreateWidget` "/Game/UI/WB_ThanksScreen.WB_ThanksScreen_C"))
  (`UserWidget.AddToViewport` _returnvalue 0)
  (`self.DisableInput` _as_pc_claws_proto_0 _as_pc_claws_proto_0))

(fn `UserConstructionScript`)