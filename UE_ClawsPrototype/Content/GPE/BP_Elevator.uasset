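; Elevator set piece that moves the player to a new area through a one-time cinematic transition.
; When a BPI_Player actor overlaps its trigger, it destroys the trigger, disables input and fades to black using the GameMode's widget.
; After a delay it creates an auto-playing Seq_Elevator player and teleports the character to hardcoded coordinates.
; Separate events show the Pink Cave announcement widget and teleport the elevator itself to a fixed, tilted position.
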(event `self.ReceiveBeginPlay`
  (bind _asgm_claws_proto (cast `/Game/Setup/GM_ClawsProto` (`GameplayStatics.GetGameMode`)))
  (set `self.As GM Claws Proto` _asgm_claws_proto)
  (bind _asbp_chara_base (cast `/Game/Setup/Remi/BP_CharaBase` (`GameplayStatics.GetPlayerCharacter` 0)))
  (set `self.As BP Chara Base` _asbp_chara_base))

(event `self.TBox_Activate.OnComponentBeginOverlap`
  (params (OverlappedComponent :type "PrimitiveComponent Object Reference") (OtherActor :type "Actor Object Reference") (OtherComp :type "PrimitiveComponent Object Reference") (OtherBodyIndex :type Integer) (bFromSweep :type Boolean) (SweepResult :type "HitResult Structure (by ref)"))
  (bind _as_bp_chara_base (`self.As BP Chara Base`))
  (bind _wb_blackbg (`/Game/Setup/GM_ClawsProto.WB_BlackBG` (`self.As GM Claws Proto`)))
  (if (`KismetSystemLibrary.DoesImplementInterface` OtherActor "/Game/Setup/Remi/BPI_Player.BPI_Player_C")
    (`ActorComponent.K2_DestroyComponent` (`self.TBox_Activate`))
    (`self.DisableInput` (`self.As BP Chara Base`) (`GameplayStatics.GetPlayerController` 0))
    (`UserWidget.AddToViewport` _wb_blackbg 0)
    (`/Game/UI/WB_BlackBG.FadingIn` _wb_blackbg)
    (`KismetSystemLibrary.Delay` 2.5)
    (`Widget.RemoveFromParent` _wb_blackbg)
    (`LevelSequencePlayer.CreateLevelSequencePlayer` "/Game/Cinematics/Sequences/Seq_Elevator.Seq_Elevator" (make `MovieSceneSequencePlaybackSettings` true (struct) 1.0 0.0 false false true true true true))
    (`self.K2_TeleportTo` _as_bp_chara_base (49610.0 0.0 10195.0) (`self.K2_GetActorRotation` _as_bp_chara_base))))

(event `SequencerEnding`
  (bind _returnvalue (`|CreateWidget` "/Game/UI/Temp-PH/WB_PinkCave_Announcement.WB_PinkCave_Announcement_C"))
  (`UserWidget.AddToViewport` _returnvalue 0))

(event `TPElevator`
  (bind (_returnvalue_roll _returnvalue_pitch _returnvalue_yaw) (`KismetMathLibrary.BreakRotator` (`self.K2_GetActorRotation`)))
  (`self.K2_TeleportTo` (48600.0 -500.0 6400.0) (`KismetMathLibrary.MakeRotator` _returnvalue_roll (+ _returnvalue_pitch 20.0) _returnvalue_yaw)))

(fn `UserConstructionScript`)