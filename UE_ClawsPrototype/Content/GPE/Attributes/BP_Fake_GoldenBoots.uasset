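; BP_Fake_GoldenBoots is a floating golden boots pickup that equips boots when the player's capsule overlaps its box.
; On overlap it calls BootsEquipment on the player controller, fetched at BeginPlay via message calls, then destroys itself.
; Two timelines animate it: one loops a full yaw spin, the other bobs it above its start location with a delay between direction changes.
; An ObtainBoots call is left unconnected.
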(event `self.ReceiveBeginPlay`
  (bind _get_player_ref (message `/Game/Setup/BPI_Player.Get Player Ref` (`GameplayStatics.GetPlayerCharacter` 0)))
  (set `self.PlayerCharacter` _get_player_ref)
  (bind _get_pc_ref (message `/Game/Interfaces/BPI_PlayerController.Get PC Ref` (`GameplayStatics.GetPlayerController` 0)))
  (set `self.PlayerController` _get_pc_ref)
  (set `self.Base Location` (`self.K2_GetActorLocation`))
  (`TimelineComponent.SetPlayRate` (`self.Hovering`) (/ 1.0 (`self.Hovering Length`)))
  (`self.Hover` true)
  (`TimelineComponent.SetPlayRate` (`self.Rotating`) (/ 1.0 (`self.Time per Revolution`)))
  (`self.Rotate`))

(event `self.Box.OnComponentBeginOverlap`
  (params (OverlappedComponent :type "PrimitiveComponent Object Reference") (OtherActor :type "Actor Object Reference") (OtherComp :type "PrimitiveComponent Object Reference") (OtherBodyIndex :type Integer) (bFromSweep :type Boolean) (SweepResult :type "HitResult Structure (by ref)"))
  (if (== OtherComp (`Character.CapsuleComponent` (`self.PlayerCharacter`)))
    (`/Game/Setup/PC_ClawsProto.BootsEquipment` (`self.PlayerController`))
    (`self.K2_DestroyActor`)))

(event `Rotate`
  (bind (_returnvalue_roll _returnvalue_pitch) (`KismetMathLibrary.BreakRotator` (`self.K2_GetActorRotation`)))
  (bind (_direction _curve_rotate_float) (`Timeline|Rotation` :!via `PlayFromStart`)
    (:`Update`
      (`self.K2_SetActorRotation` (`KismetMathLibrary.MakeRotator` _returnvalue_roll _returnvalue_pitch (`KismetMathLibrary.Lerp` 0.0 360.0 _curve_rotate_float))))
    (:`Finished`
      (`self.Rotate`))))

(event `Hover`
  (params (bUp :type Boolean))
  (if bUp
    (bind (_direction _curve_clawhovering_float) (`Timeline|Hovering` :!via `PlayFromStart` :!label _label)
      (:`Update`
        (`self.Set Hover Location` _curve_clawhovering_float))
      (:`Finished`
        (`KismetSystemLibrary.Delay` (`self.Delay between Two Hover`))
        (`self.Hover` (not bUp))))
    (else
      (goto _label :!via `ReverseFromEnd`))))

(fn `Set Hover Location`
  (params (Alpha :type "Float (double-precision)"))
  (bind (_base_location_x _base_location_y _base_location_z) (`KismetMathLibrary.BreakVector` (`self.Base Location`)))
  (`self.K2_SetActorLocation` (`KismetMathLibrary.MakeVector` _base_location_x _base_location_y (+ (`KismetMathLibrary.Lerp` 0.0 (`self.Hovering Height`) Alpha) _base_location_z))))

(fn `UserConstructionScript`)