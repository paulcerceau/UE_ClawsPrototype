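; Trigger box that plays the Pink Arsene door-opening cutscene when the player overlaps it while possessing the mustache.
; On overlap it fades in the game mode's black screen and disables input and movement, then starts the level sequence and removes the overlay.
; Fixed delays, rather than sequence callbacks, time the follow-up: it reveals the door icon, shows a map-updated widget and destroys itself.
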(event `self.ReceiveBeginPlay`
  (bind _asbp_chara_base (cast `/Game/Setup/Remi/BP_CharaBase` (`GameplayStatics.GetPlayerCharacter` 0)))
  (set `self.As BP Chara Base` _asbp_chara_base)
  (bind _asgm_claws_proto (cast `/Game/Setup/GM_ClawsProto` (`GameplayStatics.GetGameMode`)))
  (set `self.As GM Claws Proto` _asgm_claws_proto))

(event `self.TBox_Sequencer.OnComponentBeginOverlap`
  (params (OverlappedComponent :type "PrimitiveComponent Object Reference") (OtherActor :type "Actor Object Reference") (OtherComp :type "PrimitiveComponent Object Reference") (OtherBodyIndex :type Integer) (bFromSweep :type Boolean) (SweepResult :type "HitResult Structure (by ref)"))
  (bind _as_bp_chara_base (`self.As BP Chara Base`))
  (bind _wb_blackbg (`/Game/Setup/GM_ClawsProto.WB_BlackBG` (`self.As GM Claws Proto`)))
  (if (and (`KismetSystemLibrary.DoesImplementInterface` OtherActor "/Game/Setup/Remi/BPI_Player.BPI_Player_C") (`/Game/Setup/Remi/BP_CharaBase.bPossessMustache` (`self.As BP Chara Base`)))
    (`UserWidget.AddToViewport` _wb_blackbg 0)
    (`/Game/UI/WB_BlackBG.FadingIn` _wb_blackbg)
    (`self.DisableInput` _as_bp_chara_base (`GameplayStatics.GetPlayerController` 0))
    (`CharacterMovementComponent.DisableMovement` (`Character.CharacterMovement` _as_bp_chara_base))
    (`KismetSystemLibrary.Delay` 2.5)
    (`LevelSequencePlayer.CreateLevelSequencePlayer` "/Game/Cinematics/Sequences/Seq_PinkArseneDoorOpening.Seq_PinkArseneDoorOpening" (make `MovieSceneSequencePlaybackSettings` true (struct) 1.0 0.0 false false true true true true))
    (`Widget.RemoveFromParent` (`/Game/Setup/GM_ClawsProto.WB_BlackBG` (`self.As GM Claws Proto`)))
    (`KismetSystemLibrary.Delay` 19.0)
    (`self.UpdateMap`)))

(event `UpdateMap`
  (`Widget.SetVisibility` (`/Game/UI/WB_SpecialLeftMenu.IMG_DoorIcon` (`/Game/Setup/GM_ClawsProto.WB_SpecialLeft` (`self.As GM Claws Proto`))) "Visible")
  (bind _returnvalue (`|CreateWidget` "/Game/UI/WB_MapUpdated.WB_MapUpdated_C"))
  (`UserWidget.AddToViewport` _returnvalue 0)
  (`KismetSystemLibrary.Delay` 2.0)
  (`self.K2_DestroyActor`))

(fn `UserConstructionScript`)