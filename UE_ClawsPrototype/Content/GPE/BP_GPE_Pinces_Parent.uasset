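; Parent Blueprint for claw (pince) pickups that the player collects by touching them.
; It caches the player reference at BeginPlay through a GetPlayerRefMessage call on the player character.
; When that player overlaps the capsule, it passes its SMPince mesh and first material to ObtainClaw, then destroys itself.
; GetPincePowerRef is an empty function here.
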(event `self.ReceiveBeginPlay`
  (bind _get_player_ref (message `/Game/Setup/BPI_Player.Get Player Ref` (`GameplayStatics.GetPlayerCharacter` 0)))
  (set `self.PlayerCharacter Ref` _get_player_ref))

(event `self.Capsule.OnComponentBeginOverlap`
  (params (OverlappedComponent :type "PrimitiveComponent Object Reference") (OtherActor :type "Actor Object Reference") (OtherComp :type "PrimitiveComponent Object Reference") (OtherBodyIndex :type Integer) (bFromSweep :type Boolean) (SweepResult :type "HitResult Structure (by ref)"))
  (bind _playercharacter_ref (`self.PlayerCharacter Ref`))
  (bind _sm_pince (`self.SM_Pince`))
  (if (== OtherActor _playercharacter_ref)
    (`/Game/Setup/BP_CharaBase.ObtainClaw` _playercharacter_ref (`StaticMeshComponent.StaticMesh` _sm_pince) (`PrimitiveComponent.GetMaterial` _sm_pince 0))
    (`self.K2_DestroyActor`)))

(fn `Get PincePower Ref`
  (returns (`Get Power Pince` :type "/Game/GPE/BP_GPE_Pinces_Power Object Reference"))
  (return null))

(fn `UserConstructionScript`)