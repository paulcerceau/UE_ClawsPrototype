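; Unwalkable wall actor that builds a row of instanced wall meshes along a spline in the construction script.
; UnwalkableType adds a start corner, an end corner, both or neither, with flat segments filling the remaining spline length.
; Flat segment spacing comes from the mesh's Z bounds, uniform scale and a percentage overlap.
; Instances are placed unrotated in local space, with the start corner at the actor origin.
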(fn `CreateEndCornerUnwallInstance`
  (params (Offset :type "Float (double-precision)"))
  (`InstancedStaticMeshComponent.AddInstance` (`self.EndCornerWallInstancedStaticMesh`) (`KismetMathLibrary.MakeTransform` (`SplineComponent.GetLocationAtDistanceAlongSpline` (`self.Spline`) (+ (* (+ (`self.NumberOfFlatUnWallInstances`) 1) (`self.Spacing`)) (`local.Offset`)) "Local") (struct) (`KismetMathLibrary.Conv_DoubleToVector` (`self.UniformScale`))) false))

(fn `CreateFlatUnwallInstances`
  (params (InstancesCount :type Integer) (Offset :type "Float (double-precision)"))
  (bind _result (`/Engine/EditorBlueprintResources/StandardMacros.DecrementInt` InstancesCount)
    (:`  `
      (for _index (range (+ _result 1))
        (`InstancedStaticMeshComponent.AddInstance` (`self.FlatWallInstancedStaticMesh`) (`KismetMathLibrary.MakeTransform` (`SplineComponent.GetLocationAtDistanceAlongSpline` (`self.Spline`) (+ (* _index (`self.Spacing`)) (`local.Offset`)) "Local") (struct) (`KismetMathLibrary.Conv_DoubleToVector` (`self.UniformScale`))) false)))))

(fn `CreateStartCornerUnwallInstance`
  (`InstancedStaticMeshComponent.AddInstance` (`self.StartCornerWallInstancedStaticMesh`) (`KismetMathLibrary.MakeTransform` (0.0 0.0 0.0) (struct) (`KismetMathLibrary.Conv_DoubleToVector` (`self.UniformScale`))) false))

(fn `UserConstructionScript`
  (bind (_startcornerunwallmeshsize_x _startcornerunwallmeshsize_y _startcornerunwallmeshsize_z) (`KismetMathLibrary.BreakVector` (`self.StartCornerUnWallMeshSize`)))
  (bind (_flatunwallmeshsize_x _flatunwallmeshsize_y _flatunwallmeshsize_z) (`KismetMathLibrary.BreakVector` (`self.FlatUnWallMeshSize`)))
  (bind (_startcornerunwallmeshsize_x_2 _startcornerunwallmeshsize_y_2 _startcornerunwallmeshsize_z_2) (`KismetMathLibrary.BreakVector` (`self.StartCornerUnWallMeshSize`)))
  (bind (_endcornerunwallmeshsize_x _endcornerunwallmeshsize_y _endcornerunwallmeshsize_z) (`KismetMathLibrary.BreakVector` (`self.EndCornerUnWallMeshSize`)))
  (bind (_endcornerunwallmeshsize_x_2 _endcornerunwallmeshsize_y_2 _endcornerunwallmeshsize_z_2) (`KismetMathLibrary.BreakVector` (`self.EndCornerUnWallMeshSize`)))
  (bind (_startcornerunwallmeshsize_x_3 _startcornerunwallmeshsize_y_3 _startcornerunwallmeshsize_z_3) (`KismetMathLibrary.BreakVector` (`self.StartCornerUnWallMeshSize`)))
  (bind (_startcornerunwallmeshsize_x_4 _startcornerunwallmeshsize_y_4 _startcornerunwallmeshsize_z_4) (`KismetMathLibrary.BreakVector` (`self.StartCornerUnWallMeshSize`)))
  (bind (_flatunwallmeshsize_x_2 _flatunwallmeshsize_y_2 _flatunwallmeshsize_z_2) (`KismetMathLibrary.BreakVector` (`self.FlatUnWallMeshSize`)))
  (bind (_min _max) (break `Box` (`StaticMesh.GetBoundingBox` (`self.EndCornerUnWallMesh`))))
  (bind (_min_2 _max_2) (break `Box` (`StaticMesh.GetBoundingBox` (`self.FlatUnWallMesh`))))
  (bind (_min_3 _max_3) (break `Box` (`StaticMesh.GetBoundingBox` (`self.StartCornerUnWallMesh`))))
  (bind _returnvalue (* _startcornerunwallmeshsize_z (`self.UniformScale`) (- 1.0 (/ (`self.FlatUnWallPercentageOffset`) 100.0))))
  (`StaticMeshComponent.SetStaticMesh` (`self.FlatWallInstancedStaticMesh`) (`self.FlatUnWallMesh`))
  (set `self.FlatUnWallMeshSize` (- _max_2 _min_2))
  (set `self.Spacing` (* (`self.UniformScale`) (- _flatunwallmeshsize_z (* _flatunwallmeshsize_z_2 (/ (`self.FlatUnWallPercentageOffset`) 100.0)))))
  (if (`|EnumInequality` (`self.UnwalkableType`) "NewEnumerator3")
    (`StaticMeshComponent.SetStaticMesh` (`self.StartCornerWallInstancedStaticMesh`) (`self.StartCornerUnWallMesh`))
    (set `self.StartCornerUnWallMeshSize` (- _max_3 _min_3))
    (`StaticMeshComponent.SetStaticMesh` (`self.EndCornerWallInstancedStaticMesh`) (`self.EndCornerUnWallMesh`))
    (set `self.EndCornerUnWallMeshSize` (- _max _min)))
  (switch `/Game/GPE/UnwalkableWall/EUnwalkableType` (`self.UnwalkableType`)
    (:`NewEnumerator1`
      ;[1 1 1] Start Corner
      (`self.CreateStartCornerUnwallInstance`)
      (bind _output_get (set `self.NumberOfFlatUnWallInstances` (`KismetMathLibrary.FFloor` (/ (- (`SplineComponent.GetSplineLength` (`self.Spline`)) (* _startcornerunwallmeshsize_z_2 (`self.UniformScale`))) (`self.Spacing`)))))
      (`self.CreateFlatUnwallInstances` _output_get (* _startcornerunwallmeshsize_z_4 (`self.UniformScale`) (- 1.0 (/ (`self.FlatUnWallPercentageOffset`) 100.0)))))
    (:`NewEnumerator0`
      ;[1 1 1] End Corner
      (bind _output_get_2 (set `self.NumberOfFlatUnWallInstances` (`KismetMathLibrary.FFloor` (/ (- (`SplineComponent.GetSplineLength` (`self.Spline`)) (* _endcornerunwallmeshsize_z_2 (`self.UniformScale`))) (`self.Spacing`)))))
      (`self.CreateFlatUnwallInstances` _output_get_2)
      (`self.CreateEndCornerUnwallInstance` 0.0))
    (:`NewEnumerator2`
      (`self.CreateStartCornerUnwallInstance`)
      (bind _output_get_3 (set `self.NumberOfFlatUnWallInstances` (`KismetMathLibrary.FFloor` (/ (- (`SplineComponent.GetSplineLength` (`self.Spline`)) (* _startcornerunwallmeshsize_z_3 (`self.UniformScale`)) (* _endcornerunwallmeshsize_z (`self.UniformScale`))) (`self.Spacing`)))))
      (`self.CreateFlatUnwallInstances` _output_get_3 _returnvalue)
      (`self.CreateEndCornerUnwallInstance` _returnvalue))
    (:`NewEnumerator3`
      (bind _output_get_4 (set `self.NumberOfFlatUnWallInstances` (`KismetMathLibrary.FFloor` (/ (`SplineComponent.GetSplineLength` (`self.Spline`)) (`self.Spacing`)))))
      (`self.CreateFlatUnwallInstances` _output_get_4))))