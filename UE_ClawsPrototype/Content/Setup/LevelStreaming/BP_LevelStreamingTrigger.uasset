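; Trigger box actor that asynchronously streams selected levels in and out when a BPI_Player actor overlaps it.
; Construction script expands load and unload enum bitmasks into SLV_-prefixed level name arrays and sizes the box.
; LoadLevels steps through its array by re-calling itself, while UnloadLevels calls LoadLevels after its first unload instead of itself.
; A debug visibility event from the player controller toggles the box's visibility.
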(event `ToggleVisibility`
  (bind _triggerbox (`self.TriggerBox`))
  ;[0.6588 0.2275 0.9294] Toggle visibility
  (`SceneComponent.SetHiddenInGame` _triggerbox (not (`SceneComponent.bHiddenInGame` _triggerbox)) false)
  (`SceneComponent.SetHiddenInGame` _triggerbox (not (`SceneComponent.bHiddenInGame` _triggerbox)) false))

(event `self.ReceiveBeginPlay`
  ;[0.8824 0.9294 0.2275] BEGIN PLAY
  (bind _get_pc_ref (message `/Game/Interfaces/BPI_PlayerController.Get PC Ref` (`GameplayStatics.GetPlayerController` 0)))
  (add `/Game/Setup/Remi/PC_ClawsProto.DebugVisibility` _get_pc_ref (`|CreateDelegate` :!event `ToggleVisibility`)))

(event `self.TriggerBox.OnComponentBeginOverlap`
  (params (OverlappedComponent :type "PrimitiveComponent Object Reference") (OtherActor :type "Actor Object Reference") (OtherComp :type "PrimitiveComponent Object Reference") (OtherBodyIndex :type Integer) (bFromSweep :type Boolean) (SweepResult :type "HitResult Structure (by ref)"))
  ;[1 1 1] On trigger enter
  ;;[0.6588 0.2275 0.9294] Extra security, shouldn't be needed
  (if (`KismetSystemLibrary.DoesImplementInterface` OtherActor "/Game/Setup/Remi/BPI_Player.BPI_Player_C")
    (`|ExecutionSequence`
      (:`then_0`
        (if (> (`KismetArrayLibrary.Array_Length` (`self.LevelsToLoadNames`)) 0)
          (set `self.CurrentlyLoadingLevelIndex` 0)
          (set `self.LoadingLevelsMaxIndex` (- (`KismetArrayLibrary.Array_Length` (`self.LevelsToLoadNames`)) 1))
          (`self.LoadLevels`)))
      (:`then_1`
        (if (> (`KismetArrayLibrary.Array_Length` (`self.LevelsToUnloadNames`)) 0)
          (set `self.CurrentlyUnloadingLevelIndex` 0)
          (set `self.UnloadingLevelsMaxIndex` (- (`KismetArrayLibrary.Array_Length` (`self.LevelsToUnloadNames`)) 1))
          (`self.UnloadLevels`))))))

(event `LoadLevels`
  ;[1 1 1] Asynchronous load
  (`GameplayStatics.LoadStreamLevel` (`|GetArrayItem` (`self.LevelsToLoadNames`) (`self.CurrentlyLoadingLevelIndex`)) true)
  (if (< (`self.CurrentlyLoadingLevelIndex`) (`self.LoadingLevelsMaxIndex`))
    (`/Engine/EditorBlueprintResources/StandardMacros.IncrementInt` (`self.CurrentlyLoadingLevelIndex`)
      (:`  `
        (`self.LoadLevels`)))))

(event `UnloadLevels`
  ;[1 1 1] Asynchronous unload
  (`GameplayStatics.UnloadStreamLevel` (`|GetArrayItem` (`self.LevelsToUnloadNames`) (`self.CurrentlyUnloadingLevelIndex`)))
  (if (< (`self.CurrentlyUnloadingLevelIndex`) (`self.UnloadingLevelsMaxIndex`))
    (`/Engine/EditorBlueprintResources/StandardMacros.IncrementInt` (`self.CurrentlyUnloadingLevelIndex`)
      (:`  `
        (`self.LoadLevels`)))))

(fn `Convert Levels Selection to Names List`
  (params (SelectedLevels :type Integer64) (ListToUpdate :type "Array of Name"))
  (bind _enumvalue (foreach `/Game/Setup/LevelStreaming/ELevelsNames` false)
    (:`LoopBody`
      (bind _returnvalue (`KismetMathLibrary.FFloor64` (`KismetMathLibrary.MultiplyMultiply_FloatFloat` 2.0 (`KismetMathLibrary.Conv_ByteToDouble` _enumvalue))))
      (if (== (`KismetMathLibrary.And_Int64Int64` (`local.SelectedLevels`) _returnvalue) _returnvalue)
        (bind _returnvalue_2 (`|GetEnumeratorNameAsString` _enumvalue))
        (if (`KismetStringLibrary.StartsWith` _returnvalue_2 "SLV_")
          (`KismetArrayLibrary.Array_Add` (`local.ListToUpdate`) (`KismetStringLibrary.Conv_StringToName` _returnvalue_2))
          (`KismetSystemLibrary.PrintString` _returnvalue_2))))
    (:`then`
      (`KismetSystemLibrary.PrintString` "====="))))

(fn `UserConstructionScript`
  (locals (Storage :type Integer))
  (`self.Convert Levels Selection to Names List` (`self.LevelsToLoad`) (`self.LevelsToLoadNames`))
  (`self.Convert Levels Selection to Names List` (`self.LevelsToUnload`) (`self.LevelsToUnloadNames`))
  (`BoxComponent.SetBoxExtent` (`self.TriggerBox`) (`KismetMathLibrary.MakeVector` 10.0 200.0 (`self.BrushLength`)) true))