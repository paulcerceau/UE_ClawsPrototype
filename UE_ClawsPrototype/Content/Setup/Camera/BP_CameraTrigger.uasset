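; A placeable camera trigger volume that changes the camera's distance, angle and offsets when an actor overlaps its box.
; Overlap fetches the actor's camera through a message call and sends it the settings with an inverted transition speed, optionally only when the player controller's left/right direction matches.
; The construction script sizes the box and orients or hides the direction arrow, while a player controller event toggles debug visibility.
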(event `self.ReceiveBeginPlay`
  (bind _get_pc_ref (message `/Game/Interfaces/BPI_PlayerController.Get PC Ref` (`GameplayStatics.GetPlayerController` 0)))
  (bind _output_get (set `self.PlayerController` _get_pc_ref))
  (add `/Game/Setup/PC_ClawsProto.DebugVisibility` _output_get (delegate `HideShowDebug`)))

(event `HideShowDebug`
  (bind _output_get (set `self.bShowDebug` (not (`self.bShowDebug`))))
  (`SceneComponent.SetHiddenInGame` (`self.CollisionBox`) (not _output_get) true))

(event `self.CollisionBox.OnComponentBeginOverlap`
  (params (OverlappedComponent :type "PrimitiveComponent Object Reference") (OtherActor :type "Actor Object Reference") (OtherComp :type "PrimitiveComponent Object Reference") (OtherBodyIndex :type Integer) (bFromSweep :type Boolean) (SweepResult :type "HitResult Structure (by ref)"))
  (if (`|EnumEquality` (`self.Direction`) "NewEnumerator0")
    (bind _camera (message `/Game/Setup/BPI_Player.GetCamera` OtherActor :!label _label))
    (`self.TransferCameraParameters` _camera)
    (else
      (bind _direction (`/Game/Setup/PC_ClawsProto.GetIntegerDirection` (`self.PlayerController`)))
      (set `self.PlayerDirection` _direction)
      (if (or (and (`|EnumEquality` (`self.Direction`) "NewEnumerator1") (== (`self.PlayerDirection`) 1)) (and (`|EnumEquality` (`self.Direction`) "NewEnumerator2") (== (`self.PlayerDirection`) -1)))
        (goto _label)))))

(fn `GetCameraParameters`
  (returns (Distance :type "Float (double-precision)") (Angle :type "Rotator Structure") (HorizontalOffset :type "Float (double-precision)") (VerticalOffset :type "Float (double-precision)"))
  (return (`self.Distance`) (`self.Angle`) (`self.HorizontalOffset`) (`self.VerticalOffset`)))

(fn `TransferCameraParameters`
  (params (Camera :type "/Game/Setup/Camera/BP_Camera Object Reference"))
  (message `/Game/Setup/Camera/BPI_CameraController.ChangeCameraSettings` Camera (make `/Game/Setup/Camera/SCameraSettings` (`self.Distance`) (`self.Angle`) (`self.HorizontalOffset`) (`self.VerticalOffset`)) (/ 1.0 (`self.TransitionSpeed`))))

(fn `UserConstructionScript`
  (bind _arrow (`self.Arrow`))
  (bind _collisionbox (`self.CollisionBox`))
  (bind _arrow_2 (`self.Arrow`))
  (`SceneComponent.SetHiddenInGame` _collisionbox (`self.HiddenInGame`) true)
  (`BoxComponent.SetBoxExtent` _collisionbox (`self.BoxDimensions`) true)
  (switch `/Game/Setup/Camera/ECameraTriggerDirection` (`self.Direction`)
    (:`NewEnumerator0`
      (`SceneComponent.SetVisibility` _arrow_2 false false))
    (:`NewEnumerator2`
      (`SceneComponent.K2_SetRelativeRotation` _arrow (struct :`Pitch` 180.0) false false)
      (`SceneComponent.SetVisibility` _arrow_2 true false :!label _label))
    (:`NewEnumerator1`
      (`SceneComponent.K2_SetRelativeRotation` :`self` _arrow)
      (goto _label))))