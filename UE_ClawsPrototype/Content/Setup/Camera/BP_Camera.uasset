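; Camera actor that follows the first player's character from a configurable offset and becomes the view target on BeginPlay.
; Every tick it places itself relative to the player using horizontal, vertical and distance offsets along world axes, combining a fixed base rotation with an adjustable angle.
; A ChangeCameraParameters event stores new camera settings and prints a debug message.
; SetPlayerPosition caches the player's location but is not called here.
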(event `self.ReceiveBeginPlay`
  (set `self.Player` (`GameplayStatics.GetPlayerCharacter` 0))
  (set `self.BaseAngle` (struct :`Yaw` -90.0))
  (`PlayerController.SetViewTargetWithBlend` (`GameplayStatics.GetPlayerController` 0) self 0.0 "VTBlend_Linear" 0.0 false))

(event `self.ReceiveTick`
  (params (DeltaSeconds :type "Float (single-precision)"))
  (`self.SetCameraTransform`))

(event `/Game/Setup/Camera/BPI_CameraController.ChangeCameraParameters`
  (params (CameraSettings :type "/Game/Setup/Camera/SCameraSettings Structure"))
  (set `self.Camera Settings` CameraSettings)
  (`KismetSystemLibrary.PrintString` "TRIGGER CAMERA PARAM"))

(fn `SetCameraTransform`
  (bind _returnvalue (`self.GetTransform` (`self.Player`)))
  (`self.K2_SetActorLocationAndRotation` (`KismetMathLibrary.MakeVector` (+ (`self.HorizontalOffset`) (.x (.location _returnvalue))) (+ (.y (.location _returnvalue)) (`self.Distance`)) (+ (.z (.location _returnvalue)) (`self.VerticalOffset`))) (`KismetMathLibrary.ComposeRotators` (`self.BaseAngle`) (`self.Angle`))))

(fn `SetPlayerPosition`
  (bind _returnvalue_location (`KismetMathLibrary.BreakTransform` (`self.GetTransform` (`self.Player`))))
  (set `self.PlayerPosition` _returnvalue_location))

(fn `UserConstructionScript`)