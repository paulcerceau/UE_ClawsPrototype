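; BP_CameraBound is a placeable camera bound volume built on a collision box.
; The construction script sizes the box from BoxDimensions and sets its in-game visibility from HiddenInGame.
; On BeginPlay it gets the player controller through a GetPCRefMessage call and binds to its debug visibility event, which toggles the box's visibility.
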(event `self.ReceiveBeginPlay`
  (bind _get_pc_ref (message `/Game/Interfaces/BPI_PlayerController.Get PC Ref` (`GameplayStatics.GetPlayerController` 0)))
  (bind _output_get (set `self.PlayerController` _get_pc_ref))
  (add `/Game/Setup/Remi/PC_ClawsProto.DebugVisibility` _output_get (delegate `HideShowDebug`)))

(event `HideShowDebug`
  (bind _output_get (set `self.bShowDebug` (not (`self.bShowDebug`))))
  (`SceneComponent.SetHiddenInGame` (`self.CollisionBox`) (not _output_get) true))

(fn `UserConstructionScript`
  (bind _collisionbox (`self.CollisionBox`))
  (`SceneComponent.SetHiddenInGame` _collisionbox (`self.HiddenInGame`) true)
  (`BoxComponent.SetBoxExtent` _collisionbox (`self.BoxDimensions`) true))