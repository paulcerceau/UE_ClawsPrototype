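; BP_CharaBase is a base character Blueprint that holds the player's shared state and can be given a claw.
; On BeginPlay it caches the CharacterMovement gravity, walk speed and jump velocity defaults, and finds the level's BP_Camera with GetActorOfClass.
; ObtainClaw applies the passed mesh and material to the Claw component and sets HasClaw.
; GetPlayerRef and GetCamera expose the character and cached camera to callers.
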(event `self.ReceiveBeginPlay`
  (bind _charactermovement (`self.CharacterMovement`))
  (set `self.Default gravity` (`CharacterMovementComponent.GravityScale` _charactermovement))
  (set `self.Default Max Walk Speed` (`CharacterMovementComponent.MaxWalkSpeed` _charactermovement))
  (set `self.Default jump Z velocity` (`CharacterMovementComponent.JumpZVelocity` _charactermovement))
  (bind _returnvalue (`GameplayStatics.GetActorOfClass` "/Game/Setup/Camera/BP_Camera.BP_Camera_C"))
  (set `self.Camera` _returnvalue))

(fn `Get Player Ref`
  (returns (`Get Player Ref` :type "/Game/Setup/BP_CharaBase Object Reference") (NewParam :type "Float (double-precision)"))
  (return self 0.0))

(fn `GetCamera`
  (returns (Camera :type "/Game/Setup/Camera/BP_Camera Object Reference"))
  (return (`self.Camera`)))

(fn `ObtainClaw`
  (params (`Static Mesh` :type "StaticMesh Object Reference") (Material :type "MaterialInterface Object Reference"))
  (bind _claw (`self.Claw`))
  ;[0.5843 0.3137 0.8902] Hardcodé, on essaiera plutôt de passer la directement la référence de la pince - CORRIGE DIRECTEMENT
  (`StaticMeshComponent.SetStaticMesh` _claw `Static Mesh`)
  (`PrimitiveComponent.SetMaterial` _claw 0 Material)
  (set `self.has claw` true))

(fn `UserConstructionScript`)