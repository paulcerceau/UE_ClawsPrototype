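; Player controller for menus that creates the main menu, credits, options and pause menu widgets.
; On BeginPlay it builds and stores them, sets game-and-UI input and calls Add Mapping Context with none specified.
; In Lv_MainMenu it also hides the cursor and shows the main menu.
; A CinematicSound event adds and starts a media sound component, while a 2D cinematic music call sits unconnected.
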(event `self.ReceiveBeginPlay`
  (`self.Initialize Widgets` self)
  (`WidgetBlueprintLibrary.SetInputMode_GameAndUIEx` self null)
  (`EnhancedInputSubsystemInterface.AddMappingContext` (pcsubsystem `EnhancedInputLocalPlayerSubsystem` self) null 0 (struct))
  (bind _returnvalue (`GameplayStatics.GetCurrentLevelName` true))
  (if (`KismetStringLibrary.EqualEqual_StrStr` _returnvalue "Lv_MainMenu")
    (set `self.bShowMouseCursor` false)
    (`UserWidget.AddToViewport` (`self.WB_MainMenu`) 0)))

(event `CinematicSound`
  (bind _returnvalue (`AddComponent|NODE_AddMediaSoundComponent-0`))
  (`SynthComponent.Start` _returnvalue))

(fn `Initialize Widgets`
  (params (`Player Controller` :type "PlayerController Object Reference"))
  (bind _returnvalue (`|CreateWidget` "/Game/UI/WB_MainMenu.WB_MainMenu_C" `Player Controller`))
  (set `self.WB_MainMenu` _returnvalue)
  (bind _returnvalue_2 (`|CreateWidget` "/Game/UI/WB_Credits.WB_Credits_C" `Player Controller`))
  (set `self.WB_Credits` _returnvalue_2)
  (bind _returnvalue_3 (`|CreateWidget` "/Game/UI/WB_Options.WB_Options_C" `Player Controller`))
  (set `self.WB_Options` _returnvalue_3)
  (bind _returnvalue_4 (`|CreateWidget` "/Game/UI/WB_PauseMenu.WB_PauseMenu_C" `Player Controller`))
  (set `self.WB_PauseMenu` _returnvalue_4))

(fn `UserConstructionScript`)