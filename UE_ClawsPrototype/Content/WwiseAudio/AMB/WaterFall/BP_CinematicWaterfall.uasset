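; BP_CinematicWaterfall is a trigger actor that starts and stops Wwise audio for a cinematic waterfall.
; When a BP_CharaBase leaves the BoxInt volume, it posts the AkPlay event on CineCameraActor.
; When one enters the BoxOut volume, it posts the AkStop event on the same actor.
; Each trigger passes through its own DoOnce, so it fires a single time.
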(event `self.Box int.OnComponentEndOverlap`
  (params (OverlappedComponent :type "PrimitiveComponent Object Reference") (OtherActor :type "Actor Object Reference") (OtherComp :type "PrimitiveComponent Object Reference") (OtherBodyIndex :type Integer))
  (cast `/Game/Setup/Remi/BP_CharaBase` OtherActor)
  (`/Engine/EditorBlueprintResources/StandardMacros.DoOnce` false
    (:`Completed`
      (`AkGameplayStatics.PostEvent` (`self.Ak_Play`) (`self.CineCameraActor`)))))

(event `self.Box out.OnComponentBeginOverlap`
  (params (OverlappedComponent :type "PrimitiveComponent Object Reference") (OtherActor :type "Actor Object Reference") (OtherComp :type "PrimitiveComponent Object Reference") (OtherBodyIndex :type Integer) (bFromSweep :type Boolean) (SweepResult :type "HitResult Structure (by ref)"))
  (cast `/Game/Setup/Remi/BP_CharaBase` OtherActor)
  (`/Engine/EditorBlueprintResources/StandardMacros.DoOnce` false
    (:`Completed`
      (`AkGameplayStatics.PostEvent` (`self.Ak_Stop`) (`self.CineCameraActor`)))))

(fn `UserConstructionScript`)