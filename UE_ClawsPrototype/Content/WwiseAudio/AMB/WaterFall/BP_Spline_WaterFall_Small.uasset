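; Spline-based Wwise ambient emitter for a small waterfall, keeping its sound at the point along the spline nearest the player.
; Every Tick moves the AkPlay component to the spline's closest world-space point to the player pawn and draws a debug sphere there.
; The component's associated Ak event is also re-posted every Tick, not once.
; When the Ak_Play component activates, the actor's occlusion refresh interval is set to zero.
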(event `self.ReceiveTick`
  (params (DeltaSeconds :type "Float (single-precision)"))
  (bind _returnvalue (`SplineComponent.FindLocationClosestToWorldLocation` (`self.Spline`) (`self.K2_GetActorLocation` (`GameplayStatics.GetPlayerPawn` 0)) "World"))
  (`AkGameObject.PostAssociatedAkEvent` :`self` (`self.Ak_Play`))
  (`SceneComponent.K2_SetWorldLocation` (`self.Ak_Play`) _returnvalue false false)
  (`KismetSystemLibrary.DrawDebugSphere` _returnvalue 100.0 12 (struct :`R` 1.0 :`B` 0.027538 :`A` 1.0) 0.0 2.0))

(event `self.Ak_Play.OnComponentActivated`
  (params (Component :type "ActorComponent Object Reference") (bReset :type Boolean))
  (`AkGameplayStatics.SetOcclusionRefreshInterval` 0.0 self))

(fn `UserConstructionScript`)