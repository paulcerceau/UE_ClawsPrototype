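; River ambience actor whose Wwise emitter follows the spline point closest to the player pawn every Tick, with occlusion refresh interval zeroed.
; Two In/Out box pairs detect BP_CharaBase crossing direction through shared overlap flags.
; After both flags are set, leaving an Out box posts the sound and leaving an In box stops it.
; The second pair's begin-overlap handlers set the opposite flags to those their end-overlap handlers clear.
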(event `self.ReceiveTick`
  (params (DeltaSeconds :type "Float (single-precision)"))
  (`SceneComponent.K2_SetWorldLocation` (`self.Ak_Play`) (`SplineComponent.FindLocationClosestToWorldLocation` (`self.Spline`) (`self.K2_GetActorLocation` (`GameplayStatics.GetPlayerPawn` 0)) "World") false false))

(event `self.Ak_Play.OnComponentActivated`
  (params (Component :type "ActorComponent Object Reference") (bReset :type Boolean))
  (`AkGameplayStatics.SetOcclusionRefreshInterval` 0.0 self))

(event `self.Box_Out_01.OnComponentBeginOverlap`
  (params (OverlappedComponent :type "PrimitiveComponent Object Reference") (OtherActor :type "Actor Object Reference") (OtherComp :type "PrimitiveComponent Object Reference") (OtherBodyIndex :type Integer) (bFromSweep :type Boolean) (SweepResult :type "HitResult Structure (by ref)"))
  ;[1 1 1] Box 1
  (cast `/Game/Setup/Remi/BP_CharaBase` OtherActor)
  (set `self.InsideOut` true)
  (if (`self.InsideIn`)
    (set `self.Both` true)))

(event `self.Box_In_01.OnComponentBeginOverlap`
  (params (OverlappedComponent :type "PrimitiveComponent Object Reference") (OtherActor :type "Actor Object Reference") (OtherComp :type "PrimitiveComponent Object Reference") (OtherBodyIndex :type Integer) (bFromSweep :type Boolean) (SweepResult :type "HitResult Structure (by ref)"))
  ;[1 1 1] Box 1
  (cast `/Game/Setup/Remi/BP_CharaBase` OtherActor)
  (set `self.InsideIn` true)
  (if (`self.InsideOut`)
    (set `self.Both` true)))

(event `self.Box_In_01.OnComponentEndOverlap`
  (params (OverlappedComponent :type "PrimitiveComponent Object Reference") (OtherActor :type "Actor Object Reference") (OtherComp :type "PrimitiveComponent Object Reference") (OtherBodyIndex :type Integer))
  ;[1 1 1] Box 1
  (cast `/Game/Setup/Remi/BP_CharaBase` OtherActor)
  (set `self.InsideIn` false)
  (if (`self.Both`)
    (`AkGameObject.Stop` (`self.Ak_Play`))
    (set `self.Both` false)))

(event `self.Box_Out_01.OnComponentEndOverlap`
  (params (OverlappedComponent :type "PrimitiveComponent Object Reference") (OtherActor :type "Actor Object Reference") (OtherComp :type "PrimitiveComponent Object Reference") (OtherBodyIndex :type Integer))
  ;[1 1 1] Box 1
  (cast `/Game/Setup/Remi/BP_CharaBase` OtherActor)
  (set `self.InsideOut` false)
  (if (`self.Both`)
    (`AkGameObject.PostAssociatedAkEvent` :`self` (`self.Ak_Play`))
    (set `self.Both` false)))

(event `self.Box_In_02.OnComponentBeginOverlap`
  (params (OverlappedComponent :type "PrimitiveComponent Object Reference") (OtherActor :type "Actor Object Reference") (OtherComp :type "PrimitiveComponent Object Reference") (OtherBodyIndex :type Integer) (bFromSweep :type Boolean) (SweepResult :type "HitResult Structure (by ref)"))
  (cast `/Game/Setup/Remi/BP_CharaBase` OtherActor)
  (set `self.InsideOut` true)
  (if (`self.InsideIn`)
    (set `self.Both` true)))

(event `self.Box_Out_02.OnComponentBeginOverlap`
  (params (OverlappedComponent :type "PrimitiveComponent Object Reference") (OtherActor :type "Actor Object Reference") (OtherComp :type "PrimitiveComponent Object Reference") (OtherBodyIndex :type Integer) (bFromSweep :type Boolean) (SweepResult :type "HitResult Structure (by ref)"))
  (cast `/Game/Setup/Remi/BP_CharaBase` OtherActor)
  (set `self.InsideIn` true)
  (if (`self.InsideOut`)
    (set `self.Both` true)))

(event `self.Box_In_02.OnComponentEndOverlap`
  (params (OverlappedComponent :type "PrimitiveComponent Object Reference") (OtherActor :type "Actor Object Reference") (OtherComp :type "PrimitiveComponent Object Reference") (OtherBodyIndex :type Integer))
  (cast `/Game/Setup/Remi/BP_CharaBase` OtherActor)
  (set `self.InsideIn` false)
  (if (`self.Both`)
    (`AkGameObject.Stop` (`self.Ak_Play`))
    (set `self.Both` false)))

(event `self.Box_Out_02.OnComponentEndOverlap`
  (params (OverlappedComponent :type "PrimitiveComponent Object Reference") (OtherActor :type "Actor Object Reference") (OtherComp :type "PrimitiveComponent Object Reference") (OtherBodyIndex :type Integer))
  (cast `/Game/Setup/Remi/BP_CharaBase` OtherActor)
  (set `self.InsideOut` false)
  (if (`self.Both`)
    (`AkGameObject.PostAssociatedAkEvent` :`self` (`self.Ak_Play`))
    (set `self.Both` false)))

(fn `UserConstructionScript`)