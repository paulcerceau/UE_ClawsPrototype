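; Wwise audio transition trigger that switches ambience and music from the forest cave to the pink cave.
; Player entry into Box_In fires once, fading the forest RTPCs after a delay, then later starting and raising the pink layers on CharaBase.
; Each pink RTPC's interpolation time is wired from its PostEvent return value.
; Player exit from Box_Out fires once and stops pink ambience and music, without restoring the forest RTPCs.
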(event `self.Box_In.OnComponentBeginOverlap`
  (params (OverlappedComponent :type "PrimitiveComponent Object Reference") (OtherActor :type "Actor Object Reference") (OtherComp :type "PrimitiveComponent Object Reference") (OtherBodyIndex :type Integer) (bFromSweep :type Boolean) (SweepResult :type "HitResult Structure (by ref)"))
  (bind _charabase (`self.CharaBase`))
  (if (`KismetSystemLibrary.DoesImplementInterface` OtherActor "/Game/Setup/Remi/BPI_Player.BPI_Player_C")
    (`/Engine/EditorBlueprintResources/StandardMacros.DoOnce` false
      (:`Completed`
        (`KismetSystemLibrary.Delay` 10.0)
        (`AkGameplayStatics.SetRTPCValue` "/Game/WwiseAudio/Game_Parameters/Baptiste_GP/Fade_GP/Fade_GP_CaveForest/Fade_GP_CaveForest.Fade_GP_CaveForest" 0.0 5 _charabase)
        (`AkGameplayStatics.SetRTPCValue` "/Game/WwiseAudio/Game_Parameters/Baptiste_GP/Fade_GP/Fade_GP_CaveForest/Fade_GP_Music_CaveForest.Fade_GP_Music_CaveForest" 0.0 5 _charabase)
        (`KismetSystemLibrary.Delay` 5.0)
        (bind _returnvalue (`AkGameplayStatics.PostEvent` "/Game/WwiseAudio/Events/Work_Unit_Baptiste_Events/Ambiences/Cave_Pink/Play_AMB_CavePink.Play_AMB_CavePink" _charabase))
        (`AkGameplayStatics.SetRTPCValue` "/Game/WwiseAudio/Game_Parameters/Baptiste_GP/Fade_GP/Fade_GP_CavePink/Fade_GP_CavePink.Fade_GP_CavePink" 1.0 _returnvalue _charabase)
        (bind _returnvalue_2 (`AkGameplayStatics.PostEvent` "/Game/WwiseAudio/Events/Work_Unit_Baptiste_Events/Ambiences/Cave_Pink/Music_CavePink/Play_Music_CavePink.Play_Music_CavePink" _charabase))
        (`AkGameplayStatics.SetRTPCValue` "/Game/WwiseAudio/Game_Parameters/Baptiste_GP/Fade_GP/Fade_GP_CavePink/Fade_GP_Music_CavePink.Fade_GP_Music_CavePink" 1.0 _returnvalue_2 _charabase)))))

(event `self.Box_Out.OnComponentEndOverlap`
  (params (OverlappedComponent :type "PrimitiveComponent Object Reference") (OtherActor :type "Actor Object Reference") (OtherComp :type "PrimitiveComponent Object Reference") (OtherBodyIndex :type Integer))
  (bind _charabase (`self.CharaBase`))
  (if (`KismetSystemLibrary.DoesImplementInterface` OtherActor "/Game/Setup/Remi/BPI_Player.BPI_Player_C")
    (`/Engine/EditorBlueprintResources/StandardMacros.DoOnce` false
      (:`Completed`
        (`AkGameplayStatics.PostEvent` "/Game/WwiseAudio/Events/Work_Unit_Baptiste_Events/Ambiences/Cave_Pink/Stop_AMB_CavePink.Stop_AMB_CavePink" _charabase)
        (`AkGameplayStatics.PostEvent` "/Game/WwiseAudio/Events/Work_Unit_Baptiste_Events/Ambiences/Cave_Pink/Music_CavePink/Stop_Music_CavePink.Stop_Music_CavePink" _charabase)))))

(fn `UserConstructionScript`)