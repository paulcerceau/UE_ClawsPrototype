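; Audio portal that switches the Cave Forest Wwise ambience as a BP_CharaBase character passes between outside and inside.
; Overlapping In and Out trigger boxes set flags, with Both latched while the character is in both, so the first box exited gives the crossing direction.
; Leaving Out first plays the ambience and raises its fade RTPC on the character.
; Leaving In first resets the RTPC and posts the stop event.
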(event `self.Box_OutTrigger.OnComponentBeginOverlap`
  (params (OverlappedComponent :type "PrimitiveComponent Object Reference") (OtherActor :type "Actor Object Reference") (OtherComp :type "PrimitiveComponent Object Reference") (OtherBodyIndex :type Integer) (bFromSweep :type Boolean) (SweepResult :type "HitResult Structure (by ref)"))
  (cast `/Game/Setup/Remi/BP_CharaBase` OtherActor)
  (set `self.Inside Out` true)
  (if (`self.Inside In`)
    (set `self.Both` true)))

(event `self.Box_InTrigger.OnComponentBeginOverlap`
  (params (OverlappedComponent :type "PrimitiveComponent Object Reference") (OtherActor :type "Actor Object Reference") (OtherComp :type "PrimitiveComponent Object Reference") (OtherBodyIndex :type Integer) (bFromSweep :type Boolean) (SweepResult :type "HitResult Structure (by ref)"))
  (cast `/Game/Setup/Remi/BP_CharaBase` OtherActor)
  (set `self.Inside In` true)
  (if (`self.Inside Out`)
    (set `self.Both` true)))

(event `self.Box_InTrigger.OnComponentEndOverlap`
  (params (OverlappedComponent :type "PrimitiveComponent Object Reference") (OtherActor :type "Actor Object Reference") (OtherComp :type "PrimitiveComponent Object Reference") (OtherBodyIndex :type Integer))
  (bind _asbp_chara_base (cast `/Game/Setup/Remi/BP_CharaBase` OtherActor))
  (set `self.Inside In` false)
  (if (`self.Both`)
    (`AkGameplayStatics.SetRTPCValue` "/Game/WwiseAudio/Game_Parameters/Baptiste_GP/Fade_GP/Fade_GP_CaveForest/Fade_GP_CaveForest.Fade_GP_CaveForest" 0.0 (stale `self.Box_OutTrigger.OnComponentEndOverlap` _returnvalue) _asbp_chara_base)
    (set `self.Both` false)
    (`AkGameplayStatics.PostEvent` "/Game/WwiseAudio/Events/Work_Unit_Baptiste_Events/Ambiences/Cave_Forest/Stop_AMB_CaveForest.Stop_AMB_CaveForest")))

(event `self.Box_OutTrigger.OnComponentEndOverlap`
  (params (OverlappedComponent :type "PrimitiveComponent Object Reference") (OtherActor :type "Actor Object Reference") (OtherComp :type "PrimitiveComponent Object Reference") (OtherBodyIndex :type Integer))
  (bind _asbp_chara_base (cast `/Game/Setup/Remi/BP_CharaBase` OtherActor))
  (set `self.Inside Out` false)
  (if (`self.Both`)
    (bind _returnvalue (`AkGameplayStatics.PostEvent` "/Game/WwiseAudio/Events/Work_Unit_Baptiste_Events/Ambiences/Cave_Forest/Play_AMB_CaveForest.Play_AMB_CaveForest" _asbp_chara_base))
    (`AkGameplayStatics.SetRTPCValue` "/Game/WwiseAudio/Game_Parameters/Baptiste_GP/Fade_GP/Fade_GP_CaveForest/Fade_GP_CaveForest.Fade_GP_CaveForest" 1.0 _returnvalue _asbp_chara_base)
    (set `self.Both` false)))

(fn `UserConstructionScript`)