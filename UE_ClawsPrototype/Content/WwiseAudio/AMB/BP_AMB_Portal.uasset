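; Wwise audio portal that switches ambience and music as the player crosses between its In and Out trigger boxes.
; Overlap flags detect crossing direction by which box is left first after both were occupied.
; Leaving Out first posts new ambience and music events and raises their RTPCs; leaving In first resets the RTPCs.
; Construction derives RTPC names from assets, and a player-controller binding supports debug visibility.
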(event `self.ReceiveBeginPlay`
  ;[0.8824 0.9294 0.2275] BEGIN PLAY
  (bind _get_pc_ref (message `/Game/Interfaces/BPI_PlayerController.Get PC Ref` (`GameplayStatics.GetPlayerController` 0)))
  (add `/Game/Setup/Remi/PC_ClawsProto.DebugVisibility` _get_pc_ref (`|CreateDelegate` :!event `ToggleVisibility`)))

(event `ToggleVisibility`
  ;[0.6588 0.2275 0.9294] Set game visibility
  (bind _output_get (set `self.bIsVisible` (not (`self.bIsVisible`))))
  (`SceneComponent.SetHiddenInGame` (`self.DefaultSceneRoot`) (not _output_get) true))

(event `self.Box_OutTrigger.OnComponentBeginOverlap`
  (params (OverlappedComponent :type "PrimitiveComponent Object Reference") (OtherActor :type "Actor Object Reference") (OtherComp :type "PrimitiveComponent Object Reference") (OtherBodyIndex :type Integer) (bFromSweep :type Boolean) (SweepResult :type "HitResult Structure (by ref)"))
  (if (`KismetSystemLibrary.DoesImplementInterface` OtherActor "/Game/Setup/Remi/BPI_Player.BPI_Player_C")
    (set `self.Inside Out` true)
    (if (`self.Inside In`)
      (set `self.Both` true))))

(event `self.Box_InTrigger.OnComponentBeginOverlap`
  (params (OverlappedComponent :type "PrimitiveComponent Object Reference") (OtherActor :type "Actor Object Reference") (OtherComp :type "PrimitiveComponent Object Reference") (OtherBodyIndex :type Integer) (bFromSweep :type Boolean) (SweepResult :type "HitResult Structure (by ref)"))
  (if (`KismetSystemLibrary.DoesImplementInterface` OtherActor "/Game/Setup/Remi/BPI_Player.BPI_Player_C")
    (set `self.Inside In` true)
    (if (`self.Inside Out`)
      (set `self.Both` true))))

(event `self.Box_InTrigger.OnComponentEndOverlap`
  (params (OverlappedComponent :type "PrimitiveComponent Object Reference") (OtherActor :type "Actor Object Reference") (OtherComp :type "PrimitiveComponent Object Reference") (OtherBodyIndex :type Integer))
  (bind _bp_charabase (`self.Bp_Charabase`))
  (if (`KismetSystemLibrary.DoesImplementInterface` OtherActor "/Game/Setup/Remi/BPI_Player.BPI_Player_C")
    (set `self.Inside In` false)
    (if (`self.Both`)
      (`AkGameplayStatics.SetRTPCValue` (`self.RtcpValueAMB`) 0.0 (stale `self.Box_OutTrigger.OnComponentEndOverlap` _returnvalue) _bp_charabase (`self.RtpcNameAMB`))
      (`AkGameplayStatics.SetRTPCValue` (`self.RtpcValueMusic`) 0.0 (stale `self.Box_OutTrigger.OnComponentEndOverlap` _returnvalue_2) _bp_charabase (`self.RtpcNameMusic`))
      (set `self.Both` false))))

(event `self.Box_OutTrigger.OnComponentEndOverlap`
  (params (OverlappedComponent :type "PrimitiveComponent Object Reference") (OtherActor :type "Actor Object Reference") (OtherComp :type "PrimitiveComponent Object Reference") (OtherBodyIndex :type Integer))
  (bind _bp_charabase (`self.Bp_Charabase`))
  (if (`KismetSystemLibrary.DoesImplementInterface` OtherActor "/Game/Setup/Remi/BPI_Player.BPI_Player_C")
    (set `self.Inside Out` false)
    (if (`self.Both`)
      (bind _returnvalue (`AkGameplayStatics.PostEvent` (`self.PlayNewestAMB`) _bp_charabase))
      (`AkGameplayStatics.SetRTPCValue` (`self.RtcpValueAMB`) 1.0 _returnvalue _bp_charabase (`self.RtpcNameAMB`))
      (bind _returnvalue_2 (`AkGameplayStatics.PostEvent` (`self.PlayNewestMusic`) _bp_charabase))
      (`AkGameplayStatics.SetRTPCValue` (`self.RtpcValueMusic`) 1.0 _returnvalue_2 _bp_charabase (`self.RtpcNameMusic`))
      (set `self.Both` false))))

(fn `UserConstructionScript`
  (set `self.RtpcNameAMB` (`KismetStringLibrary.Conv_StringToName` (`KismetSystemLibrary.GetDisplayName` (`self.RtcpValueAMB`))))
  (set `self.RtpcNameMusic` (`KismetStringLibrary.Conv_StringToName` (`KismetSystemLibrary.GetDisplayName` (`self.RtpcValueMusic`)))))