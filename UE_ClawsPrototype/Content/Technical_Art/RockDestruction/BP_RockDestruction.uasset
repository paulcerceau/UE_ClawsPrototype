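; Rock destruction actor that plays a baked vertex animation texture (VAT) animation on its mesh.
; BeginPlay creates a dynamic material instance for the mesh and applies the PlayRate variable to the AnimRock timeline.
; The PlayAnimRock event restarts that timeline, which drives the material's Display Frame parameter through the animation's frames, so the motion comes from the material.
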(event `self.ReceiveBeginPlay`
  (bind _returnvalue (`PrimitiveComponent.CreateDynamicMaterialInstance` (`self.vertex_animation_textures1_mesh`) 0 null "None"))
  (set `self.RockMat` _returnvalue)
  (`TimelineComponent.SetPlayRate` (`self.AnimRock`) (`self.PlayRate`)))

(event `PlayAnimRock`
  (bind (_direction _alpha) (`Timeline|AnimRock` :!via `PlayFromStart`)
    (:`Update`
      (`MaterialInstanceDynamic.SetScalarParameterValue` (`self.RockMat`) "Display Frame" (`KismetMathLibrary.Lerp` 0.0 120.0 _alpha)))))

(fn `UserConstructionScript`)