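; BP_SprintParticles is a VFX actor for sprint particles that follows the player character along X and Z.
; On BeginPlay it caches the player character and controller references through message calls.
; Each tick it shows its root hierarchy unless the player is falling, mirrors actor X scale by the controller's integer direction, and places the root at a direction-flipped offset from the character.
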(event `self.ReceiveBeginPlay`
  (bind _get_player_ref (message `/Game/Setup/Remi/BPI_Player.Get Player Ref` (`GameplayStatics.GetPlayerCharacter` 0)))
  (set `self.Player Character Ref` _get_player_ref)
  (bind _get_pc_ref (message `/Game/Interfaces/BPI_PlayerController.Get PC Ref` (`GameplayStatics.GetPlayerController` 0)))
  (set `self.PlayerController` _get_pc_ref))

(event `self.ReceiveTick`
  (params (DeltaSeconds :type "Float (single-precision)"))
  (bind (_offset_x _offset_y _offset_z) (`KismetMathLibrary.BreakVector` (`self.Offset`)))
  (bind _defaultsceneroot (`self.DefaultSceneRoot`))
  (bind (_returnvalue_x _returnvalue_y _returnvalue_z) (`KismetMathLibrary.BreakVector` (`self.K2_GetActorLocation` (`self.Player Character Ref`))))
  (if (`/Game/Setup/Remi/PC_ClawsProto.IsNotFalling` (`self.PlayerController`))
    (`SceneComponent.SetVisibility` _defaultsceneroot true true)
    (bind _direction (`/Game/Setup/Remi/PC_ClawsProto.GetIntegerDirection` (`self.PlayerController`)))
    (bind _output_get (set `self.CharacterDirection` _direction))
    (`self.SetActorScale3D` (`KismetMathLibrary.MakeVector` (`KismetMathLibrary.Conv_IntToDouble` _output_get) 1.0 1.0))
    (`SceneComponent.K2_SetWorldLocation` (`self.DefaultSceneRoot`) (`KismetMathLibrary.MakeVector` (+ _returnvalue_x (* _offset_x (`self.CharacterDirection`))) 0.0 (+ _returnvalue_z _offset_z)) false false)
    (else
      (`SceneComponent.SetVisibility` _defaultsceneroot false true))))

(fn `Get PC Ref`
  (returns (`Get PC ref` :type "/Game/Setup/Remi/PC_ClawsProto Object Reference"))
  (return null))

(fn `Get Player Ref`
  (returns (`Get Player Ref` :type "/Game/Setup/Remi/BP_CharaBase Object Reference"))
  (return null))

(fn `GetCamera`
  (returns (Camera :type "/Game/Setup/Camera/BP_Camera Object Reference"))
  (return null))

(fn `UserConstructionScript`)